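; BP_DestructibleBase is a base actor for scenery that reacts to BP_BulletBase hits on its Collision overlap.
; A bullet flagged Destructibal destroys the OriginalSence component and disables collision, and the bullet itself is left alive.
; Other bullets are destroyed and briefly nudge the actor by their forward vector, applied as a local offset.
; After a short delay, the actor snaps back to the transform cached at BeginPlay.
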(event OnComponentBeginOverlap(Collision)
  (params (OverlappedComponent :type Primitive%20Component%20Object%20Reference) (OtherActor :type Actor%20Object%20Reference) (OtherComp :type Primitive%20Component%20Object%20Reference) (OtherBodyIndex :type Integer) (bFromSweep :type Boolean) (SweepResult :type Hit%20Result%20Structure%20%28by%20ref%29))
  (bind _asbp_bullet_base (Utilities|Casting|CastToBP_BulletBase OtherActor))
  (Development|PrintString "Ahhh")
  (if (Variables|/Game/Hero/Base/Blueprint/BP_BulletBase.BP_BulletBase_C|GetDestructibal _asbp_bullet_base)
    (Components|DestroyComponent (Variables|Default|GetOriginalSence))
    (Collision|SetCollisionEnabled (Variables|Default|GetCollision) "NoCollision")
    (else
      (Variables|Default|SetHitVector (Transformation|GetActorForwardVector _asbp_bullet_base))
      (Actor|DestroyActor _asbp_bullet_base)
      (Transformation|AddActorLocalOffset self (* (Variables|Default|GetHitVector) 2.0) false false)
      (Utilities|FlowControl|Delay 0.2)
      (Transformation|SetActorTransform self (Variables|Default|GetOriginalTransfrom)))))

(event EventBeginPlay
  (Variables|Default|SetOriginalTransfrom (Transformation|GetActorTransform self)))

(fn ConstructionScript)