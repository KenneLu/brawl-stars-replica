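; Shelly's normal fire skill actor, which spawns a fan-shaped spread of BP_Bullet_Shelly_Normal projectiles and then destroys itself.
; On BeginPlay it starts half of SectorAngle left of its facing and loops through BulletNumberMax shots, passing its owner to each bullet.
; Yaw advances by SectorAngle divided by the bullet count, so the last shot falls one step short of the sector's far edge.
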(event EventBeginPlay
  (bind _self self)
  (Variables|Default|SetBullet%20Number (Variables|Default|GetBullet%20Number%20Max))
  (Variables|Default|SetRotation (Transformation|GetActorRotation _self))
  (Variables|Default|SetLocation (Transformation|GetActorLocation _self))
  (Variables|Default|SetRotation (Math|Rotator|MakeRotator (.Roll (Math|Rotator|BreakRotator (Variables|Default|GetRotation))) (.Pitch (Math|Rotator|BreakRotator (Variables|Default|GetRotation))) (- (.Yaw (Math|Rotator|BreakRotator (Variables|Default|GetRotation))) (/ (Variables|Default|GetSectorAngle) 2.0))))
  (while (!= (Variables|Default|GetBullet%20Number) 0)
    (Game|SpawnActorfromClass "/Game/Hero/Shelly/Blueprint/BP_Bullet_Shelly_Normal.BP_Bullet_Shelly_Normal_C" (Math|Transform|MakeTransform (Variables|Default|GetLocation) (Variables|Default|GetRotation) "1,1,1") "Undefined" (Components|GetOwner) 0)
    (Variables|Default|SetBullet%20Number (- (Variables|Default|GetBullet%20Number) 1))
    (Variables|Default|SetRotation (Math|Rotator|MakeRotator (.Roll (Math|Rotator|BreakRotator (Variables|Default|GetRotation))) (.Pitch (Math|Rotator|BreakRotator (Variables|Default|GetRotation))) (+ (.Yaw (Math|Rotator|BreakRotator (Variables|Default|GetRotation))) (/ (Variables|Default|GetSectorAngle) (Math|Conversions|ToFloat(Integer) (Variables|Default|GetBullet%20Number%20Max)))))))
  (Actor|DestroyActor))

(fn ConstructionScript)