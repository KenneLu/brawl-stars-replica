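; BP_Bullet_Shelly_Ultimate is the projectile for Shelly's ultimate, which knocks back characters with a strong impulse.
; On BeginPlay it enables destructible sensing through SenceDestructibal.
; Cube overlaps that pass CheckTeamate push the valid Enemy along the cube's forward vector.
; HitEnemy recharges the ultimate, then applies the same impulse and calls ApplyDamageAndDestroy if Enemy is valid.
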(event OnComponentBeginOverlap(Cube)
  (params (OverlappedComponent :type Primitive%20Component%20Object%20Reference) (OtherActor :type Actor%20Object%20Reference) (OtherComp :type Primitive%20Component%20Object%20Reference) (OtherBodyIndex :type Integer) (bFromSweep :type Boolean) (SweepResult :type Hit%20Result%20Structure%20%28by%20ref%29))
  (bind _enemy (Variables|Default|GetEnemy))
  (bind _returnvalue (CallFunction|CheckTeamate OtherActor))
  (if _returnvalue
    (Utilities|IsValid _enemy
      (:Is%20Valid
        (Physics|AddImpulse (Variables|/Script/Engine.Character|GetCharacterMovement _enemy) (* (Math|Vector|GetForwardVector (Variables|Default|GetCube)) 1e+05) false)))))

(event EventBeginPlay
  (Variables|Default|SetSenceDestructibal true))

(event EventHitEnemy
  (bind _enemy (Variables|Default|GetEnemy))
  (CallFunction|RechageUltimate)
  (Utilities|IsValid _enemy
    (:Is%20Valid
      (Physics|AddImpulse (Variables|/Script/Engine.Character|GetCharacterMovement _enemy) (* (Math|Vector|GetForwardVector (Variables|Default|GetCube)) 1e+05) false)
      (CallFunction|ApplyDamageandDestroy))))

(fn ConstructionScript
  (|CallParentFunction))