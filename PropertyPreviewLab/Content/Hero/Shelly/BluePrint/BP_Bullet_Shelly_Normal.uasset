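; Shelly's normal-attack bullet actor, made of several bullet meshes with particle trails.
; The construction script applies the configured mesh and particle template to four of each, and a world scale to all but the fourth mesh.
; Trails begin on BeginPlay and end on destruction.
; The actor destroys itself when its collision overlaps any hero other than its owner, with no damage applied in this graph.
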(event OnComponentBeginOverlap(Collision)
  (params (OverlappedComponent :type Primitive%20Component%20Object%20Reference) (OtherActor :type Actor%20Object%20Reference) (OtherComp :type Primitive%20Component%20Object%20Reference) (OtherBodyIndex :type Integer) (bFromSweep :type Boolean) (SweepResult :type Hit%20Result%20Structure%20%28by%20ref%29))
  (bind _asbp_hero_base (Utilities|Casting|CastToBP_HeroBase OtherActor))
  (if (!= _asbp_hero_base (Components|GetOwner))
    (Actor|DestroyActor)))

(event EventBeginPlay
  (Effects|Particles|Trails|BeginTrails (Variables|Default|GetParticleSystem) "Trail1" "Trail2" "ETrailWidthMode_FromFirst" 1.0))

(event EventDestroyed
  (Effects|Particles|Trails|EndTrails (Variables|Default|GetParticleSystem)))

(fn ConstructionScript
  (bind _bullet (Variables|Default|GetBullet))
  (bind _staticmeshtype (Variables|Default|GetStaticMeshType))
  (|CallParentFunction)
  (Effects|Components|ParticleSystem|SetTemplate (Variables|Default|GetParticleSystem) (Variables|Default|GetParticleType))
  (Utilities|FlowControl|Sequence
    (:then_0
      (Components|StaticMesh|SetStaticMesh _bullet _staticmeshtype)
      (Transformation|SetWorldScale3D _bullet (Variables|Default|GetBulletWorldScale)))
    (:then_1
      (Components|StaticMesh|SetStaticMesh (Variables|Default|GetBullet1) _staticmeshtype))
    (:then_2
      (Components|StaticMesh|SetStaticMesh (Variables|Default|GetBullet2) _staticmeshtype))
    (:then_3
      (Components|StaticMesh|SetStaticMesh (Variables|Default|GetBullet3) _staticmeshtype))))