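; Playable hero Shelly, a character that fires a normal shot and an ultimate shot from a separate gun actor.
; BeginPlay spawns the gun and attaches it to the right wrist socket, and Destroyed removes it with the hero.
; Fire and Ultimate inputs play the same fire montage, then on blend out spawn their respective shot actor at the gun's bone socket, facing the capsule's forward direction.
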(event EventBeginPlay
  (bind _returnvalue (Game|SpawnActorfromClass "/Game/Hero/Shelly/BluePrint/BP_Shelly_Gun.BP_Shelly_Gun_C" (Math|Transform|MakeTransform "0.000000,-250.000000,0.000000" "-90.000000,180.000000,0.000000" "1,1,1") "Undefined" self 0))
  (bind _output_get (Variables|Default|SetGun _returnvalue))
  (Transformation|AttachComponentToComponent _output_get (Variables|Character|GetMesh) "R_wrist_s" "KeepRelative" "KeepRelative" "KeepRelative" true))

(event EventDestroyed
  (bind _gun (Variables|Default|GetGun))
  (Utilities|IsValid _gun
    (:Is%20Valid
      (Actor|DestroyActor _gun))))

(event Input|ActionEvents|InputActionFire
  (params (Key :type Key%20Structure :default "None"))
  (bind _gun (Variables|Default|GetGun))
  (:Pressed
    (Animation|Montage|PlayMontage (Variables|Character|GetMesh) "/Game/Hero/Shelly/Animation/Shelly_Fire_Montage.Shelly_Fire_Montage"
      (:OnBlendOut
        (Utilities|IsValid _gun
          (:Is%20Valid
            (Game|SpawnActorfromClass "/Game/Hero/Shelly/BluePrint/BP_Sheklly_Fire_Noremal.BP_Sheklly_Fire_Noremal_C" (Math|Transform|MakeTransform (Transformation|GetSocketLocation (Variables|/Game/Hero/Shelly/BluePrint/BP_Shelly_Gun.BP_Shelly_Gun_C|GetSkeletalMesh _gun) "L_gunbone_02_s_end") (Math|Conversions|RotationFromXVector (Math|Vector|GetForwardVector (Variables|Default|GetCapsuleComponent))) "1,1,1") "Undefined" 0 0)))))))

(event Input|ActionEvents|InputActionUltimate
  (params (Key :type Key%20Structure :default "None"))
  (bind _gun (Variables|Default|GetGun))
  (:Pressed
    (Animation|Montage|PlayMontage (Variables|Character|GetMesh) "/Game/Hero/Shelly/Animation/Shelly_Fire_Montage.Shelly_Fire_Montage"
      (:OnBlendOut
        (Utilities|IsValid _gun
          (:Is%20Valid
            (Game|SpawnActorfromClass "/Game/Hero/Shelly/BluePrint/BP_Sheklly_Fire_Ultimate.BP_Sheklly_Fire_Ultimate_C" (Math|Transform|MakeTransform (Transformation|GetSocketLocation (Variables|/Game/Hero/Shelly/BluePrint/BP_Shelly_Gun.BP_Shelly_Gun_C|GetSkeletalMesh _gun) "L_gunbone_02_s_end") (Math|Conversions|RotationFromXVector (Math|Vector|GetForwardVector (Variables|Default|GetCapsuleComponent))) "1,1,1") "Undefined" 0 0)))))))

(fn ConstructionScript
  (|CallParentFunction))