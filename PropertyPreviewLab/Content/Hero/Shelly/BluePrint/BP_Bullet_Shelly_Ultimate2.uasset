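; Shelly's ultimate bullet Blueprint, which knocks back the enemy it hits and deals damage.
; On hit it recharges the ultimate, stops AI movement on bot enemies, launches the enemy along the Cube's forward vector, then applies damage and destroys itself.
; The construction script runs the parent's setup, then assigns configurable meshes and Niagara effects to four bullet and four effect components and sets scales.
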(event EventHitEnemy
  (bind _enemy (Variables|Default|GetEnemy))
  (bind _returnvalue (Pawn|GetController _enemy))
  (CallFunction|RechageUltimate)
  (Utilities|IsValid _enemy
    (:Is%20Valid
      (if (and (Pawn|IsBotControlled _enemy) (Utilities|IsValid _returnvalue))
        ;[1 1 1] AI Stop Movement
        (AI|Navigation|StopMovement _returnvalue))
      (Physics|AddImpulse (Variables|/Script/Engine.Character|GetCharacterMovement (Variables|Default|GetEnemy)) (* (Math|Vector|GetForwardVector (Variables|Default|GetCube)) 1e+03) true)
      (CallFunction|ApplyDamageandDestroy))))

(fn ConstructionScript
  (bind _bullet (Variables|Default|GetBullet))
  (bind _staticmeshtype (Variables|Default|GetStaticMeshType))
  (|CallParentFunction)
  (Class|NiagaraComponent|SetAsset (Variables|Default|GetNiagara) (Variables|Default|GetNiagaraType))
  (Transformation|SetWorldScale3D (Variables|Default|GetNiagara1) "1.000000,1.000000,1.000000")
  (Utilities|FlowControl|Sequence
    (:then_0
      (Components|StaticMesh|SetStaticMesh _bullet _staticmeshtype)
      (Transformation|SetWorldScale3D _bullet (Variables|Default|GetBulletWorldScale)))
    (:then_1
      (Components|StaticMesh|SetStaticMesh (Variables|Default|GetBullet1) _staticmeshtype))
    (:then_2
      (Components|StaticMesh|SetStaticMesh (Variables|Default|GetBullet2) _staticmeshtype))
    (:then_3
      (Components|StaticMesh|SetStaticMesh (Variables|Default|GetBullet3) _staticmeshtype))))