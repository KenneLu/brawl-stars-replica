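; Hero skill manager component that gates normal and ultimate skill input through the SkillReleasable lock struct.
; Check functions test press or release enable, readiness and, for ultimates, whether the last one has ended.
; Successful ultimate checks also have side effects: both disable pressing, and release clears the ended flag.
; Off the server, these changes are passed to SetServerSkillReleasable to sync the server's copy.
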(event Custom|SetServerSkillReleasable
  (params (SkillReleasable :type F%20Skill%20Release%20Lock%20Structure))
  (Variables|Default|SetSkill%20Releasable SkillReleasable))

(event Custom|ResetUltmateRelease
  (Utilities|Struct|SetmembersinFSkillReleaseLock (Variables|Default|GetSkill%20Releasable) true true true))

(event EventBeginPlay)

(event EventTick
  (params (DeltaSeconds :type Float%20%28single-precision%29)))

(fn CheckNormalPress
  (bind _skill_releasable (Variables|Default|GetSkill%20Releasable))
  (bind (_ispressenable _isreleaseenable _isnormalready) (Utilities|Struct|BreakFSkillReleaseLock _skill_releasable))
  (if (and _ispressenable _isnormalready)
    (return true)
    (else
      (return false))))

(fn CheckNoremalRelease
  (bind _skill_releasable (Variables|Default|GetSkill%20Releasable))
  (bind (_ispressenable _isreleaseenable _isnormalready) (Utilities|Struct|BreakFSkillReleaseLock _skill_releasable))
  (if (and _isreleaseenable _isnormalready)
    (return true)
    (else
      (return false))))

(fn CheckUltimatePress
  (bind _skill_releasable (Variables|Default|GetSkill%20Releasable))
  (bind (_ispressenable _isreleaseenable _isnormalready _isultimateready _isultimateend) (Utilities|Struct|BreakFSkillReleaseLock _skill_releasable))
  (if (Math|Boolean|ANDBoolean _ispressenable _isultimateready _isultimateend)
    (bind _structout (Utilities|Struct|SetmembersinFSkillReleaseLock (Variables|Default|GetSkill%20Releasable) false))
    (if (Networking|IsServer)
      _
      (else
        (CallFunction|SetServerSkillReleasable _structout)))
    (return true)
    (else
      (return false))))

(fn CheckUltimateRelease
  (bind _skill_releasable (Variables|Default|GetSkill%20Releasable))
  (bind (_ispressenable _isreleaseenable _isnormalready _isultimateready _isultimateend) (Utilities|Struct|BreakFSkillReleaseLock _skill_releasable))
  (if (Math|Boolean|ANDBoolean _isreleaseenable _isultimateready _isultimateend)
    (bind _structout (Utilities|Struct|SetmembersinFSkillReleaseLock (Variables|Default|GetSkill%20Releasable) false false))
    (if (Networking|IsServer)
      _
      (else
        (CallFunction|SetServerSkillReleasable _structout)))
    (return true)
    (else
      (return false))))