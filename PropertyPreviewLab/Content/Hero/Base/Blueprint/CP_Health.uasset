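; CP_Health is a replicated health component that tracks damage, death and regeneration for its owning actor.
; It binds to the owner's damage event, ignores self-inflicted hits, and at zero health calls HeroDie on BP_HeroBase owners or destroys other actors.
; A looping one-second timer restores a fraction of default health once the owner has rested undamaged long enough.
; ShowDamage adds a randomly offset floating damage widget but is not called here.
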(event Custom|Restore
  (if (not (Variables|Default|GetisDead))
    (bind _output_get (Variables|Default|SetRestedTime (Math|Float|Clamp(Float) (+ (Variables|Default|GetRestedTime) 1.0) 0.0 (Variables|Default|GetMaxRestTime))))
    (if (>= _output_get (Variables|Default|GetMaxRestTime))
      (Variables|Default|SetCurrentHealth (Math|Conversions|ToFloat(Integer) (Math|Float|Ceil (Math|Float|Clamp(Float) (+ (Variables|Default|GetCurrentHealth) (Variables|Default|GetRestoreValue)) 0.0 (Variables|Default|GetDefaultHealth)))))
      (Variables|Default|SetHealthPercent (/ (Variables|Default|GetCurrentHealth) (Variables|Default|GetDefaultHealth))))
    (else
      (Utilities|Time|InvalidateTimerHandle (Variables|Default|GetRestoreTimer)))))

(event Custom|ResetRestedTime
  (Variables|Default|SetRestedTime 0.0))

(event Custom|OnDamage
  (params (DamagedActor :type Actor%20Object%20Reference) (Damage :type Float%20%28single-precision%29) (DamageType :type Damage%20Type%20Object%20Reference) (InstigatedBy :type Controller%20Object%20Reference) (DamageCauser :type Actor%20Object%20Reference))
  (bind _returnvalue (Components|GetOwner))
  (bind _returnvalue_2 (Components|GetOwner))
  (if (Math|Boolean|ANDBoolean (== _returnvalue_2 DamagedActor) (not (Variables|Default|GetisDead)) (!= _returnvalue_2 DamageCauser))
    (Variables|Default|SetRestedTime 0.0)
    (Variables|Default|SetCurrentHealth (- (Variables|Default|GetCurrentHealth) Damage))
    (Variables|Default|SetHealthPercent (/ (Variables|Default|GetCurrentHealth) (Variables|Default|GetDefaultHealth)))
    (if (<= (Variables|Default|GetCurrentHealth) 0.0)
      (Variables|Default|SetisDead true)
      (bind _asbp_hero_base (Utilities|Casting|CastToBP_HeroBase _returnvalue)
        (:then
          (Default|HeroDie _asbp_hero_base))
        (:CastFailed
          (Actor|DestroyActor _returnvalue))))))

(event Custom|ShowDamage
  (params (Damage :type Float%20%28single-precision%29))
  (bind _returnvalue (Math|Random|RandomUnitVector))
  (bind _returnvalue_2 (* _returnvalue 5e+01))
  (bind _returnvalue_3 (Game|AddComponentbyClass (Components|GetOwner) "/Game/UMG/Game/Damage/WCP_Game_Damage.WCP_Game_Damage_C" false))
  (Transformation|SetRelativeLocation _returnvalue_3 (Math|Vector|MakeVector (.x _returnvalue_2) (.y _returnvalue_2) 0.0) false false)
  (Default|SetDamageText _returnvalue_3 Damage))

(event EventBeginPlay
  (bind _defaulthealth (Variables|Default|GetDefaultHealth))
  (Class|ActorComponent|SetIsReplicated true)
  (Variables|Default|SetMaxRestTime 5.0)
  (Variables|Default|SetCurrentHealth _defaulthealth)
  (Variables|Default|SetRestoreValue (/ _defaulthealth 7.7))
  (Variables|Default|SetHealthPercent 1.0)
  (Utilities|FlowControl|Sequence
    (:then_0
      (EventDispatchers|AssignOnTakeAnyDamage (Components|GetOwner) (delegate Custom|OnDamage)))
    (:then_1
      (bind _returnvalue (Utilities|Time|SetTimerbyEvent (delegate Custom|Restore) 1.0 true))
      (Variables|Default|SetRestoreTimer _returnvalue))))

(event EventTick
  (params (DeltaSeconds :type Float%20%28single-precision%29)))