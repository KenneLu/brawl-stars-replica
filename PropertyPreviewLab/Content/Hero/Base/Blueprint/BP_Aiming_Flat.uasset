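; Hero-owned aiming actor that shows a flat skill-aim decal for the local player and provides helpers for releasing skills.
; While aiming, Tick derives distance and team-adjusted yaw from mouse offset to the cached hero screen point, rotates the decal and sends clients' aim to the server.
; Ending aim hides the decal once.
; Release events handle hero rotation, montages, movement-orientation locking and spawning skill actors from the weapon muzzle.
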(event Custom|FlatAimingManager
  (bind _aimingdecal (Variables|Default|GetAimingDecal))
  (bind _aiminginfo (Variables|Default|GetAimingInfo))
  (bind (_isflataiming _islaunchaming _isviewportcentrepointset _viewportcentrepoint _realviewportcentermousepoint _aimdistance) (Utilities|Struct|BreakFAimInfo _aiminginfo))
  ;[1 1 1] FlatAimingManager
  (if (Pawn|IsLocallyControlled (Variables|Default|GetHero))
    (if _isflataiming
      (Utilities|FlowControl|Sequence
        (:then_0
          (CallFunction|UpdateAimDistanceandRotation)
          (if (> (Math|Float|Absolute(Float) _aimdistance) 1.0)
            (Rendering|SetVisibility _aimingdecal true false)
            (Transformation|SetWorldRotation _aimingdecal (Math|Rotator|MakeRotator 1.8e+02 9e+01 (.AimRotationZ (Utilities|Struct|BreakFAimInfo (Variables|Default|GetAimingInfo)))) false false)))
        (:then_1
          (goto _label Reset)))
      (else
        (Utilities|FlowControl|DoOnce false :!label _label
          (:Completed
            (Utilities|Struct|SetmembersinFAimInfo (Variables|Default|GetAimingInfo) 0.0)
            (Rendering|SetVisibility (Variables|Default|GetAimingDecal) false false)))))))

(event Custom|InitAimingScreenPoint
  (bind _hero (Variables|Default|GetHero))
  ;[1 1 1] Init Aiming Screen Point
  (if (and (not (Pawn|IsBotControlled _hero)) (Pawn|IsLocallyControlled _hero))
    (if (.isViewportCentrePointSet (Utilities|Struct|BreakFAimInfo (Variables|Default|GetAimingInfo))) :!label _label
      (Development|PrintString "Init Verport Centre Point Done" true true "(R=0.133879,G=1.000000,B=0.000000,A=1.000000)" 3.0)
      (else
        (CallFunction|InitActorScreenPoint)
        (Utilities|FlowControl|Delay 0.2)
        (goto _label)))))

(event Custom|SetHeroSkillReleaseRotation
  (params (AddModify :type Float%20%28single-precision%29))
  ;[1 1 1] Release Skill Manager
  (Transformation|SetActorRotation (Variables|Default|GetHero) (Math|Rotator|MakeRotator 0.0 0.0 (+ AddModify (.AimRotationZ (Utilities|Struct|BreakFAimInfo (Variables|Default|GetAimingInfo)))))))

(event Custom|ClientPlayMontage
  (params (AnimMontage :type Anim%20Montage%20Object%20Reference) (InPlayRate :type Float%20%28single-precision%29) (StartSectionName :type Name))
  ;[1 1 1] Release Skill Manager
  (Animation|PlayAnimMontage (Variables|Default|GetHero) AnimMontage InPlayRate StartSectionName))

(event Custom|SkillMontageStop
  ;[1 1 1] Release Skill Manager
  (Animation|Montage|MontageStop (Components|SkeletalMesh|GetAnimInstance (Variables|/Script/Engine.Character|GetMesh (Variables|Default|GetHero))) 0.0 0))

(event Custom|ReleaseFlatSkill
  (params (SkillType :type BP%20Skill%20Base%20Class%20Reference))
  (bind _hero (Variables|Default|GetHero))
  (bind _weapon (Variables|/Game/Hero/Base/Blueprint/BP_HeroBase.BP_HeroBase_C|GetWeapon _hero))
  ;[1 1 1] Release Skill Manager
  (Utilities|IsValid _weapon
    (:Is%20Valid
      (Game|SpawnActorfromClass SkillType (Math|Transform|MakeTransform (Transformation|GetSocketLocation (Variables|/Script/Engine.Actor|GetRootComponent _weapon) "Muzzle") (Math|Conversions|RotationFromXVector (Math|Vector|GetForwardVector (Variables|/Script/Engine.Character|GetCapsuleComponent _hero))) "1,1,1") "AlwaysSpawn" (Variables|Default|GetHero) 0))))

(event Custom|UnlockMovementOrientRotation
  ;[1 1 1] Release Skill Manager
  (Variables|/Script/Engine.CharacterMovementComponent|SetbOrientRotationToMovement (Variables|/Script/Engine.Character|GetCharacterMovement (Variables|Default|GetHero)) true))

(event Custom|SetServerAimingInfo
  (params (AimingInfo :type F%20Aim%20Info%20Structure%20%28by%20ref%29))
  ;[1 1 1] FlatAimingManager
  (Variables|Default|SetAimingInfo AimingInfo))

(event Custom|LockMovementOrientRotation
  ;[1 1 1] Release Skill Manager
  (Variables|/Script/Engine.CharacterMovementComponent|SetbOrientRotationToMovement (Variables|/Script/Engine.Character|GetCharacterMovement (Variables|Default|GetHero)) false))

(event EventBeginPlay
  (Utilities|Casting|CastToPC_GameBase (Game|GetPlayerController 0))
  (bind _asbp_hero_base (Utilities|Casting|CastToBP_HeroBase (Components|GetOwner)))
  (Variables|Default|SetHero _asbp_hero_base)
  (Utilities|FlowControl|Delay 0.2)
  (CallFunction|InitAimingScreenPoint))

(event EventTick
  (params (DeltaSeconds :type Float%20%28single-precision%29))
  (Utilities|IsValid (Variables|Default|GetHero)
    (:Is%20Valid
      (CallFunction|FlatAimingManager))))

(fn ConstructionScript
  (bind _aimingdecal (Variables|Default|GetAimingDecal))
  (Rendering|Components|Decal|SetDecalMaterial _aimingdecal "/Game/Hero/Base/Asset/M_Decal_FlatAim_Sector.M_Decal_FlatAim_Sector")
  (Transformation|SetWorldRotation _aimingdecal "90.000000,35.264389,-144.735718" false false)
  (Transformation|SetWorldScale3D _aimingdecal "1.500000,1.500000,1.500000")
  (Rendering|SetVisibility _aimingdecal false false))

(fn UpdateAimDistanceandRotation
  (bind _aiminginfo (Variables|Default|GetAimingInfo))
  (bind _realviewportcentermousepoint (Utilities|Struct|BreakFAimInfo _aiminginfo))
  (bind _returnvalue (Class|WidgetLayoutLibrary|GetMousePositiononViewport))
  (if (Math|Vector|NotEqual(Vector) _realviewportcentermousepoint _returnvalue 0.0001)
    (LocalVariables|SetNewAimDistance (* 2.0 (Math|Vector2D|Vector2DLength (- _realviewportcentermousepoint _returnvalue))))
    (bind _output_get (LocalVariables|SetNewAimRotationZ (Class|KismetMathLibrary|DegAtan2 (* (.X (Math|Vector2D|BreakVector2D (- _realviewportcentermousepoint _returnvalue))) -1.0) (.Y (Math|Vector2D|BreakVector2D (- _realviewportcentermousepoint _returnvalue))))))
    (bind _aspc_game_base (Utilities|Casting|CastToPC_GameBase (Game|GetPlayerController 0))
      (:then
        (if (Utilities|Enum|Equal(Enum) (Variables|/Game/Map/Base/PC_GameBase.PC_GameBase_C|GetTeamType _aspc_game_base) "NewEnumerator1")
          (LocalVariables|SetNewAimRotationZ (+ _output_get 1.8e+02))))
      (:CastFailed
        _))
    (bind _structout (Utilities|Struct|SetmembersinFAimInfo (Variables|Default|GetAimingInfo) (LocalVariables|GetNewAimDistance) (LocalVariables|GetNewAimRotationZ)))
    (Networking|SwitchHasAuthority
      (:Remote
        (CallFunction|SetServerAimingInfo _structout)))))

(fn InitActorScreenPoint
  (bind (_getactorscreenpoint _getactorscreenmousepoint _done) (Default|GetActorScreenPoint (Variables|Default|GetCP_GetViewportCenter)))
  (if _done
    (Utilities|Struct|SetmembersinFAimInfo (Variables|Default|GetAimingInfo) true _getactorscreenpoint _getactorscreenmousepoint)))

(fn CenterMousePosition
  (bind _aiminginfo (Variables|Default|GetAimingInfo))
  (bind _viewportcentrepoint (Utilities|Struct|BreakFAimInfo _aiminginfo))
  (bind (_x _y) (Math|Vector2D|BreakVector2D _viewportcentrepoint))
  (if (not (Pawn|IsBotControlled (Variables|/Script/Engine.Actor|GetInstigator (Components|GetOwner))))
    (Class|PlayerController|SetMouseLocation (Game|GetPlayerController 0) (Math|Float|Truncate _x) (Math|Float|Truncate _y))))