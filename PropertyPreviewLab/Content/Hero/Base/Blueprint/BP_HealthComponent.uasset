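; Replicated health component for an actor, under the hero base, that tracks current health and announces changes.
; On BeginPlay it enables replication and initializes current and old health from the default value.
; The CurrentHealth RepNotify computes damage against OldHealth and calls OnHealthChanged with damage and current health.
; OldHealth is not updated after BeginPlay here, so that damage is measured from starting health.
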(event EventBeginPlay
  (Class|ActorComponent|SetIsReplicated true)
  (bind _output_get (Variables|Default|SetCurrentHealth (Variables|Default|GetDefaultHealth)))
  (Variables|Default|SetOldHealth _output_get)
  (Utilities|IsValid (Components|GetOwner)))

(event EventTick
  (params (DeltaSeconds :type Float%20%28single-precision%29)))

(fn OnRepCurrentHealth
  (bind _output_get (LocalVariables|SetDamage (- (Variables|Default|GetOldHealth) (Variables|Default|GetCurrentHealth))))
  (Default|CallOnHealthChanged _output_get (Variables|Default|GetCurrentHealth)))