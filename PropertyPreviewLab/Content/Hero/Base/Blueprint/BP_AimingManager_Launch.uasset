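; Aiming manager for a hero's launch skill, previewing the launch arc and then moving the hero along it.
; While the local player aims, it smooths the launch distance, predicts a projectile path, and draws it with spline meshes and a landing decal.
; Clients copy distance and path to the server through setter events.
; On release, after a short delay for that update, a distance-scaled timeline steps the capsule through path points until landing or completion.
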(event Custom|SetServerLaunchPath
  (params (LaunchPath :type F%20Launch%20Path%20Structure))
  ;[1 1 1] LaunchAimingManager
  (Variables|Default|SetLaunchPath LaunchPath))

(event Custom|SetServerLaunchDistance
  (params (LaunchDistance :type F%20Launch%20Distance%20Structure))
  ;[1 1 1] LaunchAimingManager
  (Variables|Default|SetLaunchDistance LaunchDistance))

(event Custom|LaunchAimManager
  (bind _aiminginfo (Variables|Default|GetAimingInfo))
  (bind _launchpath (Variables|Default|GetLaunchPath))
  (bind _launchpathcomponents (Utilities|Struct|BreakFLaunchPath _launchpath))
  (bind (_isflataiming _islaunchaming _isviewportcentrepointset _viewportcentrepoint _realviewportcentermousepoint _aimdistance) (Utilities|Struct|BreakFAimInfo _aiminginfo))
  ;[1 1 1] LaunchAimingManager
  (if (Pawn|IsLocallyControlled (Variables|Default|GetHero))
    (if _islaunchaming
      (Utilities|FlowControl|Sequence
        (:then_0
          (CallFunction|UpdateAimDistanceandRotation)
          (if (!= _aimdistance 0.0)
            (CallFunction|UpdateLaunchAimInfo)
            (CallFunction|ShowLaunchAim)))
        (:then_1
          (goto _label Reset)))
      (else
        (Utilities|FlowControl|DoOnce true :!label _label
          (:Completed
            (Rendering|SetVisibility (Variables|Default|GetAimingDecal) false false)
            (Utilities|Struct|SetmembersinFAimInfo (Variables|Default|GetAimingInfo) 0.0)
            (Utilities|Struct|SetmembersinFLaunchDistance (Variables|Default|GetLaunchDistance) 0.0)
            (Components|DestroyComponent _launchpathcomponents)
            (Utilities|Array|Clear _launchpathcomponents)
            (Networking|SwitchHasAuthority
              (:Remote
                (CallFunction|SetServerLaunchPath _launchpath)))))))))

(event Custom|ReleaseLaunchSkill
  (bind _launchpath (Variables|Default|GetLaunchPath))
  (bind _launchdistance (Variables|Default|GetLaunchDistance))
  (bind _hero (Variables|Default|GetHero))
  (bind _launchpathpositions (Utilities|Struct|BreakFLaunchPath _launchpath))
  (bind (_aimdistanceold _launchdistance_2 _aimdistancemax) (Utilities|Struct|BreakFLaunchDistance _launchdistance))
  ;[1 1 1] Release Launch Skill Manager
  ;;[1 1 1] Wait Set Server Launch Path
  (Utilities|FlowControl|Delay 0.1)
  (Components|Timeline|SetPlayRate (Variables|Default|GetLaunchTimeline) (/ _aimdistancemax (Math|Float|Clamp(Float) _aimdistanceold 0.0 _aimdistancemax)))
  (bind _timeline (Timeline|LaunchTimeline PlayFromStart)
    (:Update
      (Transformation|SetWorldLocation (Variables|/Script/Engine.Character|GetCapsuleComponent _hero) (Utilities|Array|Get(acopy) _launchpathpositions (Math|Float|Truncate (Math|Float|Lerp 0.0 (Math|Conversions|ToFloat(Integer) (Utilities|Array|Length _launchpathpositions)) _timeline))) false false)
      (if (and (not (AI|Components|NavMovement|IsFalling (Variables|/Script/Engine.Character|GetCharacterMovement _hero))) (> _timeline 0.2))
        (Audio|Components|Audio|Stop (Variables|Default|GetLaunchTimeline))
        (Default|CallLaunchEnd :!label _label)))
    (:Finished
      (goto _label))))

(event EventBeginPlay)

(event Collision|EventActorBeginOverlap
  (params (OtherActor :type Actor%20Object%20Reference)))

(event EventTick
  (params (DeltaSeconds :type Float%20%28single-precision%29))
  (Utilities|IsValid (Variables|Default|GetHero)
    (:Is%20Valid
      (CallFunction|LaunchAimManager))))

(fn ConstructionScript
  (bind _aimingdecal (Variables|Default|GetAimingDecal))
  (Rendering|Components|Decal|SetDecalMaterial _aimingdecal "/Game/Hero/Base/Property/M_Decal_LaunchAim_White.M_Decal_LaunchAim_White")
  (Transformation|SetWorldRotation _aimingdecal "90.000000,0.000000,0.000000" false false)
  (Transformation|SetWorldScale3D _aimingdecal "1.000000,1.000000,1.000000")
  (Rendering|SetVisibility _aimingdecal false false))

(fn ShowLaunchAim
  (bind _launchpath (Variables|Default|GetLaunchPath))
  (bind _launchspline (Variables|Default|GetLaunchSpline))
  (bind _launchpath_2 (Variables|Default|GetLaunchPath))
  (bind _launchpathpositions (Utilities|Struct|BreakFLaunchPath _launchpath_2))
  (bind _launchpathcomponents (Utilities|Struct|BreakFLaunchPath _launchpath))
  (bind _returnvalue (Transformation|GetWorldRotation _launchspline))
  (Rendering|SetVisibility (Variables|Default|GetAimingDecal) true false)
  (Transformation|SetWorldRotation _launchspline (Math|Rotator|MakeRotator (.roll _returnvalue) (.pitch _returnvalue) (.AimRotationZ (Utilities|Struct|BreakFAimInfo (Variables|Default|GetAimingInfo)))) false false)
  (Components|DestroyComponent _launchpathcomponents)
  (Utilities|Array|Clear _launchpathcomponents)
  (Spline|ClearSplinePoints (Variables|Default|GetLaunchSpline) true)
  (bind _returnvalue_2 (CallFunction|GetLaunchVelocity))
  (bind (_outhit _outpathpositions _outlasttracedestination) (Class|GameplayStatics|BlueprintPredictProjectilePathbyObjectType (Transformation|GetSocketLocation (Variables|/Script/Engine.Character|GetMesh (Variables|Default|GetHero)) "LaunchPoint") _returnvalue_2 true 1e+01 (Utilities|Array|MakeArray "ObjectTypeQuery1") false 0 "None" 0.0 1e+02 12.0))
  (Utilities|Struct|SetmembersinFLaunchPath (Variables|Default|GetLaunchPath) _outpathpositions)
  (Transformation|SetWorldLocation (Variables|Default|GetAimingDecal) _outlasttracedestination false false)
  (for (_array_element _array_index) _launchpathpositions
    (Spline|AddSplinePointatIndex (Variables|Default|GetLaunchSpline) _array_element _array_index "Local" true))
  (Spline|SetSplinePointType (Variables|Default|GetLaunchSpline) (Utilities|Array|LastIndex _launchpathpositions) "CurveClamped" true)
  (CallFunction|AddLaunchPathComponent 0.05))

(fn UpdateLaunchAimInfo
  (bind _aiminginfo (Variables|Default|GetAimingInfo))
  (bind _launchdistance (Variables|Default|GetLaunchDistance))
  (bind (_aimdistanceold _launchdistance_2 _aimdistancemax) (Utilities|Struct|BreakFLaunchDistance _launchdistance))
  (bind _aimdistance (Utilities|Struct|BreakFAimInfo _aiminginfo))
  (LocalVariables|SetAimDistacnDelta (- _aimdistance _aimdistanceold))
  (bind _structout (Utilities|Struct|SetmembersinFLaunchDistance (Variables|Default|GetLaunchDistance) _aimdistance (Math|Interpolation|FInterpTo _launchdistance_2 (Math|Float|Clamp(Float) (+ _launchdistance_2 (LocalVariables|GetAimDistacnDelta)) 0.0 _aimdistancemax) (Utilities|Time|GetWorldDeltaSeconds) 3.0)))
  (Networking|SwitchHasAuthority
    (:Remote
      (CallFunction|SetServerLaunchDistance _structout))))

(fn GetLaunchVelocity
  (bind _launchspline (Variables|Default|GetLaunchSpline))
  (bind _launchdistance (Variables|Default|GetLaunchDistance))
  (bind (_aimdistanceold _launchdistance_2 _aimdistancemax) (Utilities|Struct|BreakFLaunchDistance _launchdistance))
  (bind _returnvalue (Transformation|GetWorldRotation _launchspline))
  (bind _returnvalue_2 (Math|Vector|GetForwardVector _returnvalue))
  (bind _returnvalue_3 (Math|Vector|GetUpVector _returnvalue))
  (bind _returnvalue_4 (* _returnvalue_3 0.8))
  (bind _returnvalue_5 (+ _returnvalue_2 _returnvalue_4))
  (return (Math|Vector|ClampVectorSize (* (+ _returnvalue_5 (* _returnvalue_5 _launchdistance_2)) 1e+01) 0.0 _aimdistancemax)))

(fn AddLaunchPathComponent
  (params (InputPin :type Float%20%28single-precision%29))
  (bind _launchpath (Variables|Default|GetLaunchPath))
  (bind _launchpathpositions (Utilities|Struct|BreakFLaunchPath _launchpath))
  (LocalVariables|SetLaunchPathScale InputPin)
  (for _index (range 0 (- (Spline|GetNumberOfSplinePoints (Variables|Default|GetLaunchSpline)) 3))
    (LocalVariables|SetIndex _index)
    (bind _returnvalue (AddComponent|AddSplineMeshComponent true))
    (SplineMesh|SetStartScale _returnvalue (Math|Vector2D|MakeVector2D (LocalVariables|GetLaunchPathScale) (LocalVariables|GetLaunchPathScale)) true :!class /Script/Engine.SplineMeshComponent)
    (SplineMesh|SetEndScale _returnvalue (Math|Vector2D|MakeVector2D (LocalVariables|GetLaunchPathScale) (LocalVariables|GetLaunchPathScale)) true :!class /Script/Engine.SplineMeshComponent)
    (Utilities|Array|Add (.LaunchPathComponents (Utilities|Struct|BreakFLaunchPath (Variables|Default|GetLaunchPath))) _returnvalue)
    (SplineMesh|SetStartandEnd _returnvalue (Utilities|Array|Get(acopy) _launchpathpositions _index) (Spline|GetTangentatSplinePoint (Variables|Default|GetLaunchSpline) _index "Local") (Utilities|Array|Get(acopy) _launchpathpositions (+ (LocalVariables|GetIndex) 1)) (Spline|GetTangentatSplinePoint (Variables|Default|GetLaunchSpline) (+ (LocalVariables|GetIndex) 1) "Local") true :!class /Script/Engine.SplineMeshComponent)))