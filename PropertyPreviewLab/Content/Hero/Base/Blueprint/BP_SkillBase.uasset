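; Base actor for hero skills that fires a fan of bullets when spawned, then destroys itself.
; On BeginPlay it scans DT_Skill for rows whose SkillType matches its own class, taking bullet type, amount and release angle from them.
; ReleaseBullet spawns the bullets at the actor's location, stepping yaw from half the sector left of its facing, and passes its own Owner on to each.
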(event EventBeginPlay
  (bind _outrownames (DataTable|GetDataTableRowNames "/Game/Hero/Base/Data/DT_Skill.DT_Skill"))
  (for _array_element _outrownames
    (bind _returnvalue (Utilities|GetDataTableRow "/Game/Hero/Base/Data/DT_Skill.DT_Skill" _array_element)
      (:then
        (if (== (.SkillType (Utilities|Struct|BreakFSkillAttribute _returnvalue)) (Utilities|GetClass self))
          (CallFunction|ReleaseBullet (.BulletType (Utilities|Struct|BreakFSkillAttribute _returnvalue)) (.BulletAmount (Utilities|Struct|BreakFSkillAttribute _returnvalue)) (.RleaseAngle (Utilities|Struct|BreakFSkillAttribute _returnvalue))))))))

(event Collision|EventActorBeginOverlap
  (params (OtherActor :type Actor%20Object%20Reference)))

(event EventTick
  (params (DeltaSeconds :type Float%20%28single-precision%29)))

(fn ConstructionScript)

(fn ReleaseBullet
  (params (BulletType :type BP%20Bullet%20Base%20Class%20Reference) (BulletCount :type Integer) (SectorAngle :type Float%20%28single-precision%29))
  (bind _self self)
  (LocalVariables|SetSectorAngleSplit (/ SectorAngle (Math|Conversions|ToFloat(Integer) BulletCount)))
  (LocalVariables|SetRotation (Transformation|GetActorRotation _self))
  (LocalVariables|SetLocation (Transformation|GetActorLocation _self))
  (LocalVariables|SetRotation (Math|Rotator|MakeRotator (.Roll (Math|Rotator|BreakRotator (LocalVariables|GetRotation))) (.Pitch (Math|Rotator|BreakRotator (LocalVariables|GetRotation))) (- (.Yaw (Math|Rotator|BreakRotator (LocalVariables|GetRotation))) (/ SectorAngle 2.0))))
  (for _index (range 1 BulletCount)
    (Game|SpawnActorfromClass BulletType (Math|Transform|MakeTransform (LocalVariables|GetLocation) (LocalVariables|GetRotation) "1,1,1") "AlwaysSpawn" (Components|GetOwner) 0)
    (LocalVariables|SetRotation (Math|Rotator|MakeRotator (.Roll (Math|Rotator|BreakRotator (LocalVariables|GetRotation))) (.Pitch (Math|Rotator|BreakRotator (LocalVariables|GetRotation))) (+ (.Yaw (Math|Rotator|BreakRotator (LocalVariables|GetRotation))) (LocalVariables|GetSectorAngleSplit)))))
  (Actor|DestroyActor))