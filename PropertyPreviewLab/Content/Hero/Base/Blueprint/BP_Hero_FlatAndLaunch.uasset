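; Base hero Blueprint for heroes with a flat-aimed normal skill and a launch-aimed ultimate, equipping both aiming managers on BeginPlay.
; Activating a skill enables its aiming and centers the mouse, while releasing disables aiming and fires the skill.
; The normal skill rotates the hero, locks orientation and plays a montage, whose notify releases the skill and blend-out unlocks it.
; The ultimate's launch event is an empty stub.
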(event Custom|NormalFlatSkill
  (bind _heroskills (Variables|Default|GetHeroSkills))
  (bind _aimingmanager (Variables|Default|GetAimingManager))
  (bind _aimingmanager_2 (Variables|Default|GetAimingManager))
  (bind _flataimingmanager (Utilities|Struct|BreakFAimingManager _aimingmanager))
  (bind _flataimingmanager_2 (Utilities|Struct|BreakFAimingManager _aimingmanager_2))
  (bind (_herotype _normalreleaseoffset _normalmontage _normalmontagesection _normalskilltype) (Utilities|Struct|BreakFHeroSkill _heroskills))
  ;[1 1 1] Normal Flat Skill
  (Default|SetHeroSkillReleaseRotation _flataimingmanager_2 _normalreleaseoffset)
  (Default|LockMovementOrientRotation _flataimingmanager_2)
  (Default|ClientPlayMontage _flataimingmanager_2 _normalmontage 1.0 _normalmontagesection)
  (Animation|Montage|PlayMontage (Variables|Character|GetMesh) _normalmontage 1.0 0.0 _normalmontagesection
    (:OnBlendOut
      (Default|UnlockMovementOrientRotation _flataimingmanager)
      (Default|CallNormalSkillFinished (Variables|Default|GetCP_SkillLock)))
    (:OnNotifyBegin
      (Default|ReleaseFlatSkill _flataimingmanager _normalskilltype))))

(event Custom|UltimateLaunchSkill
  ;[1 1 1] Ultimate Launch Skill
)

(event EventActivateNormalSkill
  (bind _aimingmanager (Variables|Default|GetAimingManager))
  (bind _flataimingmanager (Utilities|Struct|BreakFAimingManager _aimingmanager))
  ;[1 1 1] Normal Skill
  (|CallParentFunction)
  (Utilities|Struct|SetmembersinFAimInfo (Variables|/Game/Hero/Base/Blueprint/BP_Aiming_Flat.BP_Aiming_Flat_C|GetAimingInfo _flataimingmanager) true)
  (Default|CenterMousePosition _flataimingmanager))

(event EventBeginPlay
  ;[1 1 1] Init Aiming Manager
  (|CallParentFunction)
  (CallFunction|EquipFlatAimingManager)
  (CallFunction|EquipLaunchAimingManager))

(event EventReleaseNormalSkill
  ;[1 1 1] Normal Skill
  (|CallParentFunction)
  (Utilities|Struct|SetmembersinFAimInfo (Variables|/Game/Hero/Base/Blueprint/BP_Aiming_Flat.BP_Aiming_Flat_C|GetAimingInfo (.FlatAimingManager (Utilities|Struct|BreakFAimingManager (Variables|Default|GetAimingManager)))) false)
  (CallFunction|NormalFlatSkill))

(event EventReleaseUltimateSkill
  ;[1 1 1] Ultimate Skill
  (|CallParentFunction)
  (Utilities|Struct|SetmembersinFAimInfo (Variables|/Game/Hero/Base/Blueprint/BP_Aiming_Flat.BP_Aiming_Flat_C|GetAimingInfo (.LaunchAimingManager (Utilities|Struct|BreakFAimingManager (Variables|Default|GetAimingManager)))) false)
  (CallFunction|UltimateLaunchSkill))

(event EventActivateUltimateSkill
  (bind _aimingmanager (Variables|Default|GetAimingManager))
  (bind _launchaimingmanager (Utilities|Struct|BreakFAimingManager _aimingmanager))
  ;[1 1 1] Ultimate Skill
  (|CallParentFunction)
  (Utilities|Struct|SetmembersinFAimInfo (Variables|/Game/Hero/Base/Blueprint/BP_Aiming_Flat.BP_Aiming_Flat_C|GetAimingInfo _launchaimingmanager) true)
  (Default|CenterMousePosition _launchaimingmanager))

(fn ConstructionScript
  (|CallParentFunction))