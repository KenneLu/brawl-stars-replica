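; Hero base Blueprint for heroes that use the launch aiming manager for their normal and ultimate skills.
; Activating either skill switches to flat aiming and centers the mouse; releasing turns it off and runs a shared release event.
; That event sets release rotation, locks orient rotation and plays the montage, whose notify releases the flat skill.
; Montage completion unlocks rotation and signals the skill lock component that the skill finished.
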(event Custom|ReleaseSkill
  (params (NormalSkill :type Boolean) (ReleaseRotationOffset :type Float%20%28single-precision%29) (Montage :type Anim%20Montage%20Object%20Reference) (MontageSection :type Name) (SkillType :type BP%20Skill%20Base%20Class%20Reference))
  (bind _aimingmanager (Variables|Default|GetAimingManager))
  (bind _aimingmanager_2 (Variables|Default|GetAimingManager))
  (bind _launchaimingmanager (Utilities|Struct|BreakFAimingManager _aimingmanager_2))
  (bind _launchaimingmanager_2 (Utilities|Struct|BreakFAimingManager _aimingmanager))
  ;[1 1 1] Skill Manager
  (Default|SetHeroSkillReleaseRotation _launchaimingmanager_2 ReleaseRotationOffset)
  (Default|LockMovementOrientRotation _launchaimingmanager_2)
  (Default|ClientPlayMontage _launchaimingmanager_2 Montage 1.0 MontageSection)
  (Animation|Montage|PlayMontage (Variables|Character|GetMesh) Montage 1.0 0.0 MontageSection
    (:OnCompleted
      (Default|UnlockMovementOrientRotation _launchaimingmanager)
      (if NormalSkill
        (Default|CallNormalSkillFinished (Variables|Default|GetCP_SkillLock))
        (else
          (Default|CallUltimateSkillFinished (Variables|Default|GetCP_SkillLock)))))
    (:OnNotifyBegin
      (Default|ReleaseFlatSkill _launchaimingmanager SkillType))))

(event EventBeginPlay
  ;[1 1 1] Init Aiming Manager
  (|CallParentFunction)
  (CallFunction|EquipLaunchAimingManager))

(event EventReleaseUltimateSkill
  (bind _heroskills (Variables|Default|GetHeroSkills))
  (bind (_herotype _normalneedrotating _normalreleaseoffset _normalmontage _normalmontagesection _normalskilltype _ultimateneedrotating _ultimatereleaseoffset _ultimatemontage _ultimatemontagesection _ultimateskilltype) (Utilities|Struct|BreakFHeroSkill _heroskills))
  ;[1 1 1] Skill Manager
  (|CallParentFunction)
  (Utilities|Struct|SetmembersinFAimInfo (Variables|/Game/Hero/Base/Blueprint/BP_Aiming_Flat.BP_Aiming_Flat_C|GetAimingInfo (.LaunchAimingManager (Utilities|Struct|BreakFAimingManager (Variables|Default|GetAimingManager)))) false)
  (CallFunction|ReleaseSkill false _ultimatereleaseoffset _ultimatemontage _ultimatemontagesection _ultimateskilltype))

(event EventActivateNormalSkill
  (bind _aimingmanager (Variables|Default|GetAimingManager))
  (bind _launchaimingmanager (Utilities|Struct|BreakFAimingManager _aimingmanager))
  ;[1 1 1] Skill Manager
  (|CallParentFunction)
  (Utilities|Struct|SetmembersinFAimInfo (Variables|/Game/Hero/Base/Blueprint/BP_Aiming_Flat.BP_Aiming_Flat_C|GetAimingInfo _launchaimingmanager) true)
  (Default|CenterMousePosition _launchaimingmanager))

(event EventReleaseNormalSkill
  (bind _heroskills (Variables|Default|GetHeroSkills))
  (bind (_herotype _normalneedrotating _normalreleaseoffset _normalmontage _normalmontagesection _normalskilltype _ultimateneedrotating _ultimatereleaseoffset _ultimatemontage _ultimatemontagesection _ultimateskilltype) (Utilities|Struct|BreakFHeroSkill _heroskills))
  ;[1 1 1] Skill Manager
  (|CallParentFunction)
  (Utilities|Struct|SetmembersinFAimInfo (Variables|/Game/Hero/Base/Blueprint/BP_Aiming_Flat.BP_Aiming_Flat_C|GetAimingInfo (.LaunchAimingManager (Utilities|Struct|BreakFAimingManager (Variables|Default|GetAimingManager)))) false)
  (CallFunction|ReleaseSkill false _normalreleaseoffset _normalmontage _normalmontagesection _normalskilltype))

(event EventActivateUltimateSkill
  (bind _aimingmanager (Variables|Default|GetAimingManager))
  (bind _launchaimingmanager (Utilities|Struct|BreakFAimingManager _aimingmanager))
  ;[1 1 1] Skill Manager
  (|CallParentFunction)
  (Utilities|Struct|SetmembersinFAimInfo (Variables|/Game/Hero/Base/Blueprint/BP_Aiming_Flat.BP_Aiming_Flat_C|GetAimingInfo _launchaimingmanager) true)
  (Default|CenterMousePosition _launchaimingmanager))

(fn ConstructionScript
  (|CallParentFunction))