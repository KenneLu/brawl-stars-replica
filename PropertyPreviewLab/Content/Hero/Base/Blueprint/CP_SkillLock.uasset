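; Hero skill-lock component that decides when normal and ultimate skills can be pressed, activated and released.
; A looping timer refills normal skill charges, pausing when full or while either skill runs; ultimate energy gains a point per recharge event.
; Tick updates readiness in a shared status struct, which Check functions test and update and skill-finished events unlock.
; Non-server instances push status changes and spent normal charges through server-sync events.
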(event Custom|SetServerSkillReleasable
  (params (SkillReleasable :type F%20Skill%20Status%20Structure))
  ;[1 1 1] Net Sync
  (Variables|Default|SetSkillStatus SkillReleasable))

(event Custom|CheckNormalSkillReady
  (bind _skillstatus (Variables|Default|GetSkillStatus))
  ;[1 1 1] Check Normal Skill Ready
  (if (>= (Variables|Default|GetNormalSkillCurrent) 1.0)
    (Utilities|Struct|SetmembersinFSkillStatus _skillstatus true)
    (else
      (Utilities|Struct|SetmembersinFSkillStatus _skillstatus false))))

(event Custom|ResetUltimateEnergyCurrent
  ;[1 1 1] Net Sync
  (Variables|Default|SetUltimateEnergyCurrent 0.0))

(event Custom|NormalBulletRechage
  ;[1 1 1] Init
  (Variables|Default|SetNormalSkillCurrent (Math|Float|ClampAngle (+ (Variables|Default|GetNormalSkillCurrent) (/ 0.1 (Variables|Default|GetNormalSkillRechageTime))) 0.0 (Variables|Default|GetNormalSkillMax))))

(event Custom|RechageNormalSkill
  (bind _skillstatus (Variables|Default|GetSkillStatus))
  (bind (_isskillpressenable _isskillreleaseenable _isnormalready _isnormalactivated _isnormalend _isultimateready _isultimateactivated _isultimateend) (Utilities|Struct|BreakFSkillStatus _skillstatus))
  ;[1 1 1] Rechage Normal Skill
  (if (Math|Boolean|ANDBoolean (!= (Variables|Default|GetNormalSkillCurrent) (Variables|Default|GetNormalSkillMax)) _isnormalend _isultimateend)
    (if (Class|KismetSystemLibrary|IsTimerPausedHandle (Variables|Default|GetNormalSkillRechageTimer))
      (Utilities|Time|UnpauseTimerbyHandle (Variables|Default|GetNormalSkillRechageTimer)))
    (elif (not (Class|KismetSystemLibrary|IsTimerPausedHandle (Variables|Default|GetNormalSkillRechageTimer)))
      (Utilities|Time|PauseTimerbyHandle (Variables|Default|GetNormalSkillRechageTimer)))))

(event Custom|ResetUltimateLock
  ;[1 1 1] Init
  (bind _structout (Utilities|Struct|SetmembersinFSkillStatus (Variables|Default|GetSkillStatus) true true))
  (if (not (Networking|IsServer))
    (CallFunction|SetServerSkillReleasable _structout)))

(event Custom|SetServerSkillAmountCurrent
  (params (SkillAmountCurrent :type Float%20%28single-precision%29))
  ;[1 1 1] Net Sync
  (Variables|Default|SetNormalSkillCurrent SkillAmountCurrent))

(event Custom|CheckUltimateSkillReady
  (bind _skillstatus (Variables|Default|GetSkillStatus))
  ;[1 1 1] Check Ultimate Skill Ready
  (if (>= (Variables|Default|GetUltimateEnergyCurrent) (Variables|Default|GetUltimateEnergyDefault))
    (Utilities|Struct|SetmembersinFSkillStatus _skillstatus true)
    (else
      (Utilities|Struct|SetmembersinFSkillStatus _skillstatus false))))

(event Custom|ResetNormalLock
  ;[1 1 1] Init
  (bind _structout (Utilities|Struct|SetmembersinFSkillStatus (Variables|Default|GetSkillStatus) true))
  (if (not (Networking|IsServer))
    (CallFunction|SetServerSkillReleasable _structout)))

(event Custom|RechageUltimateSkill
  ;[1 1 1] Rechage Ultimate Skill
  (if (!= (Variables|Default|GetUltimateEnergyCurrent) (Variables|Default|GetUltimateEnergyDefault))
    (Variables|Default|SetUltimateEnergyCurrent (Math|Float|Clamp(Float) (+ (Variables|Default|GetUltimateEnergyCurrent) 1.0) 0.0 (Variables|Default|GetUltimateEnergyDefault)))))

(event Custom|BindUltimateRechage
  ;[1 1 1] Init
  (CallFunction|RechageUltimateSkill))

(event EventBeginPlay
  ;[1 1 1] Init
  (Variables|Default|SetNormalSkillCurrent (Variables|Default|GetNormalSkillMax))
  (bind _returnvalue (Utilities|Time|SetTimerbyEvent (delegate Custom|NormalBulletRechage) 0.1 true))
  (Variables|Default|SetNormalSkillRechageTimer _returnvalue)
  (EventDispatchers|BindEventtoNormalSkillFinished (delegate Custom|ResetNormalLock))
  (EventDispatchers|BindEventtoUltimateSkillFinished (delegate Custom|ResetUltimateLock))
  (EventDispatchers|BindEventtoUltimateRechage (delegate Custom|BindUltimateRechage)))

(event EventTick
  (params (DeltaSeconds :type Float%20%28single-precision%29))
  ;[1 1 1] Tick
  (CallFunction|CheckNormalSkillReady)
  (CallFunction|RechageNormalSkill)
  (CallFunction|CheckUltimateSkillReady))

(fn CheckActivatableNormal
  (bind _skillstatus (Variables|Default|GetSkillStatus))
  (bind (_isskillpressenable _isskillreleaseenable _isnormalready _isnormalactivated _isnormalend _isultimateready _isultimateactivated _isultimateend) (Utilities|Struct|BreakFSkillStatus _skillstatus))
  (if (Math|Boolean|ANDBoolean _isskillpressenable _isnormalready _isnormalend _isultimateend)
    (bind _structout (Utilities|Struct|SetmembersinFSkillStatus (Variables|Default|GetSkillStatus) true))
    (if (Networking|IsServer)
      _
      (else
        (CallFunction|SetServerSkillReleasable _structout)))
    (return true)
    (else
      (return false))))

(fn CheckActivatableUltimate
  (bind _skillstatus (Variables|Default|GetSkillStatus))
  (bind (_isskillpressenable _isskillreleaseenable _isnormalready _isnormalactivated _isnormalend _isultimateready _isultimateactivated _isultimateend) (Utilities|Struct|BreakFSkillStatus _skillstatus))
  (if (Math|Boolean|ANDBoolean _isskillpressenable _isultimateready _isultimateend)
    (bind _structout (Utilities|Struct|SetmembersinFSkillStatus (Variables|Default|GetSkillStatus) false true))
    (if (Networking|IsServer)
      _
      (else
        (CallFunction|SetServerSkillReleasable _structout)))
    (return true)
    (else
      (return false))))

(fn CheckReleaseableNoremal
  (bind _skillstatus (Variables|Default|GetSkillStatus))
  (bind _skillstatus_2 (Variables|Default|GetSkillStatus))
  (bind (_isskillpressenable _isskillreleaseenable _isnormalready _isnormalactivated _isnormalend _isultimateready _isultimateactivated _isultimateend) (Utilities|Struct|BreakFSkillStatus _skillstatus))
  (if (Math|Boolean|ANDBoolean _isskillreleaseenable _isnormalready _isnormalactivated _isnormalend _isultimateend)
    (Variables|Default|SetNormalSkillCurrent (- (Variables|Default|GetNormalSkillCurrent) 1.0))
    (Utilities|Struct|SetmembersinFSkillStatus _skillstatus_2 false false)
    (if (Networking|IsServer)
      _
      (else
        (CallFunction|SetServerSkillReleasable _skillstatus_2)
        (CallFunction|SetServerSkillAmountCurrent (Variables|Default|GetNormalSkillCurrent))))
    (return true)
    (else
      (return false))))

(fn CheckReleaseableUltimate
  (bind _skillstatus (Variables|Default|GetSkillStatus))
  (bind (_isskillpressenable _isskillreleaseenable _isnormalready _isnormalactivated _isnormalend _isultimateready _isultimateactivated _isultimateend) (Utilities|Struct|BreakFSkillStatus _skillstatus))
  (if (Math|Boolean|ANDBoolean _isskillreleaseenable _isultimateready _isultimateactivated _isultimateend)
    (bind _structout (Utilities|Struct|SetmembersinFSkillStatus (Variables|Default|GetSkillStatus) false false false))
    (if (Networking|IsServer)
      _
      (else
        (CallFunction|SetServerSkillReleasable _structout)))
    (return true)
    (else
      (return false))))

(fn CheckPhysicsBottonNoremal
  (params (Press :type Boolean))
  (bind _skillstatus (Variables|Default|GetSkillStatus))
  (bind (_isskillpressenable _isskillreleaseenable _isnormalready _isnormalactivated _isnormalend _isultimateready _isultimateactivated _isultimateend) (Utilities|Struct|BreakFSkillStatus _skillstatus))
  (if Press
    (if (Variables|Default|GetNormalButtonReleased)
      (if (and _isnormalend _isultimateend)
        (Variables|Default|SetNormalButtonPressed true)
        (Variables|Default|SetNormalButtonReleased false)
        (return true)
        (else
          (return false))))
    (elif (Variables|Default|GetNormalButtonPressed)
      (Variables|Default|SetNormalButtonPressed false)
      (Variables|Default|SetNormalButtonReleased true)
      (return true)
      (else
        (return false)))))

(fn CheckPhysicsBottonUltimate
  (params (Press :type Boolean))
  (if Press
    (if (Variables|Default|GetUltimateButtonReleased)
      (if (.isSkillPressEnable (Utilities|Struct|BreakFSkillStatus (Variables|Default|GetSkillStatus)))
        (Variables|Default|SetUltimateButtonPressed true)
        (Variables|Default|SetUltimateButtonReleased false)
        (return true)
        (else
          (return false))))
    (elif (Variables|Default|GetUltimateButtonPressed)
      (Variables|Default|SetUltimateButtonPressed false)
      (Variables|Default|SetUltimateButtonReleased true)
      (return true)
      (else
        (return false)))))