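; BP_Hero_NitaBear is Nita's bear character, a team-aligned melee fighter with its own health, scale and damage set in the construction script.
; Its show-up event chains sit, stand-up and stretch montages, and both show-up and attack signal when finished.
; A right-hand collider, initially disabled, damages opposing heroes and safe boxes on overlap via CheckTeamate, which also shakes destructible scenery.
; Health restoration is turned off at BeginPlay.
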(event OnComponentBeginOverlap(MeleeCollision)
  (params (OverlappedComponent :type Primitive%20Component%20Object%20Reference) (OtherActor :type Actor%20Object%20Reference) (OtherComp :type Primitive%20Component%20Object%20Reference) (OtherBodyIndex :type Integer) (bFromSweep :type Boolean) (SweepResult :type Hit%20Result%20Structure%20%28by%20ref%29))
  (bind (_returnvalue _hitenemy) (CallFunction|CheckTeamate OtherActor))
  (if _returnvalue
    (Game|Damage|ApplyDamage _hitenemy (Variables|Default|GetAttackDamage) 0 self)))

(event Custom|NitaBearShowUp
  (bind _mesh (Variables|Character|GetMesh))
  (Animation|Montage|PlayMontage _mesh "/Game/Hero/Nita/Animation/NitaBear/AM_NitaBear_Sit.AM_NitaBear_Sit" 1.0 0.0 "Start"
    (:OnBlendOut
      (Animation|Montage|PlayMontage _mesh "/Game/Hero/Nita/Animation/NitaBear/AM_NitaBear_Stand_Up.AM_NitaBear_Stand_Up" 1.0 0.0 "Start"
        (:OnBlendOut
          (Animation|Montage|PlayMontage _mesh "/Game/Hero/Nita/Animation/NitaBear/AM_NitaBear_Stretch.AM_NitaBear_Stretch" 1.0 0.0 "Start"
            (:OnCompleted
              (Default|CallNitaBearShowUpEnd))))))))

(event Custom|Attack
  (Animation|Montage|PlayMontage (Variables|Character|GetMesh) "/Game/Hero/Nita/Animation/NitaBear/AM_NitaBear_Attack.AM_NitaBear_Attack" 1.0 0.0 ""
    (:OnCompleted
      (Default|CallNitaBearAttackEnd))))

(event EventBeginPlay
  (|CallParentFunction)
  (Variables|/Game/Hero/Base/Blueprint/CP_Health.CP_Health_C|SetCanRestore (Variables|Default|GetCP_Health) false))

(event Collision|EventActorBeginOverlap
  (params (OtherActor :type Actor%20Object%20Reference)))

(event EventTick
  (params (DeltaSeconds :type Float%20%28single-precision%29)))

(fn ConstructionScript
  (|CallParentFunction)
  (Transformation|SetWorldScale3D (Variables|Default|GetCapsuleComponent) "2.200000,2.200000,2.200000")
  (Transformation|AttachComponentToComponent (Variables|Default|GetMeleeCollision) (Variables|Character|GetMesh) "RightHand" "KeepRelative" "KeepRelative" "KeepRelative" true)
  (Collision|SetCollisionEnabled (Variables|Default|GetMeleeCollision) "NoCollision")
  (Variables|Default|SetAttackDamage 5.6e+02)
  (bind _output_get (Variables|Default|SetHealth 5.6e+03))
  (Variables|/Game/Hero/Base/Blueprint/CP_Health.CP_Health_C|SetDefaultHealth (Variables|Default|GetCP_Health) _output_get))

(fn CheckTeamate
  (params (OtherActor :type Object%20Object%20Reference))
  (bind _self self)
  (LocalVariables|SetEnemy 0)
  (LocalVariables|SetHitActor 0)
  (bind _asbp_hero_base (Utilities|Casting|CastToBP_HeroBase OtherActor)
    (:then
      (bind _output_get (LocalVariables|SetEnemy _asbp_hero_base))
      (LocalVariables|SetHitActor _output_get)
      (Utilities|IsValid _output_get
        (:Is%20Valid
          (Utilities|IsValid _self
            (:Is%20Valid
              (if (Utilities|Enum|NotEqual(Enum) (Variables|Default|GetTeamType) (Variables|/Game/Hero/Base/Blueprint/BP_HeroBase.BP_HeroBase_C|GetTeamType _output_get))
                (if (!= _self (LocalVariables|GetHitActor))
                  (return true (LocalVariables|GetHitActor)))))))))
    (:CastFailed
      (bind _asbp_safe_box (Utilities|Casting|CastToBP_SafeBox OtherActor)
        (:then
          (LocalVariables|SetHitActor _asbp_safe_box)
          (Utilities|IsValid _asbp_safe_box
            (:Is%20Valid
              (Utilities|IsValid self
                (:Is%20Valid
                  (if (Utilities|Enum|NotEqual(Enum) (Variables|Default|GetTeamType) (Variables|/Game/Map/Game/Heist/BP_SafeBox.BP_SafeBox_C|GetSafeBoxTeamType _asbp_safe_box))
                    (if (!= self (LocalVariables|GetHitActor))
                      (return true (LocalVariables|GetHitActor)))))))))
        (:CastFailed
          (bind _asbp_sence_base (Utilities|Casting|CastToBP_SenceBase OtherActor))
          (bind _asbp_sence_destructible (Utilities|Casting|CastToBP_Sence_Destructible _asbp_sence_base))
          (Default|Shake _asbp_sence_destructible (Transformation|GetActorForwardVector)))))))