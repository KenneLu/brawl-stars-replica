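; Nita's ultimate projectile, which turns into her bear summon when the launch finishes.
; On BeginPlay it caches the owning Nita hero's team and binds to the launch-end callback of her aiming manager.
; When that fires, the server spawns the bear at the projectile's location, copies the team onto the bear's PlayerState and destroys the projectile.
; The construction script disables collision on the Cube component.
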(event Custom|NitaFinishLaunch
  (bind _returnvalue (Components|GetOwner))
  (Networking|SwitchHasAuthority
    (:Authority
      (Utilities|IsValid _returnvalue
        (:Is%20Valid
          (bind _returnvalue_2 (Game|SpawnActorfromClass "/Game/Hero/Nita/Blueprint/BP_Hero_NitaBear.BP_Hero_NitaBear_C" (Math|Transform|MakeTransform (Transformation|GetActorLocation) "0, 0, 0" "1,1,1") "Undefined" _returnvalue 0))
          (Utilities|IsValid _returnvalue_2
            (:Is%20Valid
              (bind _asps_game_base (Utilities|Casting|CastToPS_GameBase (Variables|/Script/Engine.Pawn|GetPlayerState _returnvalue_2)))
              (Variables|/Game/Map/Base/PS_GameBase.PS_GameBase_C|SetTeamType _asps_game_base (Variables|Default|GetTeamType))
              (Actor|DestroyActor))))))))

(event EventBeginPlay
  (bind _asbp_hero_nita (Utilities|Casting|CastToBP_Hero_Nita (Components|GetOwner)))
  (Variables|Default|SetTeamType (Variables|/Game/Hero/Base/Blueprint/BP_HeroBase.BP_HeroBase_C|GetTeamType _asbp_hero_nita))
  (EventDispatchers|BindEventtoLaunchEnd (.LaunchAimingManager (Utilities|Struct|BreakFAimingManager (Variables|/Game/Hero/Base/Blueprint/BP_HeroBase.BP_HeroBase_C|GetAimingManager _asbp_hero_nita))) (delegate Custom|NitaFinishLaunch)))

(fn ConstructionScript
  (|CallParentFunction)
  (Collision|SetCollisionEnabled (Variables|Default|GetCube) "NoCollision"))