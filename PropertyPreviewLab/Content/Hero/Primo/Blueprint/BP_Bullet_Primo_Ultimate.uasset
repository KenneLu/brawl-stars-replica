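; Bullet actor for the hero Primo's ultimate, which knocks back heroes it hits.
; The construction script runs the parent's, then turns off Collision and enables the Sphere for query and physics.
; When the Sphere hits a hero other than the owner, a large impulse pushes that hero away from Collision and along its up vector.
; Any hero hit, owner included, destroys the bullet, while non-hero hits are ignored.
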(event OnComponentHit(Sphere)
  (params (HitComponent :type Primitive%20Component%20Object%20Reference) (OtherActor :type Actor%20Object%20Reference) (OtherComp :type Primitive%20Component%20Object%20Reference) (NormalImpulse :type Vector :default "0, 0, 0") (Hit :type Hit%20Result%20Structure%20%28by%20ref%29))
  (bind _collision (Variables|Default|GetCollision))
  (bind _asbp_hero_base (Utilities|Casting|CastToBP_HeroBase OtherActor))
  (if (!= _asbp_hero_base (Components|GetOwner))
    (Physics|AddImpulse (Variables|/Script/Engine.Character|GetCharacterMovement _asbp_hero_base) (* (+ (Math|Vector|Normalize (- (Transformation|GetActorLocation _asbp_hero_base) (Transformation|GetWorldLocation _collision))) (Math|Vector|Normalize (Math|Vector|GetUpVector _collision))) 5e+04) false))
  (Actor|DestroyActor))

(event EventBeginPlay
  (Variables|Default|SetDestructibal true))

(fn ConstructionScript
  (|CallParentFunction)
  (Collision|SetCollisionEnabled (Variables|Default|GetCollision) "NoCollision")
  (Collision|SetCollisionEnabled (Variables|Default|GetSphere) "QueryAndPhysics"))