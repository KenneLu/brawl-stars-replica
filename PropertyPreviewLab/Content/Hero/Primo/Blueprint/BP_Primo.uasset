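; BP_Primo is the Blueprint for the Primo hero, handling the punch attack bound to the Fire input.
; Pressing Fire calls ContreMousePosition; releasing it sets the fire rotation, turns off orient rotation, flags SkillNormalStart and plays the punch montage.
; Montage completion clears the flag and restores orient rotation, with no handling on the interrupted path.
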(event EventBeginPlay
  (|CallParentFunction) ; This node is disabled and will not be called.\nDrag off pins to build functionality.
)

(event Collision|EventActorBeginOverlap
  (params (OtherActor :type Actor%20Object%20Reference))
  (|CallParentFunction OtherActor) ; This node is disabled and will not be called.\nDrag off pins to build functionality.
)

(event EventTick
  (params (DeltaSeconds :type Float%20%28single-precision%29))
  (|CallParentFunction DeltaSeconds) ; This node is disabled and will not be called.\nDrag off pins to build functionality.
)

(event Input|ActionEvents|InputActionFire
  (params (Key :type Key%20Structure :default "None"))
  (:Pressed
    (CallFunction|ContreMousePosition))
  (:Released
    (CallFunction|SetActorFireRotation)
    (CallFunction|SetOrientRotation false)
    (Variables|Default|SetSkillNormalStart true)
    (Animation|Montage|PlayMontage (Variables|Character|GetMesh) "/Game/Hero/Primo/Animation/AM_Primo_Punch.AM_Primo_Punch"
      (:OnCompleted
        (Variables|Default|SetSkillNormalStart false)
        (CallFunction|SetOrientRotation true)))))

(event Input|ActionEvents|InputActionUltimate
  (params (Key :type Key%20Structure :default "None")))

(fn ConstructionScript
  (|CallParentFunction))