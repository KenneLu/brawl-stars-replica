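; Primo hero Blueprint that implements the character's ultimate, a launch skill followed by a flat skill.
; On launch, the Launch Aiming Manager stops the skill montage, sets release rotation, locks movement orientation and releases the launch.
; A callback bound to launch end releases the flat skill using the ultimate skill type, unlocks orientation and signals the skill lock component that the ultimate has finished.
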(event Custom|PrimoFinishLaunch
  (bind _aimingmanager (Variables|Default|GetAimingManager))
  (bind _launchaimingmanager (Utilities|Struct|BreakFAimingManager _aimingmanager))
  ;[1 1 1] Primo Ultimate Skill
  (Default|ReleaseFlatSkill _launchaimingmanager (.UltimateSkillType (Utilities|Struct|BreakFHeroSkill (Variables|Default|GetHeroSkills))))
  (Default|UnlockMovementOrientRotation _launchaimingmanager)
  (Default|CallUltimateSkillFinished (Variables|Default|GetCP_SkillLock)))

(event EventUltimateLaunchSkill
  (bind _aimingmanager (Variables|Default|GetAimingManager))
  (bind _launchaimingmanager (Utilities|Struct|BreakFAimingManager _aimingmanager))
  ;[1 1 1] Primo Ultimate Skill
  (Default|SkillMontageStop _launchaimingmanager)
  (Default|SetHeroSkillReleaseRotation _launchaimingmanager (.UltimateReleaseOffset (Utilities|Struct|BreakFHeroSkill (Variables|Default|GetHeroSkills))))
  (Default|LockMovementOrientRotation _launchaimingmanager)
  (Default|ReleaseLaunchSkill _launchaimingmanager)
  (EventDispatchers|BindEventtoLaunchEnd (.LaunchAimingManager (Utilities|Struct|BreakFAimingManager (Variables|Default|GetAimingManager))) (delegate Custom|PrimoFinishLaunch)))

(fn ConstructionScript
  (|CallParentFunction))