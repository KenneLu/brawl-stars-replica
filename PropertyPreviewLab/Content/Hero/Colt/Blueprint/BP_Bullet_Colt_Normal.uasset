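; BP_Bullet_Colt_Normal is the normal bullet Blueprint for the hero Colt.
; Its construction script runs the parent's, then sets the Bullet mesh from StaticMeshType and applies separate world scales to the Cube, sized by a collision variable, and to the Bullet.
; BeginPlay and Destroyed are empty, and the particle trail begin and end calls are left disconnected, so they never run.
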(event EventBeginPlay)

(event EventDestroyed)

(fn ConstructionScript
  (|CallParentFunction)
  (Components|StaticMesh|SetStaticMesh (Variables|Default|GetBullet) (Variables|Default|GetStaticMeshType))
  (Transformation|SetWorldScale3D (Variables|Default|GetCube) (Variables|Default|GetCollisionWorldScale))
  (Transformation|SetWorldScale3D (Variables|Default|GetBullet) (Variables|Default|GetBulletWorldScale)))