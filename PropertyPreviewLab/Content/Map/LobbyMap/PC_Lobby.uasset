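; Lobby player controller that shows the local player's selectable hero and handles LAN sessions.
; On BeginPlay it spawns a hero at the BP_ShowHero_Main marker, turned 180 degrees, and switches view to the lobby camera.
; Hero1/Hero2 inputs respawn the hero there, with replication disabled on the server.
; Other inputs create a session and reopen LobbyMap, search for sessions, or join the stored OnlineRoom, printing results.
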(event EventBeginPlay
  ;[1 1 1] 在中间生成自己的角色
  (if (Pawn|IsLocalController)
    (bind _outactors (Actor|GetAllActorsOfClass "/Game/Map/LobbyMap/BP_ShowHero.BP_ShowHero_C"))
    (bind _array_element (Utilities|Array|ForEachLoopwithBreak _outactors :!label _label)
      (:LoopBody
        (if (Utilities|Enum|Equal(Enum) (Utilities|GetDisplayName _array_element) "BP_ShowHero_Main")
          (Utilities|FlowControl|Sequence
            (:then_0
              (bind _output_get (Variables|Default|SetHero%20Transfrom (Math|Transform|MakeTransform (.location (Transformation|GetActorTransform _array_element)) "0,180.000000, 0" (.scale (Transformation|GetActorTransform _array_element)))))
              (bind _returnvalue (Game|SpawnActorfromClass "/Game/Role/Shelly/BluePrint/BP_Shelly.BP_Shelly_C" _output_get "Undefined" 0 0))
              (bind _output_get_2 (Variables|Default|SetHero _returnvalue))
              (if (Networking|IsServer)
                (Networking|SetReplicates _output_get_2 false))
              ;[1 1 1] 使用摄像机视角
              (bind _outactors_2 (Actor|GetAllActorsOfClass "/Game/Map/LobbyMap/BP_LobbyCamera.BP_LobbyCamera_C"))
              (Game|Player|SetViewTargetwithBlend self (Utilities|Array|Get(acopy) _outactors_2) 0.0 "VTBlend_Linear" 0.0 false))
            (:then_1
              (goto _label Break))))))))

(event Input|ActionEvents|InputActionHero1
  (params (Key :type Key%20Structure :default "None"))
  ;[1 1 1] 切换角色
  (:Pressed
    (Utilities|IsValid (Variables|Default|GetHero)
      (:Is%20Valid
        (Actor|DestroyActor (Variables|Default|GetHero)))
      (:Is%20Not%20Valid
        _))
    (bind _returnvalue (Game|SpawnActorfromClass "/Game/Role/Shelly/BluePrint/BP_Shelly.BP_Shelly_C" (Variables|Default|GetHero%20Transfrom) "Undefined" 0 0))
    (bind _output_get (Variables|Default|SetHero _returnvalue))
    (if (Networking|IsServer)
      (Networking|SetReplicates _output_get false))
    (Development|PrintString "Hero1")))

(event Input|ActionEvents|InputActionHero2
  (params (Key :type Key%20Structure :default "None"))
  ;[1 1 1] 切换角色
  (:Pressed
    (Utilities|IsValid (Variables|Default|GetHero)
      (:Is%20Valid
        (Actor|DestroyActor (Variables|Default|GetHero)))
      (:Is%20Not%20Valid
        _))
    (bind _returnvalue (Game|SpawnActorfromClass "/Game/Role/Shelly/BluePrint/BP_Shelly1.BP_Shelly1_C" (Variables|Default|GetHero%20Transfrom) "Undefined" 0 0))
    (bind _output_get (Variables|Default|SetHero _returnvalue))
    (if (Networking|IsServer)
      (Networking|SetReplicates _output_get false))
    (Development|PrintString "Hero2")))

(event Input|ActionEvents|InputActionJoinLobbyClick
  (params (Key :type Key%20Structure :default "None"))
  ;[1 1 1] 加入房间
  (:Pressed
    (Development|PrintString "JoinLobbyClick")
    (|JoinSession (Game|GetPlayerController 0) (Variables|Default|GetOnline%20Room)
      (:OnSuccess
        (Development|PrintString "成功加入大厅"))
      (:OnFailure
        (Development|PrintString "加入大厅失败")))))

(event Input|ActionEvents|InputActionCreateLobbyClick
  (params (Key :type Key%20Structure :default "None"))
  ;[1 1 1] 创建房间
  (:Pressed
    (Development|PrintString "CreateLobyClick")
    (|Session (Game|GetPlayerController 0) 3 true
      (:OnSuccess
        (Development|PrintString "成功创建大厅")
        (Game|OpenLevel(byName) "LobbyMap"))
      (:OnFailure
        (Development|PrintString "创建大厅失败")))))

(event Input|ActionEvents|InputActionFindLobbyClick
  (params (Key :type Key%20Structure :default "None"))
  ;[1 1 1] 搜索房间
  (:Pressed
    (Development|PrintString "FindLobbyClick")
    (bind _results (|FindSessions (Game|GetPlayerController 0) 10 true)
      (:OnSuccess
        (if (> (Utilities|Array|Length _results) 0)
          (Development|PrintString (Utilities|String|Append "找到大厅：" (Class|FindSessionsCallbackProxy|GetServerName (Utilities|Array|Get(acopy) _results))))
          (Variables|Default|SetOnline%20Room (Variables|Default|GetOnline%20Room))
          (else
            (Development|PrintString "没有大厅" :!label _label))))
      (:OnFailure
        (goto _label)))))

(fn ConstructionScript)