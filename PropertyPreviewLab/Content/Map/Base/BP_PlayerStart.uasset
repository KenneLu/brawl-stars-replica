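; BP_PlayerStart is a team-specific spawn point that tracks whether it is available.
; A hero of the same TeamType beginning overlap with its Sphere marks it unavailable, and ending overlap marks it available again, without counting overlapping heroes.
; Tick swaps a half-scale, collision-free marker mesh between Shelly's normal and ultimate bullet meshes to show that state.
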(event OnComponentBeginOverlap(Sphere)
  (params (OverlappedComponent :type Primitive%20Component%20Object%20Reference) (OtherActor :type Actor%20Object%20Reference) (OtherComp :type Primitive%20Component%20Object%20Reference) (OtherBodyIndex :type Integer) (bFromSweep :type Boolean) (SweepResult :type Hit%20Result%20Structure%20%28by%20ref%29))
  (bind _asbp_hero_base (Utilities|Casting|CastToBP_HeroBase OtherActor))
  (if (Utilities|Enum|Equal(Enum) (Variables|/Game/Hero/Base/Blueprint/BP_HeroBase.BP_HeroBase_C|GetTeamType _asbp_hero_base) (Variables|Default|GetTeamType))
    (CallFunction|SetIsAvailable false)))

(event OnComponentEndOverlap(Sphere)
  (params (OverlappedComponent :type Primitive%20Component%20Object%20Reference) (OtherActor :type Actor%20Object%20Reference) (OtherComp :type Primitive%20Component%20Object%20Reference) (OtherBodyIndex :type Integer))
  (bind _asbp_hero_base (Utilities|Casting|CastToBP_HeroBase OtherActor))
  (if (Utilities|Enum|Equal(Enum) (Variables|/Game/Hero/Base/Blueprint/BP_HeroBase.BP_HeroBase_C|GetTeamType _asbp_hero_base) (Variables|Default|GetTeamType))
    (CallFunction|SetIsAvailable true)))

(event Custom|SetIsAvailable
  (params (isAvailable :type Boolean))
  (Variables|Default|SetisAvailable isAvailable))

(event EventBeginPlay
  (bind _staticmesh (Variables|Default|GetStaticMesh))
  (Collision|SetCollisionEnabled _staticmesh "NoCollision")
  (Transformation|SetWorldScale3D _staticmesh "0.500000,0.500000,0.500000"))

(event EventTick
  (params (DeltaSeconds :type Float%20%28single-precision%29))
  (bind _staticmesh (Variables|Default|GetStaticMesh))
  (if (Variables|Default|GetisAvailable)
    (Components|StaticMesh|SetStaticMesh _staticmesh "/Game/Hero/Shelly/Asset/Bullet/SM_Shelly_Bullet_Normal.SM_Shelly_Bullet_Normal")
    (else
      (Components|StaticMesh|SetStaticMesh _staticmesh "/Game/Hero/Shelly/Asset/Bullet/SM_Shelly_Bullet_Ultimate.SM_Shelly_Bullet_Ultimate"))))

(fn ConstructionScript)