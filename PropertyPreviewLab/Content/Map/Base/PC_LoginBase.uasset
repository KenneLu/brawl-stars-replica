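; Base player controller for the login levels, handling hero selection and LAN matchmaking.
; Next/last input cycles heroes from DT_HeroAttribute, respawns exhibition actors at stored points, and saves the choice to BP_SaveGame and the GameInstance.
; StartGame shows the matching widget, then joins a session whose extra settings match type, matching state and level, or hosts one on L_Matching.
; DetectQuitMatching interrupts matching and travels back to the appropriate login level.
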(event Custom|NextHero
  ;[1 1 1] Switch Hero
  (bind _newherotype (CallFunction|SwitchHero true))
  (CallFunction|UpdateExhibitionHero _newherotype))

(event Custom|UpdateHeroType_of_SaveGame_and_Instace
  (params (HeroTypeSaved :type BP%20Hero%20Base%20Class%20Reference))
  (bind _save_game (Variables|Default|GetSave%20Game))
  ;[1 1 1] Switch Hero
  (bind _output_get (Variables|/Game/Map/Base/BP_SaveGame.BP_SaveGame_C|SetHeroTypeSaved _save_game HeroTypeSaved))
  (SaveGame|SaveGametoSlot _save_game (Variables|Default|GetSave%20Game%20Slot%20Name))
  (bind _asbp_game_instance (Utilities|Casting|CastToBP_GameInstance (Game|GetGameInstance)))
  (Variables|/Game/Map/Base/BP_GameInstance.BP_GameInstance_C|SetHeroTypeInstacne _asbp_game_instance _output_get))

(event Custom|CreateMatchingSession
  ;[1 1 1] Start Matching
  (Development|PrintString "Creating Match Session ...")
  (CallFunction|SetSessionExtraInfo "NewEnumerator2" true (Variables|Default|GetGameLevelName))
  (|DestroySession (Game|GetPlayerController 0)
    (:OnSuccess
      _)
    (:OnFailure
      _))
  (|AdvancedSession (Variables|Default|GetSessionExtraSettings) (Game|GetPlayerController 0) 6 0 true true false true true false false false true
    (:OnSuccess
      (Development|PrintString "Matching Created" true true "(R=0.000000,G=1.000000,B=0.071725,A=1.000000)")
      (Game|OpenLevel(byName) "L_Matching" true "Listen"))
    (:OnFailure
      (Development|PrintString "Create Matching Sesion Faild" true true "(R=1.000000,G=0.000000,B=0.008162,A=1.000000)" 1e+01))))

(event Custom|UpdateExhibitionHero
  (params (NewHeroType :type BP%20Hero%20Base%20Class%20Reference))
  ;[1 1 1] Switch Hero
  (if (Utilities|IsValidClass NewHeroType)
    (Variables|Default|SetCurrent%20Hero%20Type NewHeroType)
    (for (_array_element _array_index) (Variables|Default|GetExhibitionPointTransfrom)
      (Utilities|IsValid (Utilities|Array|Get(acopy) (Variables|Default|GetExhibitionHero) _array_index)
        (:Is%20Valid
          (Actor|DestroyActor (Utilities|Array|Get(acopy) (Variables|Default|GetExhibitionHero) _array_index)))
        (:Is%20Not%20Valid
          _))
      (bind _returnvalue (Game|SpawnActorfromClass (Variables|Default|GetCurrent%20Hero%20Type) _array_element "Undefined" 0 0))
      (Utilities|Array|SetArrayElem (Variables|Default|GetExhibitionHero) _array_index _returnvalue true))
    (CallFunction|UpdateHeroTypeOfSaveGameandInstace (Variables|Default|GetCurrent%20Hero%20Type))
    (else
      (Development|PrintString "Please Insert New Hero Type." true true "(R=1.000000,G=0.000000,B=0.009454,A=1.000000)" 1e+01))))

(event Custom|LastHero
  ;[1 1 1] Switch Hero
  (bind _newherotype (CallFunction|SwitchHero false))
  (CallFunction|UpdateExhibitionHero _newherotype))

(event Custom|StartGameMatching
  ;[1 1 1] Start Matching
  (Development|PrintString "Finding Match Session ...")
  (CallFunction|ShowMatchingWidget)
  (bind _results (|FindSessions (Game|GetPlayerController 0) 10 true)
    (:OnSuccess
      (if (> (Utilities|Array|Length _results) 0)
        (bind _array_element (Utilities|Array|ForEachLoopwithBreak _results :!label _label)
          (:LoopBody
            (Variables|Default|SetMatchingSession _array_element)
            (bind _returnvalue (CallFunction|DetectQuitMatching))
            (if _returnvalue
              (bind _extrasettings (Class|AdvancedSessionsLibrary|GetExtraSettings (Variables|Default|GetMatchingSession)))
              (bind (_sesstiontype _ismatching _gamelevelname) (CallFunction|GetSessionExtraInfo _extrasettings))
              (bind _output_get (Variables|Default|SetSessionType "NewEnumerator2"))
              (if (Math|Boolean|ANDBoolean (Utilities|Enum|Equal(Enum) _sesstiontype (Utilities|String|EnumtoString _output_get)) _ismatching (Utilities|Enum|Equal(Enum) _gamelevelname (Utilities|String|EnumtoString (Variables|Default|GetGameLevelName))))
                (Variables|Default|SetisMatchingFound true)
                (Utilities|FlowControl|Sequence
                  (:then_0
                    (|DestroySession (Game|GetPlayerController 0)))
                  (:then_1
                    (|JoinSession (Game|GetPlayerController 0) (Variables|Default|GetMatchingSession)
                      (:OnFailure
                        (Development|PrintString "Join Matching Session Faild" true true "(R=1.000000,G=0.024480,B=0.000000,A=1.000000)" 1e+01))))
                  (:then_2
                    (goto _label Break))))
              (else
                (goto _label Break))))
          (:Completed
            (if (Variables|Default|GetisMatchingFound)
              (Variables|Default|SetisMatchingFound false)
              (else
                (bind _returnvalue_2 (CallFunction|DetectQuitMatching :!label _label_2))
                (if _returnvalue_2
                  (Development|PrintString "No Matching Session" true true "(R=1.000000,G=0.904337,B=0.000000,A=1.000000)")
                  (CallFunction|CreateMatchingSession))))))
        (else
          (goto _label_2))))
    (:OnFailure
      (goto _label_2))))

(event Custom|ShowMatchingWidget
  ;[1 1 1] UMG Manager
  (Utilities|IsValid (Variables|Default|GetWBP_Login)
    (:Is%20Valid
      (Widget|RemovefromParent (Variables|Default|GetWBP_Login)))
    (:Is%20Not%20Valid
      _))
  (bind _returnvalue (UserInterface|CreateWidget "/Game/UMG/WBP_Matching.WBP_Matching_C" self))
  (bind _output_get (Variables|Default|SetWBP_Login _returnvalue))
  (UserInterface|Viewport|AddtoViewport _output_get 0))

(event EventBeginPlay
  ;[1 1 1] Check Local SaveGame Valid
  (CallFunction|GetHeroTypefromSaveGame))

(event Input|ActionEvents|InputActionNextHero
  (params (Key :type Key%20Structure))
  ;[1 1 1] Switch Hero
  (:Released
    (bind _newherotype (CallFunction|SwitchHero true))
    (CallFunction|UpdateExhibitionHero _newherotype)))

(event Input|ActionEvents|InputActionLastHero
  (params (Key :type Key%20Structure))
  ;[1 1 1] Switch Hero
  (:Released
    (bind _newherotype (CallFunction|SwitchHero false))
    (CallFunction|UpdateExhibitionHero _newherotype)))

(event Input|ActionEvents|InputActionStartGame
  (params (Key :type Key%20Structure))
  ;[1 1 1] Start Matching
  (:Released
    (Development|PrintString "Finding Match Session ...")
    (CallFunction|ShowMatchingWidget)
    (bind _results (|FindSessions (Game|GetPlayerController 0) 10 true)
      (:OnSuccess
        (if (> (Utilities|Array|Length _results) 0)
          (bind _array_element (Utilities|Array|ForEachLoopwithBreak _results :!label _label)
            (:LoopBody
              (Variables|Default|SetMatchingSession _array_element)
              (bind _returnvalue (CallFunction|DetectQuitMatching))
              (if _returnvalue
                (bind _extrasettings (Class|AdvancedSessionsLibrary|GetExtraSettings (Variables|Default|GetMatchingSession)))
                (bind (_sesstiontype _ismatching _gamelevelname) (CallFunction|GetSessionExtraInfo _extrasettings))
                (bind _output_get (Variables|Default|SetSessionType "NewEnumerator2"))
                (if (Math|Boolean|ANDBoolean (Utilities|Enum|Equal(Enum) _sesstiontype (Utilities|String|EnumtoString _output_get)) _ismatching (Utilities|Enum|Equal(Enum) _gamelevelname (Utilities|String|EnumtoString (Variables|Default|GetGameLevelName))))
                  (Variables|Default|SetisMatchingFound true)
                  (Utilities|FlowControl|Sequence
                    (:then_0
                      (|DestroySession (Game|GetPlayerController 0)))
                    (:then_1
                      (|JoinSession (Game|GetPlayerController 0) (Variables|Default|GetMatchingSession)
                        (:OnFailure
                          (Development|PrintString "Join Matching Session Faild" true true "(R=1.000000,G=0.024480,B=0.000000,A=1.000000)" 1e+01))))
                    (:then_2
                      (goto _label Break))))
                (else
                  (goto _label Break))))
            (:Completed
              (if (Variables|Default|GetisMatchingFound)
                (Variables|Default|SetisMatchingFound false)
                (else
                  (bind _returnvalue_2 (CallFunction|DetectQuitMatching :!label _label_2))
                  (if _returnvalue_2
                    (Development|PrintString "No Matching Session" true true "(R=1.000000,G=0.904337,B=0.000000,A=1.000000)")
                    (CallFunction|CreateMatchingSession))))))
          (else
            (goto _label_2))))
      (:OnFailure
        (goto _label_2)))))

(fn ConstructionScript
  (Variables|Default|SetDefault%20Hero%20Type "/Game/Hero/Shelly/Blueprint/BP_Hero_Shelly.BP_Hero_Shelly_C")
  (Variables|Default|SetSave%20Game%20Slot%20Name "HeroType"))

(fn GetHeroTypefromGameInstance
  (params (SetHeroTypeInstance :type BP%20Hero%20Base%20Class%20Reference))
  (bind _asbp_game_instance (Utilities|Casting|CastToBP_GameInstance (Game|GetGameInstance)))
  ;[1 1 1] 设置HeroTypeInstace
  (if (Utilities|IsValidClass SetHeroTypeInstance)
    (bind _output_get (Variables|/Game/Map/Base/BP_GameInstance.BP_GameInstance_C|SetHeroTypeInstacne _asbp_game_instance SetHeroTypeInstance))
    (return _output_get)
    (else
      ;[1 1 1] 读取HeroTypeInstance
      (if (Utilities|IsValidClass (Variables|/Game/Map/Base/BP_GameInstance.BP_GameInstance_C|GetHeroTypeInstacne _asbp_game_instance))
        (return (Variables|/Game/Map/Base/BP_GameInstance.BP_GameInstance_C|GetHeroTypeInstacne _asbp_game_instance))
        (else
          ;[1 1 1] 设置HeroTypeInstance为默认HeroType
          (bind _output_get_2 (Variables|/Game/Map/Base/BP_GameInstance.BP_GameInstance_C|SetHeroTypeInstacne _asbp_game_instance (Variables|Default|GetDefault%20Hero%20Type)))
          (return _output_get_2))))))

(fn GetHeroTypefromSaveGame
  (bind _returnvalue (SaveGame|LoadGamefromSlot (Variables|Default|GetSave%20Game%20Slot%20Name)))
  (Utilities|IsValid _returnvalue
    (:Is%20Valid
      (bind _asbp_save_game (Utilities|Casting|CastToBP_SaveGame _returnvalue))
      (bind _output_get (Variables|Default|SetSave%20Game _asbp_save_game))
      (if (Utilities|IsValidClass (Variables|/Game/Map/Base/BP_SaveGame.BP_SaveGame_C|GetHeroTypeSaved _output_get))
        (return (Variables|/Game/Map/Base/BP_SaveGame.BP_SaveGame_C|GetHeroTypeSaved _output_get))
        (else
          _)))
    (:Is%20Not%20Valid
      (bind _returnvalue_2 (SaveGame|CreateSaveGameObject "/Game/Map/Base/BP_SaveGame.BP_SaveGame_C"))
      (bind _output_get_2 (Variables|Default|SetSave%20Game _returnvalue_2))))
  (bind _output_get_3 (Variables|/Game/Map/Base/BP_SaveGame.BP_SaveGame_C|SetHeroTypeSaved _output_get_2 (Variables|Default|GetDefault%20Hero%20Type)))
  (SaveGame|SaveGametoSlot _output_get_2 (Variables|Default|GetSave%20Game%20Slot%20Name))
  (return _output_get_3))

(fn GetHeroExhibitionPointTransfrom
  (params (HeroExhibitionPointName :type String))
  (Utilities|Array|Clear (Variables|Default|GetExhibitionPointTransfrom))
  (bind _outactors (Actor|GetAllActorsOfClass "/Game/Map/Base/BP_ExhibitionPoint.BP_ExhibitionPoint_C"))
  (for _array_element _outactors
    (if (Utilities|Enum|Equal(Enum) (Utilities|GetDisplayName _array_element) HeroExhibitionPointName)
      (bind _output_get (LocalVariables|SetHeroTransfrom (Math|Transform|MakeTransform (.location (Transformation|GetActorTransform _array_element)) "0,180.000000, 0" (.scale (Transformation|GetActorTransform _array_element)))))
      (Utilities|Array|Add (Variables|Default|GetExhibitionPointTransfrom) _output_get)))
  (if (== (Utilities|Array|Length (Variables|Default|GetExhibitionPointTransfrom)) 0)
    (Development|PrintString (Utilities|String|Append "Couldn't Find Exhibition Point Named: " HeroExhibitionPointName))))

(fn SetSessionExtraInfo
  (params (SessionType :type ESessionType%20Enum :default "NewEnumerator0") (isMatching :type Boolean) (GameLevelName :type EGameLevelName%20Enum :default "NewEnumerator0"))
  (Utilities|Array|Clear (Variables|Default|GetSessionExtraSettings))
  (Utilities|FlowControl|Sequence
    (:then_0
      (bind _output_get (Variables|Default|SetExtraSettingsKeys "NewEnumerator0"))
      (Utilities|Array|SetArrayElem (Variables|Default|GetSessionExtraSettings) 0 (Class|AdvancedSessionsLibrary|MakeLiteralSessionPropertyString (Utilities|Name|EnumtoName _output_get) (Utilities|String|EnumtoString SessionType)) true))
    (:then_1
      (bind _output_get_2 (Variables|Default|SetExtraSettingsKeys "NewEnumerator1"))
      (Utilities|Array|SetArrayElem (Variables|Default|GetSessionExtraSettings) 1 (Class|AdvancedSessionsLibrary|MakeLiteralSessionPropertyBool (Utilities|Name|EnumtoName _output_get_2) isMatching) true))
    (:then_2
      (bind _output_get_3 (Variables|Default|SetExtraSettingsKeys "NewEnumerator2"))
      (Utilities|Array|SetArrayElem (Variables|Default|GetSessionExtraSettings) 2 (Class|AdvancedSessionsLibrary|MakeLiteralSessionPropertyString (Utilities|Name|EnumtoName _output_get_3) (Utilities|String|EnumtoString GameLevelName)) true))))

(fn GetSessionExtraInfo
  (params (SessionExtraSettings :type Array%20of%20Session%20Property%20Key%20Pair%20Structures))
  (Variables|Default|SetSessionExtraSettings SessionExtraSettings)
  (Utilities|FlowControl|Sequence
    (:then_0
      (bind _output_get (Variables|Default|SetExtraSettingsKeys "NewEnumerator0"))
      (bind _settingvalue (Class|AdvancedSessionsLibrary|GetSessionPropertyString (Variables|Default|GetSessionExtraSettings) (Utilities|Name|EnumtoName _output_get))))
    (:then_1
      (bind _output_get_2 (Variables|Default|SetExtraSettingsKeys "NewEnumerator1"))
      (bind _settingvalue_2 (Class|AdvancedSessionsLibrary|GetSessionPropertyBool (Variables|Default|GetSessionExtraSettings) (Utilities|Name|EnumtoName _output_get_2))))
    (:then_2
      (bind _output_get_3 (Variables|Default|SetExtraSettingsKeys "NewEnumerator2"))
      (bind _settingvalue_3 (Class|AdvancedSessionsLibrary|GetSessionPropertyString (Variables|Default|GetSessionExtraSettings) (Utilities|Name|EnumtoName _output_get_3))
        (:Found
          (return _settingvalue _settingvalue_2 _settingvalue_3))))))

(fn DetectQuitMatching
  (if (not (Variables|Default|GetisQuitMatching))
    (return true)
    (else
      (Development|PrintString "Matching Quitted" true true "(R=0.000000,G=1.000000,B=0.069125,A=1.000000)")
      (Utilities|Casting|CastToPC_LoginRoom self
        (:then
          (Development|ExecuteConsoleCommand (Utilities|String|Append "ServerTravel " "L_LoginRoom") 0))
        (:CastFailed
          (Development|ExecuteConsoleCommand (Utilities|String|Append "ServerTravel " "L_LoginBegin") 0)))
      (Variables|Default|SetisQuitMatching false)
      (return false))))

(fn SwitchHero
  (params (SwitchNextHero :type Boolean))
  (bind _outrownames (DataTable|GetDataTableRowNames "/Game/Hero/Base/Blueprint/DT_HeroAttribute.DT_HeroAttribute"))
  (for _array_element _outrownames
    (bind _returnvalue (Utilities|GetDataTableRow "/Game/Hero/Base/Blueprint/DT_HeroAttribute.DT_HeroAttribute" _array_element)
      (:then
        (Utilities|Array|AddUnique (LocalVariables|GetHeroTypeList) (.HeroType (Utilities|Struct|BreakFHeroAttribute _returnvalue))))))
  (if (Utilities|IsValidClass (Variables|Default|GetCurrent%20Hero%20Type))
    _
    (else
      (Variables|Default|SetCurrent%20Hero%20Type (Variables|Default|GetDefault%20Hero%20Type))))
  (if SwitchNextHero
    (if (< (+ (Utilities|Array|FindItem (LocalVariables|GetHeroTypeList) (Variables|Default|GetCurrent%20Hero%20Type)) 1) (Utilities|Array|Length (LocalVariables|GetHeroTypeList)))
      (LocalVariables|SetHeroTypeIndex (+ (Utilities|Array|FindItem (LocalVariables|GetHeroTypeList) (Variables|Default|GetCurrent%20Hero%20Type)) 1))
      (else
        (LocalVariables|SetHeroTypeIndex 0)))
    (elif (> (- (Utilities|Array|FindItem (LocalVariables|GetHeroTypeList) (Variables|Default|GetCurrent%20Hero%20Type)) 1) -1)
      (LocalVariables|SetHeroTypeIndex (- (Utilities|Array|FindItem (LocalVariables|GetHeroTypeList) (Variables|Default|GetCurrent%20Hero%20Type)) 1))
      (else
        (LocalVariables|SetHeroTypeIndex (- (Utilities|Array|Length (LocalVariables|GetHeroTypeList)) 1)))))
  (return (Utilities|Array|Get(acopy) (LocalVariables|GetHeroTypeList) (LocalVariables|GetHeroTypeIndex))))