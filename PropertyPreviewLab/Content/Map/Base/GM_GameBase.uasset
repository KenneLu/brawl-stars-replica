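; Base game mode that broadcasts the match result and fills open player starts with AI heroes.
; GameOver passes the Winner to every player's PC_GameBase controller.
; ApawnAI spawns a BP_Hero_Shelly at each available BP_PlayerStart and gives it that start's team.
; It then copies the team and the hero's display name into the AI controller's PS_GameBase player state.
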(event Custom|GameOver
  (bind _returnvalue (Class|GameModeBase|GetNumPlayers))
  (for _index (range 0 (- _returnvalue 1))
    (bind _aspc_game_base (Utilities|Casting|CastToPC_GameBase (Game|GetPlayerController _index)))
    (Default|GameOver _aspc_game_base (Variables|Default|GetWinner))))

(event Custom|ApawnAI
  (bind _outactors (Actor|GetAllActorsOfClass "/Game/Map/Base/BP_PlayerStart.BP_PlayerStart_C"))
  (for _array_element _outactors
    (if (Variables|/Game/Map/Base/BP_PlayerStart.BP_PlayerStart_C|GetisAvaliable _array_element)
      (bind _returnvalue (Game|SpawnActorfromClass "/Game/Hero/Shelly/Blueprint/BP_Hero_Shelly.BP_Hero_Shelly_C" (Math|Transform|MakeTransform (Transformation|GetActorLocation _array_element) "0, 0, 0" "1,1,1") "Undefined" 0 0))
      (bind _output_get (Variables|/Game/Hero/Base/Blueprint/BP_HeroBase.BP_HeroBase_C|SetTeamType _returnvalue (Variables|/Game/Map/Base/BP_PlayerStart.BP_PlayerStart_C|GetTeamType _array_element)))
      (bind _asaic_gam_base (Utilities|Casting|CastToAIC_GamBase (Pawn|GetController _returnvalue)))
      (bind _asps_game_base (Utilities|Casting|CastToPS_GameBase (Variables|/Script/Engine.Controller|GetPlayerState _asaic_gam_base)))
      (Variables|/Game/Map/Base/PS_GameBase.PS_GameBase_C|SetTeamType _asps_game_base _output_get)
      (Variables|/Game/Map/Base/PS_GameBase.PS_GameBase_C|SetPlayerName _asps_game_base (Utilities|GetDisplayName _returnvalue)))))

(fn ConstructionScript)