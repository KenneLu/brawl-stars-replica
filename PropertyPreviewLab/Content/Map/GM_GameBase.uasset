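; GM_GameBase is a game mode Blueprint that starts save-data retrieval when a player joins.
; On PostLogin it casts the new controller to PC_GameBase and calls ClientGetSaveGame on it, leaving the save lookup to that controller.
; An unconnected chain, which never runs, holds logic that loads the saved hero class, replaces the pawn, then spawns and possesses that hero.
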(event EventPostLogin
  (params (NewPlayer :type Player%20Controller%20Object%20Reference))
  (bind _aspc_game_base (Utilities|Casting|CastToPC_GameBase NewPlayer))
  (Default|ClientGetSaveGame _aspc_game_base))

(fn ConstructionScript)