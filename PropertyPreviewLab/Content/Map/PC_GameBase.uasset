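; PC_GameBase is a base player controller that spawns and possesses the player's chosen hero.
; ClientGetHeroType reads the hero class stored in BP_GameInstance, falling back to BP_Shelly1 when none is valid.
; It passes that class to SpawnHero, which spawns the hero at the transform from GetTransformOriginMessage, owned by the controller, and possesses it.
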(event Custom|ClientGetHeroType
  (bind _asbp_game_instance (Utilities|Casting|CastToBP_GameInstance (Game|GetGameInstance)))
  (if (Utilities|IsValidClass (Variables|/Game/Map/BP_GameInstance.BP_GameInstance_C|GetHeroTypeInstacne _asbp_game_instance))
    (Variables|Default|SetHero%20Type (Variables|/Game/Map/BP_GameInstance.BP_GameInstance_C|GetHeroTypeInstacne _asbp_game_instance))
    (else
      (bind _output_get (Variables|Default|SetHero%20Type "/Game/Hero/Shelly/BluePrint/BP_Shelly1.BP_Shelly1_C"))))
  (CallFunction|SpawnHero _output_get))

(event Custom|SpawnHero
  (params (HeroType :type BP%20Hero%20Base%20Class%20Reference))
  (bind _self self)
  (bind _returnvalue (Class|MovieSceneTransformOrigin|GetTransformOrigin(Message) _self))
  (bind _returnvalue_2 (Game|SpawnActorfromClass HeroType _returnvalue "Undefined" _self 0))
  (Pawn|Possess _returnvalue_2))

(fn ConstructionScript)