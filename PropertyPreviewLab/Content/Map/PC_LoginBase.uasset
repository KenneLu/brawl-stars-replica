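; Base player controller for the login map that handles hero selection, display and the host's start-game travel.
; Next/prior inputs cycle the hero class list, respawning the chosen hero at cached exhibition transforms gathered from name-matched BP_ShowHero actors.
; Each switch persists the choice to a SaveGame slot and mirrors it into BP_GameInstance, with getters falling back to a default hero.
; StartGame runs ServerTravel to ChineseHouse only with authority.
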(event Custom|SwitchHeroType
  (params (NewHeroType :type BP%20Hero%20Base%20Class%20Reference))
  ;[1 1 1] 切换角色
  (if (Utilities|IsValidClass NewHeroType)
    (Variables|Default|SetCurrent%20Hero%20Type NewHeroType)
    (for (_array_element _array_index) (Variables|Default|GetExhibitionPointTransfrom)
      (Utilities|IsValid (Utilities|Array|Get(acopy) (Variables|Default|GetHero) _array_index)
        (:Is%20Valid
          (Actor|DestroyActor (Utilities|Array|Get(acopy) (Variables|Default|GetHero) _array_index)))
        (:Is%20Not%20Valid
          _))
      (bind _returnvalue (Game|SpawnActorfromClass (Variables|Default|GetCurrent%20Hero%20Type) _array_element "Undefined" 0 0))
      (Utilities|Array|SetArrayElem (Variables|Default|GetHero) _array_index _returnvalue true))
    (CallFunction|UpdateHeroTypeOfSaveGameandInstace (Variables|Default|GetCurrent%20Hero%20Type))
    (else
      (Development|PrintString "Please Insert New Hero Type."))))

(event Custom|UpdateHeroType_of_SaveGame_and_Instace
  (params (HeroTypeSaved :type BP%20Hero%20Base%20Class%20Reference))
  (bind _save_game (Variables|Default|GetSave%20Game))
  ;[1 1 1] 切换角色
  (bind _output_get (Variables|/Game/Map/BP_SaveGame.BP_SaveGame_C|SetHeroTypeSaved _save_game HeroTypeSaved))
  (SaveGame|SaveGametoSlot _save_game (Variables|Default|GetSave%20Game%20Slot%20Name))
  (bind _asbp_game_instance (Utilities|Casting|CastToBP_GameInstance (Game|GetGameInstance)))
  (Variables|/Game/Map/BP_GameInstance.BP_GameInstance_C|SetHeroTypeInstacne _asbp_game_instance _output_get))

(event EventBeginPlay
  ;[1 1 1] 检查本地SaveGame可靠性
  (CallFunction|GetHeroTypefromSaveGame))

(event Input|ActionEvents|InputActionPriorHero
  (params (Key :type Key%20Structure :default "None"))
  ;[1 1 1] 切换角色
  (:Pressed
    (if (Utilities|IsValidClass (Variables|Default|GetCurrent%20Hero%20Type))
      _
      (else
        (Variables|Default|SetCurrent%20Hero%20Type (Variables|Default|GetDefault%20Hero%20Type))))
    (if (> (- (Utilities|Array|FindItem (Variables|Default|GetHeroTypeList) (Variables|Default|GetCurrent%20Hero%20Type)) 1) -1)
      (Variables|Default|SetHeroIndex (- (Utilities|Array|FindItem (Variables|Default|GetHeroTypeList) (Variables|Default|GetCurrent%20Hero%20Type)) 1))
      (else
        (Variables|Default|SetHeroIndex (- (Utilities|Array|Length (Variables|Default|GetHeroTypeList)) 1))))
    (CallFunction|SwitchHeroType (Utilities|Array|Get(acopy) (Variables|Default|GetHeroTypeList) (Variables|Default|GetHeroIndex)))))

(event Input|ActionEvents|InputActionNextHero
  (params (Key :type Key%20Structure :default "None"))
  ;[1 1 1] 切换角色
  (:Pressed
    (if (Utilities|IsValidClass (Variables|Default|GetCurrent%20Hero%20Type))
      (if (< (+ (Utilities|Array|FindItem (Variables|Default|GetHeroTypeList) (Variables|Default|GetCurrent%20Hero%20Type)) 1) (Utilities|Array|Length (Variables|Default|GetHeroTypeList)))
        (Variables|Default|SetHeroIndex (+ (Utilities|Array|FindItem (Variables|Default|GetHeroTypeList) (Variables|Default|GetCurrent%20Hero%20Type)) 1))
        (else
          (Variables|Default|SetHeroIndex 0)))
      (CallFunction|SwitchHeroType (Utilities|Array|Get(acopy) (Variables|Default|GetHeroTypeList) (Variables|Default|GetHeroIndex)))
      (else
        (Variables|Default|SetCurrent%20Hero%20Type (Variables|Default|GetDefault%20Hero%20Type))))))

(event Input|ActionEvents|InputActionStartGame
  (params (Key :type Key%20Structure :default "None"))
  ;[1 1 1] 房主切换至游戏地图
  (:Pressed
    (Networking|SwitchHasAuthority
      (:Authority
        (Development|ExecuteConsoleCommand "ServerTravel ChineseHouse" (Game|GetPlayerController 0))
        (Development|PrintString "Travel to ChineseHouse")))))

(fn ConstructionScript
  (bind _herotypelist (Variables|Default|GetHeroTypeList))
  (Variables|Default|SetDefault%20Hero%20Type "/Game/Hero/Shelly/Blueprint/BP_Hero_Shelly.BP_Hero_Shelly_C")
  (Variables|Default|SetSave%20Game%20Slot%20Name "HeroType")
  (Utilities|FlowControl|Sequence
    (:then_0
      (Utilities|Array|AddUnique _herotypelist "/Game/Hero/Shelly/Blueprint/BP_Hero_Shelly.BP_Hero_Shelly_C"))
    (:then_1
      (Utilities|Array|AddUnique _herotypelist "/Game/Hero/Primo/Blueprint/BP_Primo.BP_Primo_C"))))

(fn GetHeroTypefromGameInstance
  (params (SetHeroTypeInstance :type BP%20Hero%20Base%20Class%20Reference))
  (bind _asbp_game_instance (Utilities|Casting|CastToBP_GameInstance (Game|GetGameInstance)))
  ;[1 1 1] 设置HeroTypeInstace
  (if (Utilities|IsValidClass SetHeroTypeInstance)
    (bind _output_get (Variables|/Game/Map/BP_GameInstance.BP_GameInstance_C|SetHeroTypeInstacne _asbp_game_instance SetHeroTypeInstance))
    (return _output_get)
    (else
      ;[1 1 1] 读取HeroTypeInstance
      (if (Utilities|IsValidClass (Variables|/Game/Map/BP_GameInstance.BP_GameInstance_C|GetHeroTypeInstacne _asbp_game_instance))
        (return (Variables|/Game/Map/BP_GameInstance.BP_GameInstance_C|GetHeroTypeInstacne _asbp_game_instance))
        (else
          ;[1 1 1] 设置HeroTypeInstance为默认HeroType
          (bind _output_get_2 (Variables|/Game/Map/BP_GameInstance.BP_GameInstance_C|SetHeroTypeInstacne _asbp_game_instance (Variables|Default|GetDefault%20Hero%20Type)))
          (return _output_get_2))))))

(fn GetHeroTypefromSaveGame
  (bind _returnvalue (SaveGame|LoadGamefromSlot (Variables|Default|GetSave%20Game%20Slot%20Name)))
  (Utilities|IsValid _returnvalue
    (:Is%20Valid
      (bind _asbp_save_game (Utilities|Casting|CastToBP_SaveGame _returnvalue))
      (bind _output_get (Variables|Default|SetSave%20Game _asbp_save_game))
      (if (Utilities|IsValidClass (Variables|/Game/Map/BP_SaveGame.BP_SaveGame_C|GetHeroTypeSaved _output_get))
        (return (Variables|/Game/Map/BP_SaveGame.BP_SaveGame_C|GetHeroTypeSaved _output_get))
        (else
          _)))
    (:Is%20Not%20Valid
      (bind _returnvalue_2 (SaveGame|CreateSaveGameObject "/Game/Map/BP_SaveGame.BP_SaveGame_C"))
      (bind _output_get_2 (Variables|Default|SetSave%20Game _returnvalue_2))))
  (bind _output_get_3 (Variables|/Game/Map/BP_SaveGame.BP_SaveGame_C|SetHeroTypeSaved _output_get_2 (Variables|Default|GetDefault%20Hero%20Type)))
  (SaveGame|SaveGametoSlot _output_get_2 (Variables|Default|GetSave%20Game%20Slot%20Name))
  (return _output_get_3))

(fn GetHeroExhibitionPointTransfrom
  (params (HeroExhibitionPointName :type String))
  (Utilities|Array|Clear (Variables|Default|GetExhibitionPointTransfrom))
  (bind _outactors (Actor|GetAllActorsOfClass "/Game/Map/Lobby/BP_ShowHero.BP_ShowHero_C"))
  (for _array_element _outactors
    (if (Utilities|Enum|Equal(Enum) (Utilities|GetDisplayName _array_element) HeroExhibitionPointName)
      (bind _output_get (Variables|Default|SetHero%20Transfrom (Math|Transform|MakeTransform (.location (Transformation|GetActorTransform _array_element)) "0,180.000000, 0" (.scale (Transformation|GetActorTransform _array_element)))))
      (Utilities|Array|Add (Variables|Default|GetExhibitionPointTransfrom) _output_get)))
  (if (== (Utilities|Array|Length (Variables|Default|GetExhibitionPointTransfrom)) 0)
    (Development|PrintString (Utilities|String|Append "Couldn't Find Exhibition Point Named: " HeroExhibitionPointName))))