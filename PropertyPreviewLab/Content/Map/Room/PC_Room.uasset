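; Player controller for the room map that spawns a player's chosen hero for display and sets that player's camera.
; ServerInit stores the player number, and ClientGetHeroType reads the hero class from the GameInstance for ExhibitHero to spawn server-side.
; Exhibit points and room cameras are matched by names built from the player number.
; After a successful spawn and short delay, the client switches view to its matching BP_RoomCamera.
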(event Custom|ClientUseCameraView
  (params (NewParam :type Boolean))
  ;[1 1 1] 设置客户端相机视角
  (Variables|Default|SetClientCameraName (Utilities|String|Append "BP_RoomCamera_Player" (Utilities|String|ToString(Integer) (Variables|Default|GetPlayerNum))))
  (bind _outactors (Actor|GetAllActorsOfClass "/Game/Map/Room/BP_RoomCamera.BP_RoomCamera_C"))
  (bind (_array_element _array_index) (Utilities|Array|ForEachLoopwithBreak _outactors :!label _label)
    (:LoopBody
      (if (Utilities|Enum|Equal(Enum) (Utilities|GetDisplayName _array_element) (Variables|Default|GetClientCameraName))
        (Utilities|FlowControl|Sequence
          (:then_0
            (Game|Player|SetViewTargetwithBlend _array_element 0.0 "VTBlend_Linear" 0.0 false))
          (:then_1
            (goto _label Break)))))
    (:Completed
      (if (== _array_index (- (Utilities|Array|Length _outactors) 1))
        (Development|PrintString (Utilities|String|Append "Couldn't Find Camera Named: " (Variables|Default|GetClientCameraName)))))))

(event Custom|ClientGetHeroType
  ;[1 1 1] 获取客户端GameInstance英雄类型
  (bind _herotypeinstance (CallFunction|GetHeroTypefromGameInstance))
  (CallFunction|ExhibitHero _herotypeinstance))

(event Custom|ExhibitHero
  (params (ShowHeroType :type BP%20Hero%20Base%20Class%20Reference))
  ;[1 1 1] 服务端生成角色
  (Variables|Default|SetCurrent%20Hero%20Type ShowHeroType)
  (CallFunction|GetHeroExhibitionPointTransfrom (Utilities|String|Append "BP_ExhibitPoint_Player" (Utilities|String|ToString(Integer) (Variables|Default|GetPlayerNum))))
  (for (_array_element _array_index) (Variables|Default|GetExhibitionPointTransfrom)
    (bind _returnvalue (Game|SpawnActorfromClass (Variables|Default|GetCurrent%20Hero%20Type) _array_element "Undefined" 0 0))
    (Utilities|IsValid _returnvalue
      (:Is%20Valid
        (Utilities|Array|SetArrayElem (Variables|Default|GetHero) _array_index _returnvalue true)
        (Utilities|FlowControl|Delay 0.2)
        (CallFunction|ClientUseCameraView false))
      (:Is%20Not%20Valid
        (Development|PrintString (Utilities|String|Append "Spawn Exhibition Hero " (Utilities|String|ToString(Integer) (Variables|Default|GetPlayerNum)) " class " (Utilities|GetClassDisplayName (Variables|Default|GetCurrent%20Hero%20Type)) "Faild!"))))))

(event Custom|ServerInit
  (params (PlayerNum :type Integer))
  ;[1 1 1] 初始化玩家编号
  (Variables|Default|SetPlayerNum PlayerNum))

(fn ConstructionScript)