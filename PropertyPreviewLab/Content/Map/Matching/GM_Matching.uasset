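; GM_Matching is the matchmaking lobby game mode that gathers players and server-travels them to the chosen level once it is full.
; PostLogin counts players, puts each in one of two groups by a per-group cap computed in the construction script, and sends it to the client to save.
; When the lobby fills, it rewrites session extra settings to clear the matching flag, updates the session, then runs ServerTravel to the level named by the player controller.
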(event EventPostLogin
  (params (NewPlayer :type Player%20Controller%20Object%20Reference))
  ;[1 1 1] 开始游戏
  (Variables|Default|SetGM_PlayerNum (+ (Variables|Default|GetGM_PlayerNum) 1))
  (bind _aspc_login_base (Utilities|Casting|CastToPC_LoginBase NewPlayer))
  (Variables|Default|SetGame%20Level%20Name (Variables|/Game/Map/Base/PC_LoginBase.PC_LoginBase_C|GetGameLevelName _aspc_login_base))
  (if (<= (Variables|Default|GetGM_PlayerNum) (Variables|Default|GetGM_GroupMaxPlayer))
    (Variables|/Game/Map/Base/PC_LoginBase.PC_LoginBase_C|SetGroupType _aspc_login_base 0)
    (else
      (Variables|/Game/Map/Base/PC_LoginBase.PC_LoginBase_C|SetGroupType _aspc_login_base 1)))
  (Default|ClientSaveGroupTypeInstance _aspc_login_base (Variables|/Game/Map/Base/PC_LoginBase.PC_LoginBase_C|GetGroupType _aspc_login_base))
  (Development|PrintString "StartingGame")
  (if (== (Variables|Default|GetGM_PlayerNum) (Variables|Default|GetGM_LevelMaxPlayer))
    ;;[1 1 1] 更新匹配状态，isMatching = False
    (CallFunction|SetSessionExtraInfo "NewEnumerator2" false (Variables|Default|GetGame%20Level%20Name))
    (bind (_numconnections _numprivateconnections _bislan _bisdedicated _ballowinvites _ballowjoininprogress _bisanticheatenabled) (Class|AdvancedSessionsLibrary|GetSessionSettings)
      (:OnSuccess
        (|UpdateSession (Variables|Default|GetSession%20Extra%20Settings) _numconnections _numprivateconnections _bislan _ballowinvites _ballowjoininprogress _bisanticheatenabled _bisdedicated
          (:OnSuccess
            (Development|ExecuteConsoleCommand (Utilities|String|Append "ServerTravel " (Utilities|String|EnumtoString (Variables|Default|GetGame%20Level%20Name))) 0)
            (Development|PrintString (Utilities|String|Append "ServerTravel " (Utilities|String|EnumtoString (Variables|Default|GetGame%20Level%20Name))) true true "(R=1.000000,G=0.028928,B=0.000000,A=1.000000)" 1e+01))
          (:OnFailure
            (Development|PrintString "UpdateSessionFailure" true true "(R=1.000000,G=0.000000,B=0.051108,A=1.000000)" 1e+01)))))))

(fn ConstructionScript
  (Variables|Default|SetGM_GroupMaxPlayer (/ (Variables|Default|GetGM_LevelMaxPlayer) (Variables|Default|GetGM_GroupCount))))

(fn SetSessionExtraInfo
  (params (SessionType :type ESessionType%20Enum :default "NewEnumerator0") (isMatching :type Boolean) (GameLevelName :type EGameLevelName%20Enum :default "NewEnumerator0"))
  (Utilities|Array|Clear (Variables|Default|GetSession%20Extra%20Settings))
  (Utilities|FlowControl|Sequence
    (:then_0
      (bind _output_get (Variables|Default|SetSession%20Key "NewEnumerator0"))
      (Utilities|Array|SetArrayElem (Variables|Default|GetSession%20Extra%20Settings) 0 (Class|AdvancedSessionsLibrary|MakeLiteralSessionPropertyString (Utilities|Name|EnumtoName _output_get) (Utilities|String|EnumtoString SessionType)) true))
    (:then_1
      (bind _output_get_2 (Variables|Default|SetSession%20Key "NewEnumerator1"))
      (Utilities|Array|SetArrayElem (Variables|Default|GetSession%20Extra%20Settings) 1 (Class|AdvancedSessionsLibrary|MakeLiteralSessionPropertyBool (Utilities|Name|EnumtoName _output_get_2) isMatching) true))
    (:then_2
      (bind _output_get_3 (Variables|Default|SetSession%20Key "NewEnumerator2"))
      (Utilities|Array|SetArrayElem (Variables|Default|GetSession%20Extra%20Settings) 2 (Class|AdvancedSessionsLibrary|MakeLiteralSessionPropertyString (Utilities|Name|EnumtoName _output_get_3) (Utilities|String|EnumtoString GameLevelName)) true))))