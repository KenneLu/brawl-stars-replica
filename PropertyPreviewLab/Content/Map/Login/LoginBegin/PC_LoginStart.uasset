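; Player controller for the login start map that shows the player's hero, views it through the exhibition camera and opens the login widget.
; Hero type comes from the save game and game instance lookups, then spawns at a named exhibition point.
; Input actions and matching events create, search and join LAN rooms via Advanced Sessions.
; Creation opens the room level as listen server, while search stores the first session matching the type for joining.
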(event Custom|CreateRoom
  ;[1 1 1] Create Room
  (|DestroySession self
    (:OnSuccess
      _)
    (:OnFailure
      _))
  (Development|PrintString "Creating Room Session ...")
  (CallFunction|SetSessionExtraInfo "NewEnumerator0" false "NewEnumerator0")
  (|AdvancedSession (Variables|Default|GetSessionExtraSettings) (Game|GetPlayerController 0) 3 0 true true false true true false false false true
    (:OnSuccess
      (Development|PrintString "Room Created" true true "(R=0.028321,G=1.000000,B=0.000000,A=1.000000)")
      (Game|OpenLevel(byName) "L_LoginRoom" true "Listen"))
    (:OnFailure
      (Development|PrintString "Ceate Room Failure" true true "(R=1.000000,G=0.076232,B=0.000000,A=1.000000)" 1e+01))))

(event Custom|SearchRoom
  ;[1 1 1] Serach Room
  (Development|PrintString "Searching Room ...")
  (bind _results (|FindSessions (Game|GetPlayerController 0) 10 true)
    (:OnSuccess
      (if (> (Utilities|Array|Length _results) 0)
        (bind _array_element (Utilities|Array|ForEachLoopwithBreak _results :!label _label)
          (:LoopBody
            (bind _extrasettings (Class|AdvancedSessionsLibrary|GetExtraSettings _array_element))
            (bind _sesstiontype (CallFunction|GetSessionExtraInfo _extrasettings))
            (bind _output_get (Variables|Default|SetSessionType "NewEnumerator0"))
            (if (Utilities|Enum|Equal(Enum) _sesstiontype (Utilities|String|EnumtoString _output_get))
              (Development|PrintString (Utilities|String|Append "Find Room：" (Class|FindSessionsCallbackProxy|GetServerName _array_element) "Member：" (Utilities|String|ToString(Integer) (Class|FindSessionsCallbackProxy|GetCurrentPlayers _array_element))))
              (Variables|Default|SetRoom%20Session _array_element)
              (goto _label Break))))
        (else
          (Development|PrintString "No Room Session" true true "(R=1.000000,G=0.847106,B=0.000000,A=1.000000)" :!label _label_2))))
    (:OnFailure
      (goto _label_2))))

(event Custom|JoinRoom
  ;[1 1 1] Join Room
  (Development|PrintString "JoinRoom")
  (|JoinSession (Game|GetPlayerController 0) (Variables|Default|GetRoom%20Session)
    (:OnSuccess
      (Development|PrintString "成功加入房间"))
    (:OnFailure
      (Development|PrintString "加入房间失败"))))

(event EventBeginPlay
  ;[1 1 1] Spawn Hero For Show
  (|CallParentFunction)
  (bind _hero_type_saved (CallFunction|GetHeroTypefromSaveGame))
  (bind _herotypeinstance (CallFunction|GetHeroTypefromGameInstance _hero_type_saved))
  (bind _output_get (Variables|Default|SetCurrentHeroType _herotypeinstance))
  (CallFunction|GetHeroExhibitionPointTransfrom (Variables|Default|GetExhibitinoPointName))
  (bind _returnvalue (Game|SpawnActorfromClass _output_get (Utilities|Array|Get(acopy) (Variables|Default|GetExhibitionPointTransfrom)) "Undefined" 0 0))
  (Utilities|Array|SetArrayElem (Variables|Default|GetExhibitionHero) 0 _returnvalue true)
  ;[1 1 1] Use Exhibition Camera View
  (bind _outactors (Actor|GetAllActorsOfClass "/Game/Map/Base/BP_ExhibitionCamera.BP_ExhibitionCamera_C"))
  (Game|Player|SetViewTargetwithBlend self (Utilities|Array|Get(acopy) _outactors) 0.0 "VTBlend_Linear" 0.0 false)
  ;[1 1 1] UMG
  (if (Pawn|IsLocalController)
    (bind _returnvalue_2 (UserInterface|CreateWidget "/Game/UMG/WBP_Login.WBP_Login_C" self))
    (bind _output_get_2 (Variables|Default|SetWBP_Login _returnvalue_2))
    (UserInterface|Viewport|AddtoViewport _output_get_2 0)
    (Variables|Default|SetbShowMouseCursor true)))

(event Input|ActionEvents|InputActionSearchRoom
  (params (Key :type Key%20Structure))
  ;[1 1 1] Serach Room
  (:Released
    (Development|PrintString "Searching Room ...")
    (bind _results (|FindSessions (Game|GetPlayerController 0) 10 true)
      (:OnSuccess
        (if (> (Utilities|Array|Length _results) 0)
          (bind _array_element (Utilities|Array|ForEachLoopwithBreak _results :!label _label)
            (:LoopBody
              (bind _extrasettings (Class|AdvancedSessionsLibrary|GetExtraSettings _array_element))
              (bind _sesstiontype (CallFunction|GetSessionExtraInfo _extrasettings))
              (bind _output_get (Variables|Default|SetSessionType "NewEnumerator0"))
              (if (Utilities|Enum|Equal(Enum) _sesstiontype (Utilities|String|EnumtoString _output_get))
                (Development|PrintString (Utilities|String|Append "Find Room：" (Class|FindSessionsCallbackProxy|GetServerName _array_element) "Member：" (Utilities|String|ToString(Integer) (Class|FindSessionsCallbackProxy|GetCurrentPlayers _array_element))))
                (Variables|Default|SetRoom%20Session _array_element)
                (goto _label Break))))
          (else
            (Development|PrintString "No Room Session" true true "(R=1.000000,G=0.847106,B=0.000000,A=1.000000)" :!label _label_2))))
      (:OnFailure
        (goto _label_2)))))

(event Input|ActionEvents|InputActionJoinRoom
  (params (Key :type Key%20Structure))
  ;[1 1 1] Join Room
  (:Released
    (Development|PrintString "JoinRoom")
    (|JoinSession (Game|GetPlayerController 0) (Variables|Default|GetRoom%20Session)
      (:OnSuccess
        (Development|PrintString "成功加入房间"))
      (:OnFailure
        (Development|PrintString "加入房间失败")))))

(event Input|ActionEvents|InputActionCreateRoom
  (params (Key :type Key%20Structure))
  ;[1 1 1] Create Room
  (:Released
    (|DestroySession self
      (:OnSuccess
        _)
      (:OnFailure
        _))
    (Development|PrintString "Creating Room Session ...")
    (CallFunction|SetSessionExtraInfo "NewEnumerator0" false "NewEnumerator0")
    (|AdvancedSession (Variables|Default|GetSessionExtraSettings) (Game|GetPlayerController 0) 3 0 true true false true true false false false true
      (:OnSuccess
        (Development|PrintString "Room Created" true true "(R=0.028321,G=1.000000,B=0.000000,A=1.000000)")
        (Game|OpenLevel(byName) "L_LoginRoom" true "Listen"))
      (:OnFailure
        (Development|PrintString "Ceate Room Failure" true true "(R=1.000000,G=0.076232,B=0.000000,A=1.000000)" 1e+01)))))

(fn ConstructionScript)