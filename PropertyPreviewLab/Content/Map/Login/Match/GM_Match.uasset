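; Game mode for the matchmaking map that gathers players, assigns teams and launches the match.
; Each PostLogin shows matching UI, reads the level name from session settings, gets limits from DT_GameLevel and picks a team by join order.
; When full, it marks the session as not matching and ServerTravels to the level, with dev fallbacks on session failures.
; Tick watches a quit flag to travel back to login.
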(event Custom|SetLevelTeamInfo
  ;[1 1 1] Set Level Team Info
  (bind _outrownames (DataTable|GetDataTableRowNames "/Game/Map/Base/DT_GameLevel.DT_GameLevel"))
  (bind _array_element (Utilities|Array|ForEachLoopwithBreak _outrownames :!label _label)
    (:LoopBody
      (bind _returnvalue (Utilities|GetDataTableRow "/Game/Map/Base/DT_GameLevel.DT_GameLevel" _array_element)
        (:then
          (if (Utilities|Enum|Equal(Enum) (Utilities|String|EnumtoString (.GameLevelName (Utilities|Struct|BreakFGameLevelAttribute _returnvalue))) (Variables|Default|GetGame%20Level%20Name))
            (Utilities|FlowControl|Sequence
              (:then_0
                (Variables|Default|SetGM_TeamMax (.TeamMax (Utilities|Struct|BreakFGameLevelAttribute _returnvalue)))
                (Variables|Default|SetGM_PlayerMax (.PlayerMax (Utilities|Struct|BreakFGameLevelAttribute _returnvalue))))
              (:then_1
                (goto _label Break)))))))))

(event Custom|GMStartGame
  (bind _game_level_name (Variables|Default|GetGame%20Level%20Name))
  (bind _returnvalue (Utilities|String|Append "ServerTravel " _game_level_name))
  ;[1 1 1] Start Game
  (Development|ExecuteConsoleCommand _returnvalue 0)
  (Development|PrintString _returnvalue true true "(R=0.059851,G=1.000000,B=0.000000,A=1.000000)" 1e+01))

(event Custom|SetTeam
  (bind _playercontroller (Variables|Default|GetPlayerController))
  (bind _playercontroller_2 (Variables|Default|GetPlayerController))
  ;[1 1 1] Set Team
  (Variables|Default|SetGM_PlayerSequence (+ (Variables|Default|GetGM_PlayerSequence) 1))
  (if (<= (Variables|Default|GetGM_PlayerSequence) (Math|Float|Ceil (Math|Conversions|ToFloat(Integer) (/ (Variables|Default|GetGM_PlayerMax) (Variables|Default|GetGM_TeamMax)))))
    (Variables|/Game/Map/Base/PC_GameBase.PC_GameBase_C|SetTeamType _playercontroller "NewEnumerator0")
    (else
      (Variables|/Game/Map/Base/PC_GameBase.PC_GameBase_C|SetTeamType _playercontroller "NewEnumerator1")))
  (Default|SaveTeamTypeInstance _playercontroller_2 (Variables|/Game/Map/Base/PC_GameBase.PC_GameBase_C|GetTeamType _playercontroller_2)))

(event Custom|UpdateSession
  ;[1 1 1] Update Matching State
  (CallFunction|SetSessionExtraInfo "NewEnumerator2" false (Variables|Default|GetGame%20Level%20Name))
  (bind (_numconnections _numprivateconnections _bislan _bisdedicated _ballowinvites _ballowjoininprogress _bisanticheatenabled) (Class|AdvancedSessionsLibrary|GetSessionSettings)
    (:OnSuccess
      (|UpdateSession (Variables|Default|GetSession%20Extra%20Settings) _numconnections _numprivateconnections _bislan _ballowinvites _ballowjoininprogress _bisanticheatenabled _bisdedicated
        (:OnSuccess
          _)
        (:OnFailure
          (Development|PrintString "Update Session Failure" true true "(R=1.000000,G=0.000000,B=0.051108,A=1.000000)" 1e+01)
          ;[1 1 1] Dev Only
          (Development|PrintString "Dev" true true "(R=0.979461,G=0.000000,B=1.000000,A=1.000000)" :!label _label))))
    (:OnFailure
      (Development|PrintString "Get Session Setting Failure")
      (goto _label)))
  (Variables|Default|SetisMachingDone true))

(event Custom|SetLevelName
  ;[1 1 1] Set Level Name
  (bind _extrasettings (Class|AdvancedSessionsLibrary|GetSessionSettings)
    (:OnSuccess
      (bind _output_get (Variables|Default|SetSession%20Key "NewEnumerator2"))
      (bind _settingvalue (Class|AdvancedSessionsLibrary|GetSessionPropertyString _extrasettings (Utilities|Name|EnumtoName _output_get))
        (:Found
          (Variables|Default|SetGame%20Level%20Name _settingvalue))))
    (:OnFailure
      (Development|PrintString "Get Session Setting Failure" true true "(R=1.000000,G=0.000000,B=0.000000,A=1.000000)" 1e+01)
      ;;[1 1 1] Dev Only
      (Development|PrintString "Dev" true true "(R=0.979461,G=0.000000,B=1.000000,A=1.000000)")
      (Variables|Default|SetGame%20Level%20Name "L_GemGrab"))))

(event EventTick
  (params (DeltaSeconds :type Float%20%28single-precision%29))
  ;[1 1 1] Detect Quit Matching
  (if (Variables|Default|GetisQuitMatching)
    (Utilities|FlowControl|DoOnce false
      (:Completed
        (Development|PrintString "Matching Quitted" true true "(R=0.074001,G=1.000000,B=0.000000,A=1.000000)")
        (Development|ExecuteConsoleCommand (Utilities|String|Append "ServerTravel " "L_LoginStart") 0)))))

(event EventPostLogin
  (params (NewPlayer :type Player%20Controller%20Object%20Reference))
  ;[1 1 1] Matching Manager
  (bind _aspc_game_base (Utilities|Casting|CastToPC_GameBase NewPlayer))
  (bind _output_get (Variables|Default|SetPlayerController _aspc_game_base))
  (Default|ShowMatchingUMG _output_get)
  (CallFunction|SetLevelName)
  (CallFunction|SetLevelTeamInfo)
  (CallFunction|SetTeam)
  ;;[1 1 1] Matching Done
  (if (== (Variables|Default|GetGM_PlayerSequence) (Variables|Default|GetGM_PlayerMax))
    (CallFunction|UpdateSession)
    (if (Variables|Default|GetisMachingDone)
      (Utilities|FlowControl|Delay 0.2)
      (CallFunction|GMStartGame))))

(fn ConstructionScript)

(fn SetSessionExtraInfo
  (params (SessionType :type ESessionType%20Enum :default "NewEnumerator0") (isMatching :type Boolean) (GameLevelName :type String))
  (Utilities|Array|Clear (Variables|Default|GetSession%20Extra%20Settings))
  (Utilities|FlowControl|Sequence
    (:then_0
      (bind _output_get (Variables|Default|SetSession%20Key "NewEnumerator0"))
      (Utilities|Array|SetArrayElem (Variables|Default|GetSession%20Extra%20Settings) 0 (Class|AdvancedSessionsLibrary|MakeLiteralSessionPropertyString (Utilities|Name|EnumtoName _output_get) (Utilities|String|EnumtoString SessionType)) true))
    (:then_1
      (bind _output_get_2 (Variables|Default|SetSession%20Key "NewEnumerator1"))
      (Utilities|Array|SetArrayElem (Variables|Default|GetSession%20Extra%20Settings) 1 (Class|AdvancedSessionsLibrary|MakeLiteralSessionPropertyBool (Utilities|Name|EnumtoName _output_get_2) isMatching) true))
    (:then_2
      (bind _output_get_3 (Variables|Default|SetSession%20Key "NewEnumerator2"))
      (Utilities|Array|SetArrayElem (Variables|Default|GetSession%20Extra%20Settings) 2 (Class|AdvancedSessionsLibrary|MakeLiteralSessionPropertyString (Utilities|Name|EnumtoName _output_get_3) GameLevelName) true))))

(fn DetectQuitMatching
  (if (not (Variables|Default|GetisQuitMatching))
    (return true)
    (else
      (Utilities|FlowControl|DoOnce false
        (:Completed
          (Development|PrintString "Matching Quitted" true true "(R=0.074001,G=1.000000,B=0.000000,A=1.000000)")
          (Development|ExecuteConsoleCommand (Utilities|String|Append "ServerTravel " "L_LoginBegin") 0)
          (return false))))))