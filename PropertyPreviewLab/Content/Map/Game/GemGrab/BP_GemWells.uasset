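; BP_GemWells is the gem spawner for the GemGrab game mode.
; On the authority only, a looping one-second timer spawns a BP_Gem just above the well, adjusting for collisions but always spawning.
; Each valid gem receives a velocity built from world up plus a random horizontal offset, so gems pop upward and scatter around the well.
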(event Custom|SpawnGem
  (bind _returnvalue (Transformation|GetActorLocation))
  (bind _returnvalue_2 (Game|SpawnActorfromClass "/Game/Map/Game/GemGrab/BP_Gem.BP_Gem_C" (Math|Transform|MakeTransform (Math|Vector|MakeVector (.x _returnvalue) (.y _returnvalue) (+ (.z _returnvalue) 1e+02)) "0, 0, 0" "1,1,1") "AdjustIfPossibleButAlwaysSpawn" 0 0))
  (Utilities|IsValid _returnvalue_2
    (:Is%20Valid
      (Default|SetVelocity _returnvalue_2 (* (+ (Math|Vector|GetUpVector "0, 0, 0") (Math|Vector|MakeVector (/ (Math|Random|RandomFloatinRange -1e+02 1e+02) 1e+02) (/ (Math|Random|RandomFloatinRange -1e+02 1e+02) 1e+02) 0.0)) 3e+02)))))

(event EventBeginPlay
  (Networking|SwitchHasAuthority
    (:Authority
      (Utilities|Time|SetTimerbyEvent (delegate Custom|SpawnGem) 1.0 true))))

(fn ConstructionScript)