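; Game mode for Gem Grab, a two-team gem-collecting match that spawns six AI heroes shortly after start.
; GetGem and LossGem adjust each team's count and mirror it to the GS_GemGrab game state.
; RepNotify functions on the counts re-evaluate the leader, signalling Winning at ten or more gems with a strict lead, otherwise KeepGrabbing.
; Game over picks the team with more gems, with ties going to Team B.
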(event Custom|GetGem
  (params (TeamType :type ETeamType%20Enum :default "NewEnumerator2"))
  (bind _gamestategemgrab (Variables|Default|GetGameStateGemGrab))
  (switch Utilities|FlowControl|Switch|SwitchonETeamType TeamType
    (:NewEnumerator0
      (bind _output_get (Variables|Default|SetGemAmountTeamA (+ (Variables|Default|GetGemAmountTeamA) 1)))
      (Variables|/Game/Map/Game/GemGrab/GS_GemGrab.GS_GemGrab_C|SetGemAmountTeamA _gamestategemgrab _output_get))
    (:NewEnumerator1
      (bind _output_get_2 (Variables|Default|SetGemAmountTeamB (+ (Variables|Default|GetGemAmountTeamB) 1)))
      (Variables|/Game/Map/Game/GemGrab/GS_GemGrab.GS_GemGrab_C|SetGemAmountTeamB _gamestategemgrab _output_get_2))))

(event Custom|LossGem
  (params (TeamType :type ETeamType%20Enum :default "NewEnumerator2") (LossAmount :type Integer))
  (switch Utilities|FlowControl|Switch|SwitchonETeamType TeamType
    (:NewEnumerator0
      (bind _output_get (Variables|Default|SetGemAmountTeamA (- (Variables|Default|GetGemAmountTeamA) LossAmount)))
      (Variables|/Game/Map/Game/GemGrab/GS_GemGrab.GS_GemGrab_C|SetGemAmountTeamA (Variables|Default|GetGameStateGemGrab) _output_get))
    (:NewEnumerator1
      (bind _output_get_2 (Variables|Default|SetGemAmountTeamB (- (Variables|Default|GetGemAmountTeamB) LossAmount)))
      (Variables|/Game/Map/Game/GemGrab/GS_GemGrab.GS_GemGrab_C|SetGemAmountTeamB (Variables|Default|GetGameStateGemGrab) _output_get_2))))

(event Custom|GemGrabGameOver
  (if (> (Variables|Default|GetGemAmountTeamA) (Variables|Default|GetGemAmountTeamB))
    (Variables|Default|SetWinner "NewEnumerator0")
    (else
      (Variables|Default|SetWinner "NewEnumerator1")))
  (CallFunction|GameOver))

(event Custom|InitGame
  (bind _asgs_gem_grab (Utilities|Casting|CastToGS_GemGrab (Game|GetGameState)))
  (Variables|Default|SetGameStateGemGrab _asgs_gem_grab)
  (Variables|Default|SetGemAmountTeamA 0)
  (Variables|Default|SetGemAmountTeamB 0))

(event EventBeginPlay
  (|CallParentFunction)
  (CallFunction|InitGame)
  (Utilities|FlowControl|Delay 0.2)
  (CallFunction|SpawnAIHero "NewEnumerator2" 6))

(fn ConstructionScript
  (|CallParentFunction))

(fn OnRepGemAmountTeamA
  (CallFunction|UpdateWinner))

(fn OnRepGemAmountTeamB
  (CallFunction|UpdateWinner))

(fn UpdateWinner
  (Math|Integer|CompareInt (Variables|Default|GetGemAmountTeamA) (Variables|Default|GetGemAmountTeamB)
    (:>
      (if (>= (Variables|Default|GetGemAmountTeamA) 10)
        (Default|Winning (Variables|Default|GetGameStateGemGrab) "NewEnumerator0")
        (else
          (Default|KeepGrabbing (Variables|Default|GetGameStateGemGrab))))
      (Variables|Default|SetWinner "NewEnumerator0"))
    (:==
      (Default|KeepGrabbing (Variables|Default|GetGameStateGemGrab))
      (Variables|Default|SetWinner "NewEnumerator2"))
    (:<
      (if (>= (Variables|Default|GetGemAmountTeamB) 10)
        (Default|Winning (Variables|Default|GetGameStateGemGrab) "NewEnumerator1")
        (else
          (Default|KeepGrabbing (Variables|Default|GetGameStateGemGrab))))
      (Variables|Default|SetWinner "NewEnumerator1"))))