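; BP_Gem is the collectible gem actor for the Gem Grab game mode, moved by a projectile movement component whose local-space velocity is set through SetVelocity.
; When a hero overlaps its sphere, a locally controlled hero reports the pickup to the first player controller, PC_Game_GemGrab, via GetGem.
; Any hero overlap then calls Picked, which destroys the gem, although a failed controller cast stops before that.
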(event OnComponentBeginOverlap(Sphere)
  (params (OverlappedComponent :type Primitive%20Component%20Object%20Reference) (OtherActor :type Actor%20Object%20Reference) (OtherComp :type Primitive%20Component%20Object%20Reference) (OtherBodyIndex :type Integer) (bFromSweep :type Boolean) (SweepResult :type Hit%20Result%20Structure%20%28by%20ref%29))
  (bind _asbp_hero_base (Utilities|Casting|CastToBP_HeroBase OtherActor))
  (if (Pawn|IsLocallyControlled _asbp_hero_base)
    (bind _aspc_game_gem_grab (Utilities|Casting|CastToPC_Game_GemGrab (Game|GetPlayerController 0)))
    (Default|GetGem _aspc_game_gem_grab))
  (CallFunction|Picked))

(event Custom|SetVelocity
  (params (NewVelocity :type Vector))
  (Game|Components|ProjectileMovement|SetVelocityinLocalSpace (Variables|Default|GetProjectileMovement) NewVelocity))

(event Custom|Picked
  (Actor|DestroyActor))

(fn ConstructionScript)