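; Game mode for the Heist mode, where each team has a safe box and loses when it is destroyed.
; On BeginPlay it finds both safe boxes, passes them to GS_Heist, binds their damage and destroy events, then spawns AI after short delays.
; Damage updates the provisional Winner by comparing truncated safe box health, allowing a tie.
; Destruction sets the opposing team as Winner and calls GameOver.
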(event Custom|TeamB%20Won
  (params (DestroyedActor :type Actor%20Object%20Reference))
  (Variables|Default|SetWinner "NewEnumerator1")
  (CallFunction|GameOver))

(event Custom|TeamA%20Won
  (params (DestroyedActor :type Actor%20Object%20Reference))
  (Variables|Default|SetWinner "NewEnumerator0")
  (CallFunction|GameOver))

(event Custom|BindSafeBoxDestroyEvent
  (Game|BindEventtoOnDestroyed (Variables|Default|GetSafeBox_TeamA) (delegate Custom|TeamB%20Won))
  (Game|BindEventtoOnDestroyed (Variables|Default|GetSafeBox_TeamB) (delegate Custom|TeamA%20Won)))

(event Custom|SetWinnerEvent
  (params (DamagedActor :type Actor%20Object%20Reference) (Damage :type Float%20%28single-precision%29) (DamageType :type Damage%20Type%20Object%20Reference) (InstigatedBy :type Controller%20Object%20Reference) (DamageCauser :type Actor%20Object%20Reference))
  (bind _safebox_teama (Variables|Default|GetSafeBox_TeamA))
  (bind _safebox_teamb (Variables|Default|GetSafeBox_TeamB))
  (if (and (Utilities|IsValid _safebox_teama) (Utilities|IsValid _safebox_teamb))
    (Math|Integer|CompareInt (Math|Float|Truncate (Variables|/Game/Hero/Base/Blueprint/CP_Health.CP_Health_C|GetCurrentHealth (Variables|/Game/Map/Game/Heist/BP_SafeBox.BP_SafeBox_C|GetCP_Health _safebox_teama))) (Math|Float|Truncate (Variables|/Game/Hero/Base/Blueprint/CP_Health.CP_Health_C|GetCurrentHealth (Variables|/Game/Map/Game/Heist/BP_SafeBox.BP_SafeBox_C|GetCP_Health _safebox_teamb)))
      (:>
        (Variables|Default|SetWinner "NewEnumerator0"))
      (:==
        (Variables|Default|SetWinner "NewEnumerator2"))
      (:<
        (Variables|Default|SetWinner "NewEnumerator1")))))

(event Custom|GetSafeBox
  (bind _outactors (Actor|GetAllActorsOfClass "/Game/Map/Game/Heist/BP_SafeBox.BP_SafeBox_C"))
  (for _array_element _outactors
    (bind _asbp_safe_box (Utilities|Casting|CastToBP_SafeBox _array_element))
    (switch Utilities|FlowControl|Switch|SwitchonETeamType (Variables|/Game/Map/Game/Heist/BP_SafeBox.BP_SafeBox_C|GetSafeBoxTeamType _asbp_safe_box)
      (:NewEnumerator0
        (Variables|Default|SetSafeBox_TeamA _asbp_safe_box))
      (:NewEnumerator1
        (Variables|Default|SetSafeBox_TeamB _asbp_safe_box))))
  (bind _asgs_heist (Utilities|Casting|CastToGS_Heist (Game|GetGameState)))
  (Variables|/Game/Map/Game/Heist/GS_Heist.GS_Heist_C|SetSafeBox_TeamA _asgs_heist (Variables|Default|GetSafeBox_TeamA))
  (Variables|/Game/Map/Game/Heist/GS_Heist.GS_Heist_C|SetSafeBox_TeamB _asgs_heist (Variables|Default|GetSafeBox_TeamB)))

(event Custom|BindSafeBoxDamageEvent
  (EventDispatchers|BindEventtoOnTakeAnyDamage (Variables|Default|GetSafeBox_TeamA) (delegate Custom|SetWinnerEvent)))

(event EventBeginPlay
  (|CallParentFunction)
  (CallFunction|GetSafeBox)
  (Utilities|FlowControl|Delay 0.2)
  (CallFunction|BindSafeBoxDamageEvent)
  (CallFunction|BindSafeBoxDestroyEvent)
  (Utilities|FlowControl|Delay 1.0)
  (CallFunction|SpawnAI "NewEnumerator2" 6))

(fn ConstructionScript)