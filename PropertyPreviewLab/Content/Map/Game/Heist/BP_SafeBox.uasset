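; BP_SafeBox is a heist-map safe box with a team assignment and a large health pool.
; On BeginPlay it pauses health regeneration, sets the instance's team and health on its CPHealth component, and links itself to its WBP_SafeBox health widget.
; Any damage taken triggers CPHealth to show a damage number, and the construction script enlarges the Box component.
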(event Custom|ShowDamageNum
  (params (DamagedActor :type Actor%20Object%20Reference) (Damage :type Float%20%28single-precision%29) (DamageType :type Damage%20Type%20Object%20Reference) (InstigatedBy :type Controller%20Object%20Reference) (DamageCauser :type Actor%20Object%20Reference))
  ;[1 1 1] Set Team Type By Instance
  (Default|ShowDamage (Variables|Default|GetCP_Health) Damage))

(event EventBeginPlay
  (bind _cp_health (Variables|Default|GetCP_Health))
  ;[1 1 1] Set Team Type By Instance
  (Utilities|Time|PauseTimerbyHandle (Variables|/Game/Hero/Base/Blueprint/CP_Health.CP_Health_C|GetRestoreTimer _cp_health))
  (Variables|/Game/Hero/Base/Blueprint/CP_Health.CP_Health_C|SetTeamType _cp_health (Variables|TeamType|GetSafeBoxTeamType))
  (bind _output_get (Variables|/Game/Hero/Base/Blueprint/CP_Health.CP_Health_C|SetDefaultHealth _cp_health 4.5e+04))
  (Variables|/Game/Hero/Base/Blueprint/CP_Health.CP_Health_C|SetCurrentHealth _cp_health _output_get)
  (bind _aswbp_safe_box (Utilities|Casting|CastToWBP_SafeBox (UserInterface|GetUserWidgetObject (Variables|Default|GetHealth))))
  (Variables|/Game/UMG/WBP_SafeBox.WBP_SafeBox_C|SetSafeBox _aswbp_safe_box self)
  (EventDispatchers|BindEventtoOnTakeAnyDamage (delegate Custom|ShowDamageNum)))

(fn ConstructionScript
  (Transformation|SetWorldScale3D (Variables|Default|GetBox) "3.500000,3.500000,3.500000"))