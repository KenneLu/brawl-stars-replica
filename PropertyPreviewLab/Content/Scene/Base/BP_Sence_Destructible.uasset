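; BP_Sence_Destructible is a destructible scenery actor that can shake when hit and be ruined.
; Shake nudges the actor along a hit vector, then restores the transform saved at BeginPlay after a short delay.
; Ruined disables collision and, on the authority only, destroys the DestructibleBody component.
; The collision overlap only casts to BP_BulletBase, and nothing in this graph calls Shake or Ruined.
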(event OnComponentBeginOverlap(Collision)
  (params (OverlappedComponent :type Primitive%20Component%20Object%20Reference) (OtherActor :type Actor%20Object%20Reference) (OtherComp :type Primitive%20Component%20Object%20Reference) (OtherBodyIndex :type Integer) (bFromSweep :type Boolean) (SweepResult :type Hit%20Result%20Structure%20%28by%20ref%29))
  (Utilities|Casting|CastToBP_BulletBase OtherActor))

(event Custom|Ruined
  (Collision|SetCollisionEnabled (Variables|Default|GetCollision) "NoCollision")
  (Networking|SwitchHasAuthority
    (:Authority
      (Components|DestroyComponent (Variables|Default|GetDestructibleBody)))))

(event Custom|Shake
  (params (HitVector :type Vector))
  (Variables|Default|SetHitVector HitVector)
  (Transformation|AddActorLocalOffset self (* (Variables|Default|GetHitVector) 2.0) false false)
  (Utilities|FlowControl|Delay 0.2)
  (Transformation|SetActorTransform self (Variables|Default|GetOriginalTransfrom)))

(event EventBeginPlay
  (Variables|Default|SetOriginalTransfrom (Transformation|GetActorTransform self)))

(fn ConstructionScript
  (|CallParentFunction))