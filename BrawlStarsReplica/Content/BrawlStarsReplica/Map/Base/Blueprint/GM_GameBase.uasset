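; Base game mode for a Brawl Stars replica that runs match flow from player login through game over.
; Once enough players join and a timer sees a pawn, it announces the start, spawns six AI heroes at available player starts and enables input.
; SpawnAI picks random DT_Hero rows unless given a class.
; Level-matched music plays server-side, its tracked playback percent setting the start time sent to each PC_GameBase.
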(event Custom|GameOver
  ;[1 1 1] Game Manager
  (bind _returnvalue (Class|GameModeBase|GetNumPlayers))
  (for _index (range 0 (- _returnvalue 1))
    (bind _aspc_game_base (Utilities|Casting|CastToPC_GameBase (Game|GetPlayerController _index)))
    (Default|GameOver _aspc_game_base (Variables|Default|GetWinner))))

(event Custom|UpdateMusicPercent
  (params (PlayingSoundWave :type Sound%20Wave%20Object%20Reference) (PlaybackPercent :type Float%20%28single-precision%29))
  ;[1 1 1] Game Music Manager
  (Variables|Default|SetMusic%20Playback%20Percent PlaybackPercent))

(event Custom|PlayerInputEnable
  ;[1 1 1] Player Input Manager
  (Utilities|FlowControl|Delay 0.3)
  (bind _returnvalue (Class|GameModeBase|GetNumPlayers))
  (for _index (range 0 (- _returnvalue 1))
    (bind _aspc_game_base (Utilities|Casting|CastToPC_GameBase (Game|GetPlayerController _index)))
    (Default|PlayerControllerInputEnable _aspc_game_base)))

(event Custom|PlayerInputDisable
  ;[1 1 1] Player Input Manager
  (Utilities|FlowControl|Delay 0.3)
  (bind _returnvalue (Class|GameModeBase|GetNumPlayers))
  (for _index (range 0 (- _returnvalue 1))
    (bind _aspc_game_base (Utilities|Casting|CastToPC_GameBase (Game|GetPlayerController _index)))
    (Default|PlayerControllerInputDisable _aspc_game_base)))

(event Custom|GameBegin
  ;[1 1 1] Game Manager
  (Utilities|FlowControl|Delay 3.0)
  (bind _returnvalue (Class|GameModeBase|GetNumPlayers))
  (for _index (range 0 (- _returnvalue 1))
    (bind _aspc_game_base (Utilities|Casting|CastToPC_GameBase (Game|GetPlayerController _index)))
    (Default|PlayGameBeginSound _aspc_game_base)
    (Default|ShowGameBegin _aspc_game_base))
  (CallFunction|SpawnAI "NewEnumerator2" 6)
  (CallFunction|PlayerInputEnable)
  (Utilities|FlowControl|Delay 1.0)
  (CallFunction|PlayBackGroundMusic)
  (CallFunction|PlayMusic))

(event Custom|PlayBackGroundMusic
  ;[1 1 1] Game Music Manager
  (bind _asbp_game_instance (Utilities|Casting|CastToBP_GameInstance (Game|GetGameInstance)))
  (bind _output_get (Variables|Default|SetGame%20Music%20Volume (Variables|/Game/BrawlStarsReplica/Map/Base/Blueprint/BP_GameInstance.BP_GameInstance_C|GetGameMusicVolume _asbp_game_instance)))
  (bind _music (CallFunction|GetGameBackGroundMusic))
  (bind _returnvalue (Audio|CreateSound2D _music _output_get 1.0 0.0 0))
  (bind _output_get_2 (Variables|Default|SetBackGroundMusic _returnvalue))
  (EventDispatchers|BindEventtoOnAudioPlaybackPercent _output_get_2 (delegate Custom|UpdateMusicPercent))
  (Audio|Components|Audio|Play _output_get_2 0.0))

(event Custom|CustomEvent_0
  ;[1 1 1] Game Manager
  (Utilities|IsValid (Pawn|GetControlledPawn (stale EventPostLogin NewPlayer))
    (:Is%20Valid
      (CallFunction|GameBegin)
      (Utilities|Time|ClearandInvalidateTimerbyHandle (Variables|Default|GetCheckPlayerReadyTimer)))))

(event Custom|PlayMusic
  (bind _backgroundmusic (Variables|Default|GetBackGroundMusic))
  (bind _sound (Variables|/Script/Engine.AudioComponent|GetSound _backgroundmusic))
  ;[1 1 1] Game Music Manager
  (bind _returnvalue (Class|GameModeBase|GetNumPlayers))
  (for _index (range 0 (- _returnvalue 1))
    (bind _aspc_game_base (Utilities|Casting|CastToPC_GameBase (Game|GetPlayerController _index)))
    (Default|PlayGameBackGroundMusic _aspc_game_base _sound (Variables|Default|GetGame%20Music%20Volume) (* (Variables|/Script/Engine.SoundBase|GetDuration _sound) (Variables|Default|GetMusic%20Playback%20Percent)))))

(event EventPostLogin
  (params (NewPlayer :type Player%20Controller%20Object%20Reference))
  ;[1 1 1] Game Manager
  (bind _aspc_game_base (Utilities|Casting|CastToPC_GameBase NewPlayer))
  (Default|ShowTouchInterface _aspc_game_base)
  (Default|GameIntro _aspc_game_base)
  (Variables|Default|SetPlayerAmount (+ (Variables|Default|GetPlayerAmount) 1))
  (bind _pass (CallFunction|CheckPlayerAmount))
  (if _pass
    (bind _returnvalue (Utilities|Time|SetTimerbyEvent (delegate Custom|CustomEvent_0) 0.5 true))
    (Variables|Default|SetCheckPlayerReadyTimer _returnvalue)))

(fn ConstructionScript)

(fn SpawnAI
  (params (TeamType :type ETeamType%20Enum :default "NewEnumerator2") (Amount :type Integer) (HeroType :type BP%20Hero%20Base%20Class%20Reference))
  (LocalVariables|SetAIAmountRemain Amount)
  (bind _outactors (Actor|GetAllActorsOfClass "/Game/BrawlStarsReplica/Map/Base/Blueprint/BP_PlayerStart.BP_PlayerStart_C"))
  (bind _array_element (Utilities|Array|ForEachLoopwithBreak _outactors :!label _label)
    (:LoopBody
      (if (> (LocalVariables|GetAIAmountRemain) 0)
        (LocalVariables|SetPlayerStartPoint _array_element)
        (if (Utilities|Enum|Equal(Enum) TeamType "NewEnumerator2")
          (if (Variables|/Game/BrawlStarsReplica/Map/Base/Blueprint/BP_PlayerStart.BP_PlayerStart_C|GetisAvailable (LocalVariables|GetPlayerStartPoint)) :!label _label_2
            (Variables|/Game/BrawlStarsReplica/Map/Base/Blueprint/BP_PlayerStart.BP_PlayerStart_C|SetisAvailable (LocalVariables|GetPlayerStartPoint) false)
            (bind _herotype (LocalVariables|GetHeroType)
              (:then
                (LocalVariables|SetSpawnedHeroClass _herotype))
              (:else
                (bind _outrownames (DataTable|GetDataTableRowNames "/Game/BrawlStarsReplica/Hero/Base/Data/DT_Hero.DT_Hero"))
                (bind _returnvalue (Utilities|GetDataTableRow "/Game/BrawlStarsReplica/Hero/Base/Data/DT_Hero.DT_Hero" (Utilities|Array|Get(acopy) _outrownames (Math|Random|RandomInteger (Utilities|Array|Length _outrownames))))
                  (:then
                    (LocalVariables|SetSpawnedHeroClass (.HeroType (Utilities|Struct|BreakFHeroAttribute _returnvalue)))))))
            (bind _returnvalue_2 (Game|SpawnActorfromClass (LocalVariables|GetSpawnedHeroClass) (Math|Transform|MakeTransform (Transformation|GetActorLocation (LocalVariables|GetPlayerStartPoint)) "0, 0, 0" "1,1,1") "Undefined" 0 0))
            (LocalVariables|SetSpawnedHero _returnvalue_2)
            (Variables|/Game/BrawlStarsReplica/Hero/Base/Blueprint/BP_HeroBase.BP_HeroBase_C|SetTeamType (LocalVariables|GetSpawnedHero) (Variables|/Game/BrawlStarsReplica/Map/Base/Blueprint/BP_PlayerStart.BP_PlayerStart_C|GetTeamType (LocalVariables|GetPlayerStartPoint)))
            (bind _asaic_game_base (Utilities|Casting|CastToAIC_GameBase (Pawn|GetController (LocalVariables|GetSpawnedHero))))
            (bind _asps_game_base (Utilities|Casting|CastToPS_GameBase (Variables|/Script/Engine.Controller|GetPlayerState _asaic_game_base)))
            (Variables|/Game/BrawlStarsReplica/Map/Base/Blueprint/PS_GameBase.PS_GameBase_C|SetTeamType _asps_game_base (Variables|/Game/BrawlStarsReplica/Hero/Base/Blueprint/BP_HeroBase.BP_HeroBase_C|GetTeamType (LocalVariables|GetSpawnedHero)))
            (bind (_outname _hassuffix) (CallFunction|FLAdjustHeroName (Utilities|GetDisplayName (LocalVariables|GetSpawnedHero))))
            (if _hassuffix
              (Variables|/Game/BrawlStarsReplica/Map/Base/Blueprint/PS_GameBase.PS_GameBase_C|SetPlayerName _asps_game_base (Utilities|String|Append "AI " _outname))
              (else
                (Variables|/Game/BrawlStarsReplica/Map/Base/Blueprint/PS_GameBase.PS_GameBase_C|SetPlayerName _asps_game_base (Utilities|String|Append "AI " _outname))))
            (LocalVariables|SetAIAmountRemain (- (LocalVariables|GetAIAmountRemain) 1)))
          (elif (Utilities|Enum|Equal(Enum) TeamType (Variables|/Game/BrawlStarsReplica/Map/Base/Blueprint/BP_PlayerStart.BP_PlayerStart_C|GetTeamType (LocalVariables|GetPlayerStartPoint)))
            (goto _label_2)))
        (else
          (goto _label Break))))))

(fn GetGameBackGroundMusic
  (bind _returnvalue (Game|GetCurrentLevelName true))
  (LocalVariables|SetCurrentLevel _returnvalue)
  (bind _outrownames (DataTable|GetDataTableRowNames "/Game/BrawlStarsReplica/Map/Base/Data/DT_GameMusic.DT_GameMusic"))
  (for _array_element _outrownames
    (bind _returnvalue_2 (Utilities|GetDataTableRow "/Game/BrawlStarsReplica/Map/Base/Data/DT_GameMusic.DT_GameMusic" _array_element)
      (:then
        (if (Utilities|Enum|Equal(Enum) (Utilities|String|EnumtoString (.LevelName (Utilities|Struct|BreakFGameMusic _returnvalue_2))) (LocalVariables|GetCurrentLevel))
          (LocalVariables|SetMusicList (.Music (Utilities|Struct|BreakFGameMusic _returnvalue_2)))))))
  (bind _sound (CallFunction|FLGetRandomSound (LocalVariables|GetMusicList)))
  (return _sound))

(fn GetGameIntro
  (bind _returnvalue (Game|GetCurrentLevelName true))
  (bind _outrownames (DataTable|GetDataTableRowNames "/Game/BrawlStarsReplica/Map/Base/Data/DT_GameLevel.DT_GameLevel"))
  (for _array_element _outrownames
    (bind _returnvalue_2 (Utilities|GetDataTableRow "/Game/BrawlStarsReplica/Map/Base/Data/DT_GameLevel.DT_GameLevel" _array_element)
      (:then
        (if (Utilities|Enum|Equal(Enum) (Utilities|String|EnumtoString (.GameLevelName (Utilities|Struct|BreakFGameLevelAttribute _returnvalue_2))) _returnvalue)
          (return (.GameLeveChineseName (Utilities|Struct|BreakFGameLevelAttribute _returnvalue_2)) (.GameIntro (Utilities|Struct|BreakFGameLevelAttribute _returnvalue_2))))))))

(fn CheckPlayerAmount
  (bind _asbp_game_instance (Utilities|Casting|CastToBP_GameInstance (Game|GetGameInstance)))
  (return (>= (Variables|Default|GetPlayerAmount) (Variables|/Game/BrawlStarsReplica/Map/Base/Blueprint/BP_GameInstance.BP_GameInstance_C|GetPlayerAmount _asbp_game_instance))))