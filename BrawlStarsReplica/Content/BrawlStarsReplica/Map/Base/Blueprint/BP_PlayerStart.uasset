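; BP_PlayerStart is a team spawn point marker in the Brawl Stars replica map that tracks whether it is free.
; A sphere overlap sets IsAvailable false when a BP_HeroBase of the same TeamType enters and true when one leaves, without counting multiple occupants.
; Tick swaps the marker mesh material every frame to match availability.
; The construction script sets up the scaled, collision-free mesh and starts it as available.
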(event OnComponentBeginOverlap(Sphere)
  (params (OverlappedComponent :type Primitive%20Component%20Object%20Reference) (OtherActor :type Actor%20Object%20Reference) (OtherComp :type Primitive%20Component%20Object%20Reference) (OtherBodyIndex :type Integer) (bFromSweep :type Boolean) (SweepResult :type Hit%20Result%20Structure%20%28by%20ref%29))
  (bind _asbp_hero_base (Utilities|Casting|CastToBP_HeroBase OtherActor))
  (if (Utilities|Enum|Equal(Enum) (Variables|/Game/BrawlStarsReplica/Hero/Base/Blueprint/BP_HeroBase.BP_HeroBase_C|GetTeamType _asbp_hero_base) (Variables|Default|GetTeamType))
    (CallFunction|SetIsAvailable false)))

(event OnComponentEndOverlap(Sphere)
  (params (OverlappedComponent :type Primitive%20Component%20Object%20Reference) (OtherActor :type Actor%20Object%20Reference) (OtherComp :type Primitive%20Component%20Object%20Reference) (OtherBodyIndex :type Integer))
  (bind _asbp_hero_base (Utilities|Casting|CastToBP_HeroBase OtherActor))
  (if (Utilities|Enum|Equal(Enum) (Variables|/Game/BrawlStarsReplica/Hero/Base/Blueprint/BP_HeroBase.BP_HeroBase_C|GetTeamType _asbp_hero_base) (Variables|Default|GetTeamType))
    (CallFunction|SetIsAvailable true)))

(event Custom|SetIsAvailable
  (params (isAvailable :type Boolean))
  (Variables|Default|SetisAvailable isAvailable))

(event EventTick
  (params (DeltaSeconds :type Float%20%28single-precision%29))
  (bind _staticmesh (Variables|Default|GetStaticMesh))
  (if (Variables|Default|GetisAvailable)
    (Rendering|Material|SetMaterial _staticmesh 0 "/Game/BrawlStarsReplica/Map/Base/Asset/MI_Map_PlayerStartPoint_Avaliable.MI_Map_PlayerStartPoint_Avaliable")
    (else
      (Rendering|Material|SetMaterial _staticmesh 0 "/Game/BrawlStarsReplica/Map/Base/Asset/MI_Map_PlayerStartPoint_NotAvaliable.MI_Map_PlayerStartPoint_NotAvaliable"))))

(fn ConstructionScript
  (bind _staticmesh (Variables|Default|GetStaticMesh))
  (Components|StaticMesh|SetStaticMesh _staticmesh "/Game/BrawlStarsReplica/Map/Base/Asset/SM_Map_PlayerStartPoint.SM_Map_PlayerStartPoint")
  (Rendering|Material|SetMaterial _staticmesh 0 "/Game/BrawlStarsReplica/Map/Base/Asset/MI_Map_PlayerStartPoint_Avaliable.MI_Map_PlayerStartPoint_Avaliable")
  (Collision|SetCollisionEnabled _staticmesh "NoCollision")
  (Transformation|SetWorldScale3D _staticmesh "0.500000,0.500000,0.500000")
  (Variables|Default|SetisAvailable true))