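; Game state base for the Brawl Stars replica that runs the match countdown and ends the game when time runs out.
; On BeginPlay it looks up the current level in DT_GameMode and converts that row's minutes into seconds.
; After a short delay, a looping timer decrements GameCountDown each second, stopping at zero.
; GameCountDown's RepNotify calls GameOver on GM_GameBase at zero, where the game mode cast succeeds.
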(event Custom|GameTimeCountDown
  (if (>= (- (Variables|Default|GetGameCountDown) 1) 0)
    (Variables|Default|SetGameCountDown (- (Variables|Default|GetGameCountDown) 1))))

(event EventBeginPlay
  (CallFunction|InitCountDownTime)
  (Utilities|FlowControl|Delay 3.0)
  (Utilities|Time|SetTimerbyEvent (delegate Custom|GameTimeCountDown) 1.0 true))

(fn ConstructionScript)

(fn OnRepGameCountDown
  (if (== (Variables|Default|GetGameCountDown) 0)
    (bind _asgm_game_base (Utilities|Casting|CastToGM_GameBase (Game|GetGameMode)))
    (Default|GameOver _asgm_game_base)))

(fn InitCountDownTime
  (bind _returnvalue (Game|GetCurrentLevelName true))
  (bind _outrownames (DataTable|GetDataTableRowNames "/Game/BrawlStarsReplica/Map/Base/Data/DT_GameMode.DT_GameMode"))
  (for _array_element _outrownames
    (bind _returnvalue_2 (Utilities|GetDataTableRow "/Game/BrawlStarsReplica/Map/Base/Data/DT_GameMode.DT_GameMode" _array_element)
      (:then
        (if (Utilities|Enum|Equal(Enum) _returnvalue (Utilities|String|EnumtoString (.GameLevel (Utilities|Struct|BreakFGameModeAttribute _returnvalue_2))))
          (Variables|Default|SetGameCountDown (Math|Float|Truncate (* 60 (.CountDownTime_Min (Utilities|Struct|BreakFGameModeAttribute _returnvalue_2))))))))))