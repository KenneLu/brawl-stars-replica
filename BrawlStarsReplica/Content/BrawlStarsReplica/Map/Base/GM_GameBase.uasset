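; Base game mode for the Brawl Stars replica that spawns AI heroes and announces game over.
; SpawnAI claims available BP_PlayerStart points matching the requested team, with one enum value accepting any, and spawns the given hero or a random DT_Hero pick.
; Each bot takes the start point's team, copied to its PlayerState alongside a name parsed from its display name.
; GameOver forwards the winner to every player's PC_GameBase.
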(event Custom|GameOver
  (bind _returnvalue (Class|GameModeBase|GetNumPlayers))
  (for _index (range 0 (- _returnvalue 1))
    (bind _aspc_game_base (Utilities|Casting|CastToPC_GameBase (Game|GetPlayerController _index)))
    (Default|GameOver _aspc_game_base (Variables|Default|GetWinner))))

(fn ConstructionScript)

(fn SpawnAI
  (params (TeamType :type ETeamType%20Enum :default "NewEnumerator2") (Amount :type Integer) (HeroType :type BP%20Hero%20Base%20Class%20Reference))
  (LocalVariables|SetAmountRemain Amount)
  (bind _outactors (Actor|GetAllActorsOfClass "/Game/BrawlStarsReplica/Map/Base/BP_PlayerStart.BP_PlayerStart_C"))
  (bind _array_element (Utilities|Array|ForEachLoopwithBreak _outactors :!label _label)
    (:LoopBody
      (if (> (LocalVariables|GetAmountRemain) 0)
        (LocalVariables|SetPlayerStartPoint _array_element)
        (if (Utilities|Enum|Equal(Enum) TeamType "NewEnumerator2")
          (if (Variables|/Game/BrawlStarsReplica/Map/Base/BP_PlayerStart.BP_PlayerStart_C|GetisAvailable (LocalVariables|GetPlayerStartPoint)) :!label _label_2
            (Variables|/Game/BrawlStarsReplica/Map/Base/BP_PlayerStart.BP_PlayerStart_C|SetisAvailable (LocalVariables|GetPlayerStartPoint) false)
            (if (not (Utilities|IsValidClass HeroType))
              (bind _outrownames (DataTable|GetDataTableRowNames "/Game/BrawlStarsReplica/Hero/Base/Data/DT_Hero.DT_Hero"))
              (bind _returnvalue (Utilities|GetDataTableRow "/Game/BrawlStarsReplica/Hero/Base/Data/DT_Hero.DT_Hero" (Utilities|Array|Get(acopy) _outrownames (Math|Random|RandomInteger (Utilities|Array|Length _outrownames))))
                (:then
                  (bind _returnvalue_2 (Game|SpawnActorfromClass (.HeroType (Utilities|Struct|BreakFHeroAttribute _returnvalue)) (Math|Transform|MakeTransform (Transformation|GetActorLocation (LocalVariables|GetPlayerStartPoint)) "0, 0, 0" "1,1,1") "Undefined" 0 0))
                  (LocalVariables|SetSpawnedHero _returnvalue_2)))
              (else
                (bind _returnvalue_3 (Game|SpawnActorfromClass HeroType (Math|Transform|MakeTransform (Transformation|GetActorLocation (LocalVariables|GetPlayerStartPoint)) "0, 0, 0" "1,1,1") "Undefined" 0 0))
                (LocalVariables|SetSpawnedHero _returnvalue_3)))
            (Variables|/Game/BrawlStarsReplica/Hero/Base/Blueprint/BP_HeroBase.BP_HeroBase_C|SetTeamType (LocalVariables|GetSpawnedHero) (Variables|/Game/BrawlStarsReplica/Map/Base/BP_PlayerStart.BP_PlayerStart_C|GetTeamType (LocalVariables|GetPlayerStartPoint)))
            (bind _asaic_game_base (Utilities|Casting|CastToAIC_GameBase (Pawn|GetController (LocalVariables|GetSpawnedHero))))
            (bind _asps_game_base (Utilities|Casting|CastToPS_GameBase (Variables|/Script/Engine.Controller|GetPlayerState _asaic_game_base)))
            (Variables|/Game/BrawlStarsReplica/Map/Base/PS_GameBase.PS_GameBase_C|SetTeamType _asps_game_base (Variables|/Game/BrawlStarsReplica/Hero/Base/Blueprint/BP_HeroBase.BP_HeroBase_C|GetTeamType (LocalVariables|GetSpawnedHero)))
            (if (.ReturnValue (Utilities|String|Split (Utilities|String|Replace (Utilities|GetDisplayName (LocalVariables|GetSpawnedHero)) "BP_Hero_") "_"))
              (Variables|/Game/BrawlStarsReplica/Map/Base/PS_GameBase.PS_GameBase_C|SetPlayerName _asps_game_base (.LeftS (Utilities|String|Split (Utilities|String|Replace (Utilities|GetDisplayName (LocalVariables|GetSpawnedHero)) "BP_Hero_") "_")))
              (else
                (Variables|/Game/BrawlStarsReplica/Map/Base/PS_GameBase.PS_GameBase_C|SetPlayerName _asps_game_base (Utilities|String|Replace (Utilities|GetDisplayName (LocalVariables|GetSpawnedHero)) "BP_Hero_"))))
            (LocalVariables|SetAmountRemain (- (LocalVariables|GetAmountRemain) 1)))
          (elif (Utilities|Enum|Equal(Enum) TeamType (Variables|/Game/BrawlStarsReplica/Map/Base/BP_PlayerStart.BP_PlayerStart_C|GetTeamType (LocalVariables|GetPlayerStartPoint)))
            (goto _label_2)))
        (else
          (goto _label Break))))))