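; Base player controller for a Brawl Stars replica, handling hero spawning, team setup, matchmaking UI and game over.
; On begin play it reads hero (default Nita) and team from the game instance, passes them to SetServerHeroTypeAndTeamType, then possesses a hero at a free team-matched player start.
; After a short possession delay it flips rotation for one team and shows the countdown.
; It also handles delayed respawns and a viewport-size settings widget.
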(event Custom|RespawnHero
  ;[1 1 1] RespawnHero
  ;;[1 1 1] Hero respawn interval
  (Utilities|FlowControl|Delay 3.0)
  (CallFunction|SpawnHero))

(event Custom|SetServerHeroTypeAndTeamType
  (params (ClientHeroType :type BP%20Hero%20Base%20Class%20Reference) (ClientTeamType :type ETeamType%20Enum :default "NewEnumerator0"))
  ;[1 1 1] Set Server HeroType And TeamType
  (Variables|Default|SetHero%20Type ClientHeroType)
  (bind _output_get (Variables|Default|SetTeamType ClientTeamType))
  (bind _asps_game_base (Utilities|Casting|CastToPS_GameBase (Variables|GetPlayerState)))
  (Variables|/Game/BrawlStarsReplica/Map/Base/PS_GameBase.PS_GameBase_C|SetTeamType _asps_game_base _output_get))

(event Custom|ClientGetHeroTypeAndSpawn
  ;[1 1 1] Get Hero Type Instance And Spawn
  (bind _asbp_game_instance (Utilities|Casting|CastToBP_GameInstance (Game|GetGameInstance)))
  (if (Utilities|IsValidClass (Variables|/Game/BrawlStarsReplica/Map/Base/BP_GameInstance.BP_GameInstance_C|GetHeroTypeInstacne _asbp_game_instance))
    (Variables|Default|SetHero%20Type (Variables|/Game/BrawlStarsReplica/Map/Base/BP_GameInstance.BP_GameInstance_C|GetHeroTypeInstacne _asbp_game_instance))
    (else
      (Variables|Default|SetHero%20Type "/Game/BrawlStarsReplica/Hero/Nita/Blueprint/BP_Hero_Nita.BP_Hero_Nita_C")))
  (Variables|Default|SetTeamType (Variables|/Game/BrawlStarsReplica/Map/Base/BP_GameInstance.BP_GameInstance_C|GetTeamTypeInstance _asbp_game_instance))
  (CallFunction|SetServerHeroTypeandTeamType (Variables|Default|GetHero%20Type) (Variables|Default|GetTeamType))
  (CallFunction|SpawnHero))

(event Custom|GetMatchingState
  ;[1 1 1] Matching
  ;;[1 1 1] Get Matching State
  (bind _asgm_match (Utilities|Casting|CastToGM_Match (Game|GetGameMode)))
  (Variables|Default|SetGM%20Player%20Amount (Variables|/Game/BrawlStarsReplica/Map/Login/Match/GM_Match.GM_Match_C|GetGM_PlayerSequence _asgm_match))
  (Variables|Default|SetGM%20Level%20Max%20Player (Variables|/Game/BrawlStarsReplica/Map/Login/Match/GM_Match.GM_Match_C|GetGM_PlayerMax _asgm_match)))

(event Custom|SaveTeamTypeInstance
  (params (TeamTypeInstance :type ETeamType%20Enum :default "NewEnumerator0"))
  ;[1 1 1] Matching
  ;;[1 1 1] Save Team Type Instance
  (bind _asbp_game_instance (Utilities|Casting|CastToBP_GameInstance (Game|GetGameInstance)))
  (Variables|/Game/BrawlStarsReplica/Map/Base/BP_GameInstance.BP_GameInstance_C|SetTeamTypeInstance _asbp_game_instance TeamTypeInstance))

(event Custom|SpawnHero
  ;[1 1 1] Spawn Hero
  (bind _outactors (Actor|GetAllActorsOfClass "/Game/BrawlStarsReplica/Map/Base/BP_PlayerStart.BP_PlayerStart_C"))
  (bind _array_element (Utilities|Array|ForEachLoopwithBreak _outactors :!label _label)
    (:LoopBody
      (if (and (Variables|/Game/BrawlStarsReplica/Map/Base/BP_PlayerStart.BP_PlayerStart_C|GetisAvailable _array_element) (Utilities|Enum|Equal(Enum) (Variables|/Game/BrawlStarsReplica/Map/Base/BP_PlayerStart.BP_PlayerStart_C|GetTeamType _array_element) (Variables|Default|GetTeamType)))
        (Variables|/Game/BrawlStarsReplica/Map/Base/BP_PlayerStart.BP_PlayerStart_C|SetisAvailable _array_element false)
        (Utilities|FlowControl|Sequence
          (:then_0
            (bind _returnvalue (Game|SpawnActorfromClass (Variables|Default|GetHero%20Type) (Math|Transform|MakeTransform (.location (Transformation|GetActorTransform _array_element)) "0, 0, 0" "1,1,1") "Undefined" self 0))
            (Pawn|Possess _returnvalue)
            (bind _asps_game_base (Utilities|Casting|CastToPS_GameBase (Variables|GetPlayerState)))
            (if (.ReturnValue (Utilities|String|Split (Utilities|String|Replace (Utilities|GetDisplayName _returnvalue) "BP_Hero_") "_"))
              (Variables|/Game/BrawlStarsReplica/Map/Base/PS_GameBase.PS_GameBase_C|SetPlayerName _asps_game_base (.LeftS (Utilities|String|Split (Utilities|String|Replace (Utilities|GetDisplayName _returnvalue) "BP_Hero_") "_")))
              (else
                (Variables|/Game/BrawlStarsReplica/Map/Base/PS_GameBase.PS_GameBase_C|SetPlayerName _asps_game_base (Utilities|String|Replace (Utilities|GetDisplayName _returnvalue) "BP_Hero_")))))
          (:then_1
            (goto _label Break)))))))

(event Custom|ShowMatchingUMG
  ;[1 1 1] Matching
  ;;[1 1 1] Show Matching UMG
  (if (Pawn|IsLocalController)
    (Utilities|IsValid (Variables|Default|GetWBP_Matching)
      (:Is%20Valid
        (Widget|RemovefromParent (Variables|Default|GetWBP_Matching)))
      (:Is%20Not%20Valid
        _))
    (bind _returnvalue (UserInterface|CreateWidget "/Game/BrawlStarsReplica/UMG/Login/WBP_LoginMatching.WBP_LoginMatching_C" self))
    (bind _output_get (Variables|Default|SetWBP_Matching _returnvalue))
    (UserInterface|Viewport|AddtoViewport _output_get 0)))

(event Custom|GameOver
  (params (WinnerTeam :type ETeamType%20Enum :default "NewEnumerator2"))
  ;[1 1 1] Game Over
  (if (Pawn|IsLocalController)
    (bind _returnvalue (UserInterface|CreateWidget "/Game/BrawlStarsReplica/UMG/Game/Base/WBP_GameBase_GameOver.WBP_GameBase_GameOver_C"))
    (Variables|/Game/BrawlStarsReplica/UMG/Game/Base/WBP_GameBase_GameOver.WBP_GameBase_GameOver_C|SetWinnerTeam _returnvalue WinnerTeam)
    (UserInterface|Viewport|AddtoPlayerScreen _returnvalue)
    (Pawn|UnPossess)
    (Game|SetGamePaused true)))

(event Custom|SetPlayerControllerRotationByTeamType
  (bind _returnvalue (Pawn|GetControlledPawn))
  ;[1 1 1] Set Player Controller Rotation
  (if (Utilities|Enum|Equal(Enum) (Variables|Default|GetTeamType) "NewEnumerator1")
    (Utilities|IsValid _returnvalue
      (:Is%20Valid
        (Transformation|SetActorRotation _returnvalue (Math|Rotator|MakeRotator 0.0 0.0 1.8e+02))
        (Class|Controller|SetInitialLocationandRotation (Transformation|GetActorLocation _returnvalue) (Math|Rotator|MakeRotator 0.0 0.0 1.8e+02))))))

(event EventBeginPlay
  ;[1 1 1] Init Hero And PlayerController Rotation
  (if (Pawn|IsLocalPlayerController)
    (CallFunction|ClientGetHeroTypeandSpawn)
    ;;[1 1 1] Wait Until Possess
    (Utilities|FlowControl|Delay 0.2)
    (CallFunction|SetPlayerControllerRotationbyTeamType)
    ;[1 1 1] Init UHD
    (Utilities|Casting|CastToGS_GameBase (Game|GetGameState))
    (bind _returnvalue (UserInterface|CreateWidget "/Game/BrawlStarsReplica/UMG/Game/Base/WBP_GameBase_CountDown.WBP_GameBase_CountDown_C"))
    (UserInterface|Viewport|AddtoViewport _returnvalue 0)))

(event Input|ActionEvents|InputActionGameSetting
  (params (Key :type Key%20Structure :default "None"))
  (:Pressed
    (bind _returnvalue (UserInterface|CreateWidget "/Game/BrawlStarsReplica/UMG/Viewport/WBP_ChangeViewportSize.WBP_ChangeViewportSize_C"))
    (UserInterface|Viewport|AddtoViewport _returnvalue 0)))

(fn ConstructionScript)