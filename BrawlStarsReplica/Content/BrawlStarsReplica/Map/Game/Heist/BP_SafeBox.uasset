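; Safe box objective for the Heist mode of a Brawl Stars replica, with a configurable team and health.
; On BeginPlay it initializes its CPHealth component from those settings with restore disabled, and passes itself to the Heist safe box widget in its Health widget component.
; Its any-damage event forwards the damage amount to CPHealth to display damage numbers.
; The construction script sets the Box component's scale.
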(event Custom|ShowDamageNum
  (params (DamagedActor :type Actor%20Object%20Reference) (Damage :type Float%20%28single-precision%29) (DamageType :type Damage%20Type%20Object%20Reference) (InstigatedBy :type Controller%20Object%20Reference) (DamageCauser :type Actor%20Object%20Reference))
  (Default|ShowDamage (Variables|Default|GetCP_Health) Damage))

(event EventBeginPlay
  (bind _cp_health (Variables|Default|GetCP_Health))
  (Variables|/Game/BrawlStarsReplica/Hero/Base/Blueprint/CP_Health.CP_Health_C|SetCanRestore _cp_health false)
  (Variables|/Game/BrawlStarsReplica/Hero/Base/Blueprint/CP_Health.CP_Health_C|SetTeamType _cp_health (Variables|TeamType|GetSafeBoxTeamType))
  (bind _output_get (Variables|/Game/BrawlStarsReplica/Hero/Base/Blueprint/CP_Health.CP_Health_C|SetDefaultHealth _cp_health (Variables|Default|GetSafeBoxHealth)))
  (Variables|/Game/BrawlStarsReplica/Hero/Base/Blueprint/CP_Health.CP_Health_C|SetCurrentHealth _cp_health _output_get)
  (bind _aswbp_game_heist_safe_box (Utilities|Casting|CastToWBP_Game_Heist_SafeBox (UserInterface|GetUserWidgetObject (Variables|Default|GetHealth))))
  (Variables|/Game/BrawlStarsReplica/UMG/Game/Heist/WBP_Game_Heist_SafeBox.WBP_Game_Heist_SafeBox_C|SetSafeBox _aswbp_game_heist_safe_box self)
  (EventDispatchers|BindEventtoOnTakeAnyDamage (delegate Custom|ShowDamageNum)))

(fn ConstructionScript
  (Transformation|SetWorldScale3D (Variables|Default|GetBox) "3.500000,3.500000,3.500000"))