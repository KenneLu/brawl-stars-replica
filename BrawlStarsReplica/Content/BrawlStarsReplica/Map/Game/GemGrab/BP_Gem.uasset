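; BP_Gem is the collectible gem for the Gem Grab mode, launched through SetVelocity on its projectile movement in local space.
; When a BP_HeroBase overlaps PickupDetect, it credits the local player's PC_Game_GemGrab or the hero's AI controller via GetGem.
; Picked then destroys the gem and plays a 2D pickup sound; non-local player heroes also trigger this, without a GetGem call.
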(event OnComponentBeginOverlap(PickupDetect)
  (params (OverlappedComponent :type Primitive%20Component%20Object%20Reference) (OtherActor :type Actor%20Object%20Reference) (OtherComp :type Primitive%20Component%20Object%20Reference) (OtherBodyIndex :type Integer) (bFromSweep :type Boolean) (SweepResult :type Hit%20Result%20Structure%20%28by%20ref%29))
  (bind _asbp_hero_base (Utilities|Casting|CastToBP_HeroBase OtherActor))
  (Utilities|Casting|CastToPC_GameBase (Pawn|GetController _asbp_hero_base)
    (:then
      (if (Pawn|IsLocallyControlled _asbp_hero_base)
        (bind _aspc_game_gem_grab (Utilities|Casting|CastToPC_Game_GemGrab (Game|GetPlayerController 0)))
        (Default|GetGem _aspc_game_gem_grab)))
    (:CastFailed
      (bind _asaic_game_base (Utilities|Casting|CastToAIC_GameBase (Pawn|GetController _asbp_hero_base)))
      (Default|GetGem _asaic_game_base)))
  (CallFunction|Picked))

(event Custom|SetVelocity
  (params (NewVelocity :type Vector))
  (Game|Components|ProjectileMovement|SetVelocityinLocalSpace (Variables|Default|GetProjectileMovement) NewVelocity))

(event Custom|Picked
  (Actor|DestroyActor)
  (Audio|PlaySound2D "/Game/BrawlStarsReplica/Sound/Game/GemGrab/get_pickup_06.get_pickup_06" 0.2 1.0 0.0 0 0))

(fn ConstructionScript
  (Transformation|SetWorldScale3D (Variables|Default|GetSphere) "2.000000,2.000000,2.000000")
  (Transformation|SetWorldScale3D (Variables|Default|GetPickupDetect) "3.000000,3.000000,3.000000"))