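; Player controller for the Gem Grab mode that shows the mode UI and handles gem pickup and loss.
; For local controllers, a one-second timer creates a gem counter widget per hero, mapped to its player state.
; Tick updates each count, projects it to the hero's screen position and binds hero destruction.
; Hero death removes the widget, scatters the carried gems, reports the loss to GM_GemGrab and zeroes the count.
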(event Custom|GetHeroGemUIInstatnce
  (if (Pawn|IsLocalController)
    (bind _outactors (Actor|GetAllActorsOfClass "/Game/BrawlStarsReplica/Hero/Base/Blueprint/BP_HeroBase.BP_HeroBase_C"))
    (for _array_element _outactors
      (Variables|Default|SetHeroInstance _array_element)
      (if (not (Utilities|Map|Contains (Variables|Default|GetHeroGemWidget) (Variables|Default|GetHeroInstance)))
        (bind _returnvalue (UserInterface|CreateWidget "/Game/BrawlStarsReplica/UMG/Game/GemGrab/WBP_Game_GemGrab_GemAmount.WBP_Game_GemGrab_GemAmount_C"))
        (bind _output_get (Variables|Default|SetGemWidgetInstance _returnvalue))
        (UserInterface|Viewport|AddtoViewport _output_get 0)
        (bind _asps_game_gem_grab (Utilities|Casting|CastToPS_Game_GemGrab (Variables|/Script/Engine.Pawn|GetPlayerState (Variables|Default|GetHeroInstance))))
        (Utilities|Map|Add (Variables|Default|GetHeroGemWidget) (Variables|Default|GetHeroInstance) (Utilities|Struct|MakeFHeroGem (Variables|Default|GetGemWidgetInstance) _asps_game_gem_grab))))))

(event Custom|UpdateGemUI
  (if (Pawn|IsLocalController)
    ;[1 1 1] For Loop GemUI
    (bind _keys (Utilities|Map|Keys (Variables|Default|GetHeroGemWidget)))
    (for _array_element _keys
      (bind _output_get (Variables|Default|SetHeroInstance _array_element))
      (Variables|Default|SetGemWidgetInstance (.gemwidget (.Value (Utilities|Map|Find (Variables|Default|GetHeroGemWidget) _output_get))))
      ;[1 1 1] GemAmount
      (bind _output_get_2 (Variables|Default|SetPlayerStateInstance (.heroplayerstate (.Value (Utilities|Map|Find (Variables|Default|GetHeroGemWidget) _output_get)))))
      (Variables|/Game/BrawlStarsReplica/UMG/Game/GemGrab/WBP_Game_GemGrab_GemAmount.WBP_Game_GemGrab_GemAmount_C|SetGemAmount (Variables|Default|GetGemWidgetInstance) (Variables|/Game/BrawlStarsReplica/Map/Game/GemGrab/PS_Game_GemGrab.PS_Game_GemGrab_C|GetGemAmount _output_get_2))
      ;[1 1 1] Widget Screen Position
      (Class|UserWidget|SetPositioninViewport (Variables|Default|GetGemWidgetInstance) (.ScreenPosition (Class|GameplayStatics|ProjectWorldtoScreen self (Transformation|GetActorLocation (Variables|Default|GetHeroInstance)) false)) true)
      (Game|BindEventtoOnDestroyed (Variables|Default|GetHeroInstance) (delegate Custom|Die)))))

(event Custom|GetGem
  (bind _asps_game_gem_grab (Utilities|Casting|CastToPS_Game_GemGrab (Variables|Default|GetPlayerState)))
  (Variables|/Game/BrawlStarsReplica/Map/Game/GemGrab/PS_Game_GemGrab.PS_Game_GemGrab_C|SetGemAmount _asps_game_gem_grab (+ (Variables|/Game/BrawlStarsReplica/Map/Game/GemGrab/PS_Game_GemGrab.PS_Game_GemGrab_C|GetGemAmount _asps_game_gem_grab) 1))
  (bind _asgm_gem_grab (Utilities|Casting|CastToGM_GemGrab (Game|GetGameMode)))
  (Default|GetGem _asgm_gem_grab (Variables|Default|GetTeamType)))

(event Custom|Die
  (params (DestroyedActor :type Actor%20Object%20Reference))
  ;[1 1 1] Get Instance
  (bind _asbp_hero_base (Utilities|Casting|CastToBP_HeroBase DestroyedActor))
  (bind _output_get (Variables|Default|SetHeroInstance _asbp_hero_base))
  (Variables|Default|SetHeroDieLocation (Transformation|GetActorLocation _output_get))
  (Variables|Default|SetGemWidgetInstance (.gemwidget (.Value (Utilities|Map|Find (Variables|Default|GetHeroGemWidget) (Variables|Default|GetHeroInstance)))))
  (Variables|Default|SetPlayerStateInstance (.heroplayerstate (.Value (Utilities|Map|Find (Variables|Default|GetHeroGemWidget) (Variables|Default|GetHeroInstance)))))
  ;[1 1 1] Clear Gem Widget
  (Widget|RemovefromParent (Variables|Default|GetGemWidgetInstance))
  (Utilities|Map|Remove (Variables|Default|GetHeroGemWidget) (Variables|Default|GetHeroInstance))
  ;[1 1 1] Clear Gem
  (CallFunction|LossGem (Variables|Default|GetPlayerStateInstance) (Variables|Default|GetHeroDieLocation)))

(event Custom|LossGem
  (params (PlayerState :type PS%20Game%20Gem%20Grab%20Object%20Reference) (DieLocation :type Vector))
  (bind (_x _y _z) (Math|Vector|BreakVector DieLocation))
  (for _index (range 0 (- (Variables|/Game/BrawlStarsReplica/Map/Game/GemGrab/PS_Game_GemGrab.PS_Game_GemGrab_C|GetGemAmount PlayerState) 1))
    (bind _returnvalue (Game|SpawnActorfromClass "/Game/BrawlStarsReplica/Map/Game/GemGrab/BP_Gem.BP_Gem_C" (Math|Transform|MakeTransform (Math|Vector|MakeVector _x _y (+ _z 2e+02)) "0, 0, 0" "1,1,1") "AdjustIfPossibleButAlwaysSpawn" 0 0))
    (Utilities|IsValid _returnvalue
      (:Is%20Valid
        (Default|SetVelocity _returnvalue (* (+ (Math|Vector|GetUpVector "0, 0, 0") (Math|Vector|MakeVector (/ (Math|Random|RandomFloatinRange -1e+02 1e+02) 1e+02) (/ (Math|Random|RandomFloatinRange -1e+02 1e+02) 1e+02) 0.0)) 3e+02)))))
  (bind _asgm_gem_grab (Utilities|Casting|CastToGM_GemGrab (Game|GetGameMode)))
  (Default|LossGem _asgm_gem_grab (Variables|/Game/BrawlStarsReplica/Map/Base/PS_GameBase.PS_GameBase_C|GetTeamType PlayerState) (Variables|/Game/BrawlStarsReplica/Map/Game/GemGrab/PS_Game_GemGrab.PS_Game_GemGrab_C|GetGemAmount PlayerState))
  (Variables|/Game/BrawlStarsReplica/Map/Game/GemGrab/PS_Game_GemGrab.PS_Game_GemGrab_C|SetGemAmount PlayerState 0))

(event Custom|Update%20Hero%20UI%20Instantce
  (CallFunction|GetHeroGemUIInstatnce))

(event EventBeginPlay
  (|CallParentFunction)
  (Utilities|Time|SetTimerbyEvent (delegate Custom|Update%20Hero%20UI%20Instantce) 1.0 true)
  ;[1 1 1] GemGrab UMG
  (if (Pawn|IsLocalController)
    (bind _returnvalue (UserInterface|CreateWidget "/Game/BrawlStarsReplica/UMG/Game/GemGrab/WBP_Game_GemGrab.WBP_Game_GemGrab_C"))
    (UserInterface|Viewport|AddtoViewport _returnvalue 0)))

(event EventTick
  (params (DeltaSeconds :type Float%20%28single-precision%29))
  (CallFunction|UpdateGemUI))

(fn ConstructionScript
  (|CallParentFunction))