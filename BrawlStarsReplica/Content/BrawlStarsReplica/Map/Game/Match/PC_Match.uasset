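; Player controller for the matchmaking screen: it shows the mouse cursor and fades in looping matching music for the local player on BeginPlay.
; ShowMatchingUMG replaces any existing matching widget with a new WBP_LoginMatch on the local viewport.
; GetMatchingState copies the current player sequence and max player count from GM_Match.
; SaveTeamTypeInstance stores the given team type in BP_GameInstance.
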(event Custom|PlayMatchingMusic
  (if (Pawn|IsLocalController)
    (bind _returnvalue (Audio|CreateSound2D "/Game/BrawlStarsReplica/Sound/Game/Match/draw_screen_loop_4x_01.draw_screen_loop_4x_01" 0.5 1.0 0.0 0))
    (Audio|Components|Audio|FadeIn _returnvalue 2.0 0.5 0.0 "Linear" :!class /Script/Engine.AudioComponent)))

(event Custom|GetMatchingState
  ;[1 1 1] Get Matching State
  (bind _asgm_match (Utilities|Casting|CastToGM_Match (Game|GetGameMode)))
  (Variables|Default|SetGM%20Player%20Amount (Variables|/Game/BrawlStarsReplica/Map/Game/Match/GM_Match.GM_Match_C|GetGM_PlayerSequence _asgm_match))
  (Variables|Default|SetGM%20Level%20Max%20Player (Variables|/Game/BrawlStarsReplica/Map/Game/Match/GM_Match.GM_Match_C|GetGM_PlayerMax _asgm_match)))

(event Custom|SaveTeamTypeInstance
  (params (TeamTypeInstance :type ETeamType%20Enum :default "NewEnumerator0"))
  ;[1 1 1] Save Team Type Instance
  (bind _asbp_game_instance (Utilities|Casting|CastToBP_GameInstance (Game|GetGameInstance)))
  (Variables|/Game/BrawlStarsReplica/Map/Base/Blueprint/BP_GameInstance.BP_GameInstance_C|SetTeamTypeInstance _asbp_game_instance TeamTypeInstance))

(event Custom|ShowMatchingUMG
  ;[1 1 1] Show Matching UMG
  (if (Pawn|IsLocalController)
    (bind _wbp_matching (Variables|Default|GetWBP_Matching)
      (:then
        (Widget|RemovefromParent _wbp_matching))
      (:else
        _))
    (bind _returnvalue (UserInterface|CreateWidget "/Game/BrawlStarsReplica/UMG/Login/WBP_LoginMatch.WBP_LoginMatch_C" self))
    (bind _output_get (Variables|Default|SetWBP_Matching _returnvalue))
    (UserInterface|Viewport|AddtoViewport _output_get 0)))

(event EventBeginPlay
  (|CallParentFunction)
  (Variables|Default|SetbShowMouseCursor true)
  (CallFunction|PlayMatchingMusic))

(event EventTick
  (params (DeltaSeconds :type Float%20%28single-precision%29)))

(fn ConstructionScript
  (|CallParentFunction))