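; Player controller for the login room that shows the login UI and exhibits the player's selected hero.
; On BeginPlay, the local controller adds the login widget and shows the mouse cursor.
; ExhibitHero reads the hero type from the game instance and spawns it at this room number's exhibition point.
; After a short delay, the view switches to the exhibition camera, found by matching display names built from the room number.
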(event Custom|UseRoomCameraView
  (params (NewParam :type Boolean))
  ;[1 1 1] Use Room Camera View
  (Variables|Default|SetExhibitCamera (Utilities|String|Append "BP_ExhibitionCamera_Player" (Utilities|String|ToString(Integer) (Variables|Default|GetPlayerRoomNum))))
  (bind _outactors (Actor|GetAllActorsOfClass "/Game/BrawlStarsReplica/Map/Base/BP_ExhibitionCamera.BP_ExhibitionCamera_C"))
  (bind (_array_element _array_index) (Utilities|Array|ForEachLoopwithBreak _outactors :!label _label)
    (:LoopBody
      (if (Utilities|Enum|Equal(Enum) (Utilities|GetDisplayName _array_element) (Variables|Default|GetExhibitCamera))
        (Utilities|FlowControl|Sequence
          (:then_0
            (Game|Player|SetViewTargetwithBlend _array_element 0.0 "VTBlend_Linear" 0.0 false))
          (:then_1
            (goto _label Break)))))
    (:Completed
      (if (== _array_index (- (Utilities|Array|Length _outactors) 1))
        (Development|PrintString (Utilities|String|Append "Couldn't Find Camera Named: " (Variables|Default|GetExhibitCamera)))))))

(event Custom|ExhibitHero
  ;[1 1 1] Exhibit Hero
  (bind _herotypeinstance (CallFunction|GetHeroTypefromGameInstance))
  (CallFunction|SpawnHeroforShow _herotypeinstance))

(event Custom|SpawnHeroForShow
  (params (ShowHeroType :type BP%20Hero%20Base%20Class%20Reference))
  ;[1 1 1] Spawn Hero For Show
  (Variables|Default|SetCurrentHeroType ShowHeroType)
  (CallFunction|GetHeroExhibitionPointTransfrom (Utilities|String|Append "BP_ExhibitionPoint_Player" (Utilities|String|ToString(Integer) (Variables|Default|GetPlayerRoomNum))))
  (for (_array_element _array_index) (Variables|Default|GetExhibitionPointTransfrom)
    (bind _returnvalue (Game|SpawnActorfromClass (Variables|Default|GetCurrentHeroType) _array_element "Undefined" 0 0))
    (Utilities|IsValid _returnvalue
      (:Is%20Valid
        (Utilities|Array|SetArrayElem (Variables|Default|GetExhibitionHero) _array_index _returnvalue true)
        ;;[1 1 1] Wait For Camera Ready
        (Utilities|FlowControl|Delay 0.1)
        (CallFunction|UseRoomCameraView false))
      (:Is%20Not%20Valid
        (Development|PrintString (Utilities|String|Append "Spawn Exhibition Hero " (Utilities|String|ToString(Integer) (Variables|Default|GetPlayerRoomNum)) " class " (Utilities|GetClassDisplayName (Variables|Default|GetCurrentHeroType)) "Faild!"))))))

(event EventBeginPlay
  ;[1 1 1] UMG
  (|CallParentFunction)
  (if (Pawn|IsLocalController)
    (bind _returnvalue (UserInterface|CreateWidget "/Game/BrawlStarsReplica/UMG/Login/WBP_LoginBase.WBP_LoginBase_C" self))
    (UserInterface|Viewport|AddtoViewport _returnvalue 0)
    (Variables|Default|SetbShowMouseCursor true)))

(fn ConstructionScript)