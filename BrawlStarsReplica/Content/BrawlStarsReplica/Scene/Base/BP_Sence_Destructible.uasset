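; Base destructible scene prop for a Brawl Stars replica that reacts to hits and can be ruined.
; Shake nudges the actor along the hit vector, restores its BeginPlay transform shortly after, spawns a hit spark and occasionally plays a sound.
; Ruined disables collision, destroys the body component only with authority and briefly activates explosion particles.
; Neither event is triggered within this Blueprint, and no health is tracked here.
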(event Custom|Ruined
  (bind _explosionsparticle (Variables|Default|GetExplosionsParticle))
  (Collision|SetCollisionEnabled (Variables|Default|GetCollision) "NoCollision")
  (Networking|SwitchHasAuthority
    (:Authority
      (Components|DestroyComponent (Variables|Default|GetDestructibleBody)))
    (:Remote
      _))
  (Components|Activation|Activate _explosionsparticle false)
  (Utilities|FlowControl|Delay 1.0)
  (Components|Activation|Deactivate _explosionsparticle))

(event Custom|Shake
  (params (HitVector :type Vector) (HitLocation :type Vector))
  (Variables|Default|SetHitVector HitVector)
  (Transformation|AddActorLocalOffset self (* (Variables|Default|GetHitVector) 2.0) false false)
  (Utilities|FlowControl|Sequence
    (:then_0
      ;[1 1 1] Make Shake Visual Effect
      (Utilities|FlowControl|Delay 0.2)
      (Transformation|SetActorTransform self (Variables|Default|GetOriginalTransfrom)))
    (:then_1
      (bind _happen (CallFunction|FLEventOdds 0.4))
      (if _happen
        (Audio|PlaySoundatLocation "/Game/BrawlStarsReplica/Sound/Game/Event/guntown_select_char_01.guntown_select_char_01" (Transformation|GetActorLocation) "0, 0, 0" 0.07 1.0 0.0 "/Game/BrawlStarsReplica/Sound/Blueprint/SA_Bullet.SA_Bullet" 0 0)))
    (:then_2
      (Game|SpawnActorfromClass "/Game/BrawlStarsReplica/Scene/Base/BP_Sence_HitSpark.BP_Sence_HitSpark_C" (Math|Transform|MakeTransform HitLocation "0, 0, 0" "1,1,1") "AdjustIfPossibleButAlwaysSpawn" 0 0))))

(event EventBeginPlay
  (Variables|Default|SetOriginalTransfrom (Transformation|GetActorTransform self)))

(fn ConstructionScript
  (|CallParentFunction))