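; BP_SenceBase is a base scene-object actor that can interrupt hero launch abilities when its CanStopLaunch flag is set.
; A Collision hit by BP_Hero_Primo calls ServerStopLaunch on that hero's LaunchAimingManager if it is valid and mid-launch.
; A Collision overlap with Nita's ultimate bullet makes the same call on the bullet's Nita instigator, without those checks.
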(event OnComponentHit(Collision)
  (params (HitComponent :type Primitive%20Component%20Object%20Reference) (OtherActor :type Actor%20Object%20Reference) (OtherComp :type Primitive%20Component%20Object%20Reference) (NormalImpulse :type Vector :default "0, 0, 0") (Hit :type Hit%20Result%20Structure%20%28by%20ref%29))
  (if (Variables|Default|GetCan%20Stop%20Launch)
    (bind _asbp_hero_primo (Utilities|Casting|CastToBP_Hero_Primo OtherActor))
    (if (and (Utilities|IsValid (.LaunchAimingManager (Utilities|Struct|BreakFAimingManager (Variables|/Game/BrawlStarsReplica/Hero/Base/Blueprint/BP_HeroBase.BP_HeroBase_C|GetAimingManager _asbp_hero_primo)))) (Variables|/Game/BrawlStarsReplica/Hero/Base/Blueprint/BP_Aiming_Launch.BP_Aiming_Launch_C|GetIs%20Hero%20Launch (.LaunchAimingManager (Utilities|Struct|BreakFAimingManager (Variables|/Game/BrawlStarsReplica/Hero/Base/Blueprint/BP_HeroBase.BP_HeroBase_C|GetAimingManager _asbp_hero_primo)))))
      (Default|ServerStopLaunch (.LaunchAimingManager (Utilities|Struct|BreakFAimingManager (Variables|/Game/BrawlStarsReplica/Hero/Base/Blueprint/BP_HeroBase.BP_HeroBase_C|GetAimingManager _asbp_hero_primo)))))))

(event OnComponentBeginOverlap(Collision)
  (params (OverlappedComponent :type Primitive%20Component%20Object%20Reference) (OtherActor :type Actor%20Object%20Reference) (OtherComp :type Primitive%20Component%20Object%20Reference) (OtherBodyIndex :type Integer) (bFromSweep :type Boolean) (SweepResult :type Hit%20Result%20Structure%20%28by%20ref%29))
  (if (Variables|Default|GetCan%20Stop%20Launch)
    (bind _asbp_bullet_nita_ultimate (Utilities|Casting|CastToBP_Bullet_Nita_Ultimate OtherActor))
    (bind _asbp_hero_nita (Utilities|Casting|CastToBP_Hero_Nita (Game|GetInstigator _asbp_bullet_nita_ultimate)))
    (Default|ServerStopLaunch (.LaunchAimingManager (Utilities|Struct|BreakFAimingManager (Variables|/Game/BrawlStarsReplica/Hero/Base/Blueprint/BP_HeroBase.BP_HeroBase_C|GetAimingManager _asbp_hero_nita))))))

(fn ConstructionScript)