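; Projectile Blueprint for Colt's ultimate bullet in a Brawl Stars replica, built as a child class that calls its parent's BeginPlay and construction script.
; The construction script sets the bullet mesh from a variable and applies the ultimate-specific material.
; It then scales the Cube, apparently the collision volume, and the visible bullet independently through separate world-scale variables.
; The file adds no runtime logic of its own.
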(event EventBeginPlay
  (|CallParentFunction))

(fn ConstructionScript
  (bind _bullet (Variables|Default|GetBullet))
  (|CallParentFunction)
  (Components|StaticMesh|SetStaticMesh _bullet (Variables|Default|GetStaticMeshType))
  (Rendering|Material|SetMaterial _bullet 0 "/Game/BrawlStarsReplica/Hero/Colt/Asset/Bullet/M_Colt_Bullet_Ultimate.M_Colt_Bullet_Ultimate")
  (Transformation|SetWorldScale3D (Variables|Default|GetCube) (Variables|Default|GetCollisionWorldScale))
  (Transformation|SetWorldScale3D (Variables|Default|GetBullet) (Variables|Default|GetBulletWorldScale)))