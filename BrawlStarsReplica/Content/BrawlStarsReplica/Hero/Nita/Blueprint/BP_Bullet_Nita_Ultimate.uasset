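; Nita's ultimate projectile in a Brawl Stars replica, which summons her bear at the point where its launch finishes.
; On BeginPlay it caches the instigating Nita's team and binds to her launch aiming manager's launch-end event.
; On that event the server replaces any existing bear with a new one, copies the team to its PlayerState, then destroys the projectile.
; Its Cube and Sphere overlap events are empty.
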(event OnComponentBeginOverlap(Cube)
  (params (OverlappedComponent :type Primitive%20Component%20Object%20Reference) (OtherActor :type Actor%20Object%20Reference) (OtherComp :type Primitive%20Component%20Object%20Reference) (OtherBodyIndex :type Integer) (bFromSweep :type Boolean) (SweepResult :type Hit%20Result%20Structure%20%28by%20ref%29)))

(event OnComponentBeginOverlap(Sphere)
  (params (OverlappedComponent :type Primitive%20Component%20Object%20Reference) (OtherActor :type Actor%20Object%20Reference) (OtherComp :type Primitive%20Component%20Object%20Reference) (OtherBodyIndex :type Integer) (bFromSweep :type Boolean) (SweepResult :type Hit%20Result%20Structure%20%28by%20ref%29)))

(event Custom|NitaFinishLaunch
  (Networking|SwitchHasAuthority
    (:Authority
      (bind _asbp_hero_nita (Utilities|Casting|CastToBP_Hero_Nita (Game|GetInstigator)))
      (bind _nitabear (Variables|/Game/BrawlStarsReplica/Hero/Nita/Blueprint/BP_Hero_Nita.BP_Hero_Nita_C|GetNitaBear _asbp_hero_nita)
        (:then
          (Actor|DestroyActor _nitabear))
        (:else
          _))
      (bind _returnvalue (Game|SpawnActorfromClass "/Game/BrawlStarsReplica/Hero/Nita/Blueprint/BP_Hero_NitaBear.BP_Hero_NitaBear_C" (Math|Transform|MakeTransform (Transformation|GetActorLocation) "0, 0, 0" "1,1,1") "AdjustIfPossibleButAlwaysSpawn" 0 _asbp_hero_nita))
      (bind _output_get (Variables|/Game/BrawlStarsReplica/Hero/Nita/Blueprint/BP_Hero_Nita.BP_Hero_Nita_C|SetNitaBear _asbp_hero_nita _returnvalue))
      (bind _asps_game_base (Utilities|Casting|CastToPS_GameBase (Variables|/Script/Engine.Pawn|GetPlayerState _output_get)))
      (Variables|/Game/BrawlStarsReplica/Map/Base/Blueprint/PS_GameBase.PS_GameBase_C|SetTeamType _asps_game_base (Variables|Default|GetTeamType))
      (Actor|DestroyActor))))

(event EventBeginPlay
  (|CallParentFunction)
  (bind _asbp_hero_nita (Utilities|Casting|CastToBP_Hero_Nita (Game|GetInstigator)))
  (Variables|Default|SetTeamType (Variables|/Game/BrawlStarsReplica/Hero/Base/Blueprint/BP_HeroBase.BP_HeroBase_C|GetTeamType _asbp_hero_nita))
  (EventDispatchers|BindEventtoLaunchEnd (.LaunchAimingManager (Utilities|Struct|BreakFAimingManager (Variables|/Game/BrawlStarsReplica/Hero/Base/Blueprint/BP_HeroBase.BP_HeroBase_C|GetAimingManager _asbp_hero_nita))) (delegate Custom|NitaFinishLaunch)))

(fn ConstructionScript
  (|CallParentFunction))