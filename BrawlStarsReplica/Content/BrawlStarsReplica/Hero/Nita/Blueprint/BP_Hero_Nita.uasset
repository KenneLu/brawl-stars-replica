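; Hero Blueprint for Nita in a Brawl Stars replica, implementing her ultimate skill launch.
; The launch stops any skill montage, turns the hero to the release direction, locks movement rotation and plays the ultimate montage.
; On the montage notify it spawns the ultimate bullet at the right-hand socket with her team, hands it to the AimingManager to launch, unlocks rotation and signals the skill finished.
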(event EventUltimateLaunchSkill
  (bind _mesh (Variables|Character|GetMesh))
  (bind _aimingmanager (Variables|Default|GetAimingManager))
  (bind _aimingmanager_2 (Variables|Default|GetAimingManager))
  (bind _heroskills (Variables|Default|GetHeroSkills))
  (bind _launchaimingmanager (Utilities|Struct|BreakFAimingManager _aimingmanager))
  (bind _launchaimingmanager_2 (Utilities|Struct|BreakFAimingManager _aimingmanager_2))
  (bind (_herotype _normalreleaseoffset _normalmontage _normalmontagesection _normalskilltype _ultimatereleaseoffset _ultimatemontage _ultimatemontagesection) (Utilities|Struct|BreakFSkillMontage _heroskills))
  (Default|SkillMontageStop _launchaimingmanager_2)
  (Default|SetHeroSkillReleaseRotation _launchaimingmanager_2 _ultimatereleaseoffset)
  (Default|LockMovementOrientRotation _launchaimingmanager_2)
  (Default|ClientPlayMontage _launchaimingmanager_2 _ultimatemontage 1.0 _ultimatemontagesection)
  (Animation|Montage|PlayMontage _mesh _ultimatemontage 1.0 0.0 _ultimatemontagesection
    (:OnNotifyBegin
      (bind _returnvalue (Game|SpawnActorfromClass "/Game/BrawlStarsReplica/Hero/Nita/Blueprint/BP_Bullet_Nita_Ultimate.BP_Bullet_Nita_Ultimate_C" (Math|Transform|MakeTransform (Transformation|GetSocketLocation _mesh "RightHand") "0, 0, 0" "1,1,1") "Undefined" self 0))
      (Variables|/Game/BrawlStarsReplica/Hero/Nita/Blueprint/BP_Bullet_Nita_Ultimate.BP_Bullet_Nita_Ultimate_C|SetTeamType _returnvalue (Variables|Default|GetTeamType))
      (Default|ReleaseLaunchSkill _launchaimingmanager false _returnvalue)
      (Default|UnlockMovementOrientRotation _launchaimingmanager)
      (Default|CallUltimateSkillFinished (Variables|Default|GetCP_SkillLock)))))

(event Collision|EventActorBeginOverlap
  (params (OtherActor :type Actor%20Object%20Reference)))

(event EventTick
  (params (DeltaSeconds :type Float%20%28single-precision%29)))

(event EventBeginPlay
  (|CallParentFunction) ; This node is disabled and will not be called.\nDrag off pins to build functionality.
)

(fn ConstructionScript
  (|CallParentFunction))