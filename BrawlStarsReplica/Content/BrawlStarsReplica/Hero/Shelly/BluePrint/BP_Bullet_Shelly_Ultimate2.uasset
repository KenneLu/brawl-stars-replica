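; Shelly's ultimate projectile in the Brawl Stars replica, a child bullet that knocks back the enemy it hits.
; On hit it recharges the ultimate, stops bot movement, launches a valid enemy along the Cube's forward vector with a velocity-change impulse, then deals damage and destroys itself.
; Without a valid enemy, it still applies damage for the SafeBox case.
; The construction script extends the parent's, applying configurable meshes, Niagara effects and scales to its multiple bullet components.
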(event EventHitEnemy
  (CallFunction|RechageUltimate)
  (bind _enemy (Variables|Default|GetEnemy)
    (:then
      (if (and (Pawn|IsBotControlled _enemy) (Utilities|IsValid (Pawn|GetController _enemy)))
        ;[1 1 1] AI Stop Movement
        (AI|Navigation|StopMovement (Pawn|GetController _enemy)))
      (Physics|AddImpulse (Variables|/Script/Engine.Character|GetCharacterMovement (Variables|Default|GetEnemy)) (* (Math|Vector|GetForwardVector (Variables|Default|GetCube)) 1e+03) true)
      (CallFunction|ApplyDamageandDestroy))
    (:else
      ;[1 1 1] Damage SafeBox
      (CallFunction|ApplyDamageandDestroy))))

(fn ConstructionScript
  (bind _bullet (Variables|Default|GetBullet))
  (bind _staticmeshtype (Variables|Default|GetStaticMeshType))
  (|CallParentFunction)
  (Class|NiagaraComponent|SetAsset (Variables|Default|GetNiagara) (Variables|Default|GetNiagaraType))
  (Transformation|SetWorldScale3D (Variables|Default|GetNiagara1) "1.000000,1.000000,1.000000")
  (Utilities|FlowControl|Sequence
    (:then_0
      (Components|StaticMesh|SetStaticMesh _bullet _staticmeshtype)
      (Transformation|SetWorldScale3D _bullet (Variables|Default|GetBulletWorldScale)))
    (:then_1
      (Components|StaticMesh|SetStaticMesh (Variables|Default|GetBullet1) _staticmeshtype))
    (:then_2
      (Components|StaticMesh|SetStaticMesh (Variables|Default|GetBullet2) _staticmeshtype))
    (:then_3
      (Components|StaticMesh|SetStaticMesh (Variables|Default|GetBullet3) _staticmeshtype))))