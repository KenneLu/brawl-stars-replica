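; Projectile for Shelly's ultimate in a Brawl Stars replica, a child bullet Blueprint that knocks enemies back along its forward direction.
; On cube overlap, a team check gates a strong impulse on the Enemy's character movement.
; The HitEnemy event recharges the ultimate, then applies the same impulse as a mass-independent velocity change before dealing damage and destroying itself.
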(event OnComponentBeginOverlap(Cube)
  (params (OverlappedComponent :type Primitive%20Component%20Object%20Reference) (OtherActor :type Actor%20Object%20Reference) (OtherComp :type Primitive%20Component%20Object%20Reference) (OtherBodyIndex :type Integer) (bFromSweep :type Boolean) (SweepResult :type Hit%20Result%20Structure%20%28by%20ref%29))
  (bind _returnvalue (CallFunction|CheckTeamate OtherActor))
  (if _returnvalue
    (bind _enemy (Variables|Default|GetEnemy)
      (:then
        (Physics|AddImpulse (Variables|/Script/Engine.Character|GetCharacterMovement _enemy) (* (Math|Vector|GetForwardVector (Variables|Default|GetCube)) 1e+05) false))
      (:else))))

(event EventHitEnemy
  (CallFunction|RechageUltimate)
  (bind _enemy (Variables|Default|GetEnemy)
    (:then
      (Physics|AddImpulse (Variables|/Script/Engine.Character|GetCharacterMovement _enemy) (* (Math|Vector|GetForwardVector (Variables|Default|GetCube)) 1e+05) true)
      (CallFunction|ApplyDamageandDestroy))
    (:else)))

(fn ConstructionScript
  (|CallParentFunction))