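; Ultimate-attack bullet for hero Primo in a Brawl Stars replica, built on a parent bullet class with its destructible-sensing flag enabled.
; Construction disables Cube collision and leaves Sphere query-only.
; On an enemy hit, it restores a third of the owning Primo's default ultimate energy.
; A valid enemy is then launched away from the Cube and along its up vector before bullet damage applies.
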(event EventBeginPlay
  (|CallParentFunction)
  (Variables|Default|SetSenceDestructibal true))

(event EventHitEnemy
  (bind _cube (Variables|Default|GetCube))
  (bind _enemy (Variables|Default|GetEnemy))
  (bind _asbp_hero_primo (Utilities|Casting|CastToBP_Hero_Primo (Components|GetOwner)))
  (Variables|/Game/BrawlStarsReplica/Hero/Base/Blueprint/CP_SkillLock.CP_SkillLock_C|SetUltimateEnergyCurrent (Variables|/Game/BrawlStarsReplica/Hero/Base/Blueprint/BP_HeroBase.BP_HeroBase_C|GetCP_SkillLock _asbp_hero_primo) (+ (Variables|/Game/BrawlStarsReplica/Hero/Base/Blueprint/CP_SkillLock.CP_SkillLock_C|GetUltimateEnergyCurrent (Variables|/Game/BrawlStarsReplica/Hero/Base/Blueprint/BP_HeroBase.BP_HeroBase_C|GetCP_SkillLock _asbp_hero_primo)) (/ (Variables|/Game/BrawlStarsReplica/Hero/Base/Blueprint/CP_SkillLock.CP_SkillLock_C|GetUltimateEnergyDefault (Variables|/Game/BrawlStarsReplica/Hero/Base/Blueprint/BP_HeroBase.BP_HeroBase_C|GetCP_SkillLock _asbp_hero_primo)) 3.0)))
  (Utilities|IsValid _enemy
    (:Is%20Valid
      (Physics|AddImpulse (Variables|/Script/Engine.Character|GetCharacterMovement _enemy) (* (+ (Math|Vector|Normalize (- (Transformation|GetActorLocation _enemy) (Transformation|GetWorldLocation _cube))) (Math|Vector|Normalize (Math|Vector|GetUpVector _cube))) 5e+04) false)
      (CallFunction|ApplyBulletDamage))))

(fn ConstructionScript
  (|CallParentFunction)
  (Collision|SetCollisionEnabled (Variables|Default|GetCube) "NoCollision")
  (Collision|SetCollisionEnabled (Variables|Default|GetSphere) "QueryOnly"))