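; Primo hero Blueprint for the Brawl Stars replica, implementing his launch-style ultimate skill.
; UltimateLaunchSkill stops the skill montage, sets release rotation, locks movement orientation and launches the hero through the LaunchAimingManager.
; The capsule ignores collision during launch, except for overlaps on GameTraceChannel3.
; A bound launch-end callback releases the flat ultimate skill, unlocks orientation, signals completion and restores blocking on selected channels.
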(event Custom|PrimoFinishLaunch
  (bind _aimingmanager (Variables|Default|GetAimingManager))
  (bind _capsulecomponent (Variables|Default|GetCapsuleComponent))
  (bind _launchaimingmanager (Utilities|Struct|BreakFAimingManager _aimingmanager))
  ;[1 1 1] Primo Ultimate Skill
  (Default|ReleaseFlatSkill _launchaimingmanager (.UltimateSkillType (Utilities|Struct|BreakFSkillMontage (Variables|Default|GetHeroSkills))))
  (Default|UnlockMovementOrientRotation _launchaimingmanager)
  (Default|CallUltimateSkillFinished (Variables|Default|GetCP_SkillLock))
  (Collision|SetCollisionResponsetoChannel _capsulecomponent "ECC_WorldStatic" "ECR_Block")
  (Collision|SetCollisionResponsetoChannel _capsulecomponent "ECC_Pawn" "ECR_Block")
  (Collision|SetCollisionResponsetoChannel _capsulecomponent "ECC_GameTraceChannel1" "ECR_Block")
  (Collision|SetCollisionResponsetoChannel _capsulecomponent "ECC_GameTraceChannel3" "ECR_Block"))

(event EventUltimateLaunchSkill
  (bind _capsulecomponent (Variables|Default|GetCapsuleComponent))
  (bind _aimingmanager (Variables|Default|GetAimingManager))
  (bind _launchaimingmanager (Utilities|Struct|BreakFAimingManager _aimingmanager))
  ;[1 1 1] Primo Ultimate Skill
  (Default|SkillMontageStop _launchaimingmanager)
  (Default|SetHeroSkillReleaseRotation _launchaimingmanager (.UltimateReleaseOffset (Utilities|Struct|BreakFSkillMontage (Variables|Default|GetHeroSkills))))
  (Default|LockMovementOrientRotation _launchaimingmanager)
  (Default|ReleaseLaunchSkill _launchaimingmanager true)
  (Collision|SetCollisionResponsetoAllChannels _capsulecomponent "ECR_Ignore")
  (Collision|SetCollisionResponsetoChannel _capsulecomponent "ECC_GameTraceChannel3" "ECR_Overlap")
  (EventDispatchers|BindEventtoLaunchEnd (.LaunchAimingManager (Utilities|Struct|BreakFAimingManager (Variables|Default|GetAimingManager))) (delegate Custom|PrimoFinishLaunch)))

(fn ConstructionScript
  (|CallParentFunction))