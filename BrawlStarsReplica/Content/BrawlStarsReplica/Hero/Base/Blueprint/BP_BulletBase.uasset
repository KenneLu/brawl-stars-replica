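; Base projectile actor for hero bullets in a Brawl Stars replica.
; Construction script pulls stats and sound from DataTables by matching rows to its class, and disables Sphere collision.
; Overlaps damage opposing heroes or safe boxes and destroy the bullet, with hero hits also recharging the shooter's ultimate.
; Destructible scenery is ruined or shaken depending on bullet data, and only long-lived bullets survive that contact.
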(event OnComponentBeginOverlap(Cube)
  (params (OverlappedComponent :type Primitive%20Component%20Object%20Reference) (OtherActor :type Actor%20Object%20Reference) (OtherComp :type Primitive%20Component%20Object%20Reference) (OtherBodyIndex :type Integer) (bFromSweep :type Boolean) (SweepResult :type Hit%20Result%20Structure%20%28by%20ref%29))
  (bind _returnvalue (CallFunction|CheckTeamate OtherActor))
  (if _returnvalue
    (CallFunction|HitEnemy)))

(event OnComponentBeginOverlap(Sphere)
  (params (OverlappedComponent :type Primitive%20Component%20Object%20Reference) (OtherActor :type Actor%20Object%20Reference) (OtherComp :type Primitive%20Component%20Object%20Reference) (OtherBodyIndex :type Integer) (bFromSweep :type Boolean) (SweepResult :type Hit%20Result%20Structure%20%28by%20ref%29))
  (bind _returnvalue (CallFunction|CheckTeamate OtherActor))
  (if _returnvalue
    (CallFunction|HitEnemy)))

(event Custom|HitEnemy
  (CallFunction|RechageUltimate)
  (CallFunction|ApplyDamageandDestroy))

(event EventBeginPlay
  (bind _bulletsoundeffect (Variables|Default|GetBulletSoundEffect)
    (:then
      (Audio|PlaySoundatLocation _bulletsoundeffect (Transformation|GetActorLocation) "0, 0, 0" (Variables|Default|GetBulletSoundVolume) 1.0 0.0 "/Game/BrawlStarsReplica/Sound/Blueprint/SA_Bullet.SA_Bullet" 0 0))
    (:else)))

(fn ConstructionScript
  (bind _projectilemovement (Variables|Default|GetProjectileMovement))
  (Collision|SetCollisionEnabled (Variables|Default|GetSphere) "NoCollision")
  (Utilities|FlowControl|Sequence
    (:then_0
      (bind _outrownames (DataTable|GetDataTableRowNames "/Game/BrawlStarsReplica/Hero/Base/Data/DT_Skill.DT_Skill"))
      (for _array_element _outrownames
        (bind _returnvalue (Utilities|GetDataTableRow "/Game/BrawlStarsReplica/Hero/Base/Data/DT_Skill.DT_Skill" _array_element)
          (:then
            (if (== (.BulletType (Utilities|Struct|BreakFSkillAttribute _returnvalue)) (Utilities|GetClass self))
              (Variables|Default|SetDamage (.BulletDamage (Utilities|Struct|BreakFSkillAttribute _returnvalue)))
              (Variables|/Script/Engine.ProjectileMovementComponent|SetInitialSpeed _projectilemovement (.BulletMoveSpeed (Utilities|Struct|BreakFSkillAttribute _returnvalue)))
              (Variables|/Script/Engine.ProjectileMovementComponent|SetMaxSpeed _projectilemovement (.BulletMoveSpeed (Utilities|Struct|BreakFSkillAttribute _returnvalue)))
              (Actor|SetLifeSpan (.BulletLifeSpan (Utilities|Struct|BreakFSkillAttribute _returnvalue)))
              (Variables|Default|SetSenceDestructibal (.BulletSenceDestructible (Utilities|Struct|BreakFSkillAttribute _returnvalue)))
              (Variables|Default|SetisLongLive (.BulletIsLongLive (Utilities|Struct|BreakFSkillAttribute _returnvalue))))))))
    (:then_1
      (bind _outrownames_2 (DataTable|GetDataTableRowNames "/Game/BrawlStarsReplica/Hero/Base/Data/DT_BulletSoundEffect.DT_BulletSoundEffect"))
      (for _array_element_2 _outrownames_2
        (bind _returnvalue_2 (Utilities|GetDataTableRow "/Game/BrawlStarsReplica/Hero/Base/Data/DT_BulletSoundEffect.DT_BulletSoundEffect" _array_element_2)
          (:then
            (if (== (.BulletType (Utilities|Struct|BreakFBulletSoundEffect _returnvalue_2)) (Utilities|GetClass self))
              (Variables|Default|SetBulletSoundEffect (.BulletSoundEffct (Utilities|Struct|BreakFBulletSoundEffect _returnvalue_2)))
              (Variables|Default|SetBulletSoundVolume (.BulletSoundVolume (Utilities|Struct|BreakFBulletSoundEffect _returnvalue_2))))))))))

(fn CheckTeamate
  (params (OtherActor :type Object%20Object%20Reference))
  (Variables|Default|SetEnemy 0)
  (Variables|Default|SetHitActor 0)
  (bind _asbp_hero_base (Utilities|Casting|CastToBP_HeroBase (Game|GetInstigator)))
  (Variables|Default|SetHeroSelf _asbp_hero_base)
  (bind _asbp_hero_base_2 (Utilities|Casting|CastToBP_HeroBase OtherActor)
    (:then
      (bind _output_get (Variables|Default|SetEnemy _asbp_hero_base_2))
      (Variables|Default|SetHitActor _output_get)
      (bind _enemy (Variables|Default|GetEnemy)
        (:then
          (bind _heroself (Variables|Default|GetHeroSelf)
            (:then
              (if (Utilities|Enum|NotEqual(Enum) (Variables|/Game/BrawlStarsReplica/Hero/Base/Blueprint/BP_HeroBase.BP_HeroBase_C|GetTeamType _heroself) (Variables|/Game/BrawlStarsReplica/Hero/Base/Blueprint/BP_HeroBase.BP_HeroBase_C|GetTeamType _enemy))
                (if (!= (Variables|Default|GetHitActor) (Variables|Default|GetHeroSelf))
                  (return true))))
            (:else)))
        (:else)))
    (:CastFailed
      (bind _asbp_safe_box (Utilities|Casting|CastToBP_SafeBox OtherActor)
        (:then
          (Variables|Default|SetHitActor _asbp_safe_box)
          (bind _heroself_2 (Variables|Default|GetHeroSelf)
            (:then
              (if (Utilities|Enum|NotEqual(Enum) (Variables|/Game/BrawlStarsReplica/Hero/Base/Blueprint/BP_HeroBase.BP_HeroBase_C|GetTeamType _heroself_2) (Variables|/Game/BrawlStarsReplica/Map/Game/Heist/BP_SafeBox.BP_SafeBox_C|GetSafeBoxTeamType _asbp_safe_box))
                (if (!= (Variables|Default|GetHitActor) (Variables|Default|GetHeroSelf))
                  (return true))))
            (:else)))
        (:CastFailed
          (bind _asbp_sence_base (Utilities|Casting|CastToBP_SenceBase OtherActor))
          (bind _asbp_sence_destructible (Utilities|Casting|CastToBP_Sence_Destructible _asbp_sence_base))
          (if (Variables|Default|GetSenceDestructibal)
            (Default|Ruined _asbp_sence_destructible)
            (else
              (Default|Shake _asbp_sence_destructible (Transformation|GetActorForwardVector) (Transformation|GetWorldLocation (Variables|Default|GetBulletHead)))))
          (if (not (Variables|Default|GetisLongLive))
            (Actor|DestroyActor)))))))

(fn ApplyDamageandDestroy
  (Game|Damage|ApplyDamage (Variables|Default|GetHitActor) (Variables|Default|GetDamage) 0 (Variables|Default|GetHeroSelf))
  (Actor|DestroyActor))

(fn RechageUltimate
  (bind _returnvalue (Game|GetInstigator))
  (Variables|Default|GetEnemy
    (:then
      (Utilities|IsValid _returnvalue
        (:Is%20Valid
          (bind _asbp_hero_base (Utilities|Casting|CastToBP_HeroBase _returnvalue))
          (Default|CallUltimateRechage (Variables|/Game/BrawlStarsReplica/Hero/Base/Blueprint/BP_HeroBase.BP_HeroBase_C|GetCP_SkillLock _asbp_hero_base)))))
    (:else)))

(fn ApplyBulletDamage
  (Game|Damage|ApplyDamage (Variables|Default|GetHitActor) (Variables|Default|GetDamage) 0 (Variables|Default|GetHeroSelf)))