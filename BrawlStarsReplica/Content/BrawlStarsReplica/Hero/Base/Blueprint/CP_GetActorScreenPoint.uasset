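; Actor component for heroes in a Brawl Stars replica that finds the owning actor's position on screen.
; GetActorScreenPoint projects the owner's location through player controller 0 and warps the mouse cursor to that pixel.
; It then reads back the viewport mouse position, returning both points when that position is positive on both axes, or zeros with Done false otherwise.
; The event graph holds only disabled stubs.
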(event EventBeginPlay)

(event EventTick
  (params (DeltaSeconds :type Float%20%28single-precision%29)))

(fn GetActorScreenPoint
  (bind _returnvalue (Components|GetOwner))
  (bind _returnvalue_2 (Game|GetPlayerController 0))
  (bind _returnvalue_3 (Transformation|GetActorLocation _returnvalue))
  (bind _screenlocation (Class|PlayerController|ProjectWorldLocationtoScreen _returnvalue_2 _returnvalue_3 false))
  (bind (_x _y) (Math|Vector2D|BreakVector2D _screenlocation))
  (Class|PlayerController|SetMouseLocation (Game|GetPlayerController 0) (Math|Float|Truncate _x) (Math|Float|Truncate _y))
  (bind _returnvalue_4 (Class|WidgetLayoutLibrary|GetMousePositiononViewport))
  (if (and (> (.X (Math|Vector2D|BreakVector2D _returnvalue_4)) 0.0) (> (.Y (Math|Vector2D|BreakVector2D _returnvalue_4)) 0.0))
    (return _screenlocation _returnvalue_4 true)
    (else
      (return "" "" false))))