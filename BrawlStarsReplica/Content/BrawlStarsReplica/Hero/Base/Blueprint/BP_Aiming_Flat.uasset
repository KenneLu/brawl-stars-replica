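; BP_Aiming_Flat handles a hero's flat skill aiming, showing a ground decal and providing skill-release helpers for rotation, montages and projectile spawning.
; Construction reads normal and ultimate angle and range from DT_Skill, which drive rectangle or sector decals through MPC_Aim_Decal.
; While aiming, mouse offset from the hero's screen point sets distance and smoothed yaw, flipped for one team.
; Remote clients send this aim to SetServerAimingInfo, and bots skip mouse aiming.
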(event Custom|FlatAimingManager
  (bind _aimingdecal (Variables|Default|GetAimingDecal))
  (bind _aiminginfo (Variables|Default|GetAimingInfo))
  (bind (_isflataiming _islaunchaming _isviewportcentrepointset _viewportcentrepoint _realviewportcentermousepoint _aimdistance) (Utilities|Struct|BreakFAimInfo _aiminginfo))
  ;[1 1 1] FlatAimingManager
  (if (Pawn|IsLocallyControlled (Variables|Default|GetHero))
    (if _isflataiming
      (Utilities|FlowControl|Sequence
        (:then_0
          (CallFunction|UpdateDecalShap)
          (CallFunction|UpdateAimDistanceandRotation)
          (bind _returnvalue (CallFunction|NotAIControlled))
          (if (and _returnvalue (> (Math|Float|Absolute(Float) _aimdistance) 1.0))
            (Rendering|SetVisibility _aimingdecal true false)
            (Transformation|SetWorldRotation _aimingdecal (Math|Rotator|MakeRotator 1.8e+02 9e+01 (.AimRotationZ (Utilities|Struct|BreakFAimInfo (Variables|Default|GetAimingInfo)))) false false)))
        (:then_1
          (goto _label Reset)))
      (else
        (Utilities|FlowControl|DoOnce false :!label _label
          (:Completed
            (Utilities|Struct|SetmembersinFAimInfo (Variables|Default|GetAimingInfo) 0.0)
            (Rendering|SetVisibility (Variables|Default|GetAimingDecal) false false)))))))

(event Custom|InitAimingScreenPoint
  (bind _hero (Variables|Default|GetHero))
  ;[1 1 1] Init Aiming Screen Point
  ;;[1 1 1] Wait Controller Possess
  (Utilities|FlowControl|Delay 0.2)
  (if (and (not (Pawn|IsBotControlled _hero)) (Pawn|IsLocallyControlled _hero))
    (if (not (.isViewportCentrePointSet (Utilities|Struct|BreakFAimInfo (Variables|Default|GetAimingInfo)))) :!label _label
      (CallFunction|InitActorScreenPoint)
      ;;[1 1 1] Wait Verport Init Done
      (Utilities|FlowControl|Delay 0.2)
      (goto _label))))

(event Custom|SetHeroSkillReleaseRotation
  (params (AddModify :type Float%20%28single-precision%29))
  ;[1 1 1] Release Skill Manager
  (bind _hero (Variables|Default|GetHero)
    (:then
      (Transformation|SetActorRotation _hero (Math|Rotator|MakeRotator 0.0 0.0 (+ AddModify (.AimRotationZ (Utilities|Struct|BreakFAimInfo (Variables|Default|GetAimingInfo)))))))
    (:else)))

(event Custom|ClientPlayMontage
  (params (AnimMontage :type Anim%20Montage%20Object%20Reference) (InPlayRate :type Float%20%28single-precision%29) (StartSectionName :type Name))
  ;[1 1 1] Release Skill Manager
  (bind _hero (Variables|Default|GetHero)
    (:then
      (Animation|PlayAnimMontage _hero AnimMontage InPlayRate StartSectionName))
    (:else)))

(event Custom|SkillMontageStop
  ;[1 1 1] Release Skill Manager
  (bind _hero (Variables|Default|GetHero)
    (:then
      (Animation|Montage|MontageStop (Components|SkeletalMesh|GetAnimInstance (Variables|/Script/Engine.Character|GetMesh _hero)) 0.0 0))
    (:else)))

(event Custom|ReleaseFlatSkill
  (params (SkillType :type BP%20Skill%20Base%20Class%20Reference))
  ;[1 1 1] Release Skill Manager
  (bind _hero (Variables|Default|GetHero)
    (:then
      (bind _weapon (Variables|/Game/BrawlStarsReplica/Hero/Base/Blueprint/BP_HeroBase.BP_HeroBase_C|GetWeapon _hero)
        (:then
          (Game|SpawnActorfromClass SkillType (Math|Transform|MakeTransform (Transformation|GetSocketLocation (Variables|/Script/Engine.Actor|GetRootComponent _weapon) "Muzzle") (Math|Conversions|RotationFromXVector (Math|Vector|GetForwardVector (Variables|/Script/Engine.Character|GetCapsuleComponent _hero))) "1,1,1") "AlwaysSpawn" 0 (Variables|Default|GetHero)))
        (:else)))
    (:else)))

(event Custom|UnlockMovementOrientRotation
  ;[1 1 1] Release Skill Manager
  (bind _hero (Variables|Default|GetHero)
    (:then
      (Variables|/Script/Engine.CharacterMovementComponent|SetbOrientRotationToMovement (Variables|/Script/Engine.Character|GetCharacterMovement _hero) true))
    (:else)))

(event Custom|SetServerAimingInfo
  (params (AimingInfo :type F%20Aim%20Info%20Structure%20%28by%20ref%29))
  ;[1 1 1] FlatAimingManager
  (Variables|Default|SetAimingInfo AimingInfo))

(event Custom|LockMovementOrientRotation
  ;[1 1 1] Release Skill Manager
  (bind _hero (Variables|Default|GetHero)
    (:then
      (Variables|/Script/Engine.CharacterMovementComponent|SetbOrientRotationToMovement (Variables|/Script/Engine.Character|GetCharacterMovement _hero) false))
    (:else)))

(event EventBeginPlay
  (Utilities|Casting|CastToPC_GameBase (Game|GetPlayerController 0))
  (bind _asbp_hero_base (Utilities|Casting|CastToBP_HeroBase (Components|GetOwner)))
  (Variables|Default|SetHero _asbp_hero_base)
  (CallFunction|InitAimingScreenPoint))

(event EventTick
  (params (DeltaSeconds :type Float%20%28single-precision%29))
  (Variables|Default|GetHero
    (:then
      (CallFunction|FlatAimingManager))
    (:else)))

(fn ConstructionScript
  (bind _aimingdecal (Variables|Default|GetAimingDecal))
  (bind _outrownames (DataTable|GetDataTableRowNames "/Game/BrawlStarsReplica/Hero/Base/Data/DT_Skill.DT_Skill"))
  (for _array_element _outrownames
    (bind _returnvalue (Utilities|GetDataTableRow "/Game/BrawlStarsReplica/Hero/Base/Data/DT_Skill.DT_Skill" _array_element)
      (:then
        (if (== (.HeroType (Utilities|Struct|BreakFSkillAttribute _returnvalue)) (Utilities|GetClass (Components|GetOwner)))
          (if (Utilities|Enum|Equal(Enum) (.SkillClassification (Utilities|Struct|BreakFSkillAttribute _returnvalue)) "NewEnumerator0")
            (Variables|Default|SetDecalAngelNormal (.SkillRleaseAngle (Utilities|Struct|BreakFSkillAttribute _returnvalue)))
            (Variables|Default|SetDecalDistanceNormal (* (.BulletMoveSpeed (Utilities|Struct|BreakFSkillAttribute _returnvalue)) (.BulletLifeSpan (Utilities|Struct|BreakFSkillAttribute _returnvalue))))
            (else
              (Variables|Default|SetDecalAngelUltimate (.SkillRleaseAngle (Utilities|Struct|BreakFSkillAttribute _returnvalue)))
              (Variables|Default|SetDecalDistanceUltimate (* (.BulletMoveSpeed (Utilities|Struct|BreakFSkillAttribute _returnvalue)) (.BulletLifeSpan (Utilities|Struct|BreakFSkillAttribute _returnvalue))))))))))
  (Rendering|Components|Decal|SetDecalMaterial _aimingdecal "/Game/BrawlStarsReplica/Hero/Base/Asset/M_Decal_FlatAim_Rectangle.M_Decal_FlatAim_Rectangle")
  (Transformation|SetWorldRotation _aimingdecal "90.000000,35.264389,-144.735718" false false)
  (Transformation|SetWorldScale3D _aimingdecal "1.000000,4.000000,4.000000")
  (Rendering|SetVisibility _aimingdecal false false))

(fn UpdateAimDistanceandRotation
  (bind _aiminginfo (Variables|Default|GetAimingInfo))
  (bind _realviewportcentermousepoint (Utilities|Struct|BreakFAimInfo _aiminginfo))
  (bind _returnvalue (CallFunction|NotAIControlled))
  (if _returnvalue
    (bind _returnvalue_2 (Class|WidgetLayoutLibrary|GetMousePositiononViewport))
    (if (Math|Vector|NotEqual(Vector) _realviewportcentermousepoint _returnvalue_2 0.0001)
      (Utilities|FlowControl|Sequence
        (:then_0
          (LocalVariables|SetNewAimDistance (Math|Vector2D|Vector2DLength (- _realviewportcentermousepoint _returnvalue_2))))
        (:then_1
          (bind _output_get (LocalVariables|SetNewAimRotationZ (Class|KismetMathLibrary|DegAtan2 (* (.X (Math|Vector2D|BreakVector2D (- _realviewportcentermousepoint _returnvalue_2))) -1.0) (.Y (Math|Vector2D|BreakVector2D (- _realviewportcentermousepoint _returnvalue_2))))))
          (bind _aspc_game_base (Utilities|Casting|CastToPC_GameBase (Game|GetPlayerController 0))
            (:then
              (if (Utilities|Enum|Equal(Enum) (Variables|/Game/BrawlStarsReplica/Map/Base/Blueprint/PC_GameBase.PC_GameBase_C|GetTeamType _aspc_game_base) "NewEnumerator1")
                (LocalVariables|SetNewAimRotationZ (+ _output_get 1.8e+02))))
            (:CastFailed
              _))
          (LocalVariables|SetAimRotationZ (.AimRotationZ (Utilities|Struct|BreakFAimInfo (Variables|Default|GetAimingInfo))))
          (if (< (Math|Float|Absolute(Float) (- (LocalVariables|GetAimRotationZ) (LocalVariables|GetNewAimRotationZ))) 1e+02)
            (LocalVariables|SetNewAimRotationZ (Math|Interpolation|FInterpTo (LocalVariables|GetAimRotationZ) (LocalVariables|GetNewAimRotationZ) (Utilities|Time|GetWorldDeltaSeconds) 4e+01))))
        (:then_2
          (Utilities|Struct|SetmembersinFAimInfo (Variables|Default|GetAimingInfo) (LocalVariables|GetNewAimDistance) (LocalVariables|GetNewAimRotationZ))
          (Networking|SwitchHasAuthority
            (:Remote
              (CallFunction|SetServerAimingInfo (Variables|Default|GetAimingInfo)))))))))

(fn InitActorScreenPoint
  (bind (_getactorscreenpoint _getactorscreenmousepoint _done) (Default|GetActorScreenPoint (Variables|Default|GetCP_GetViewportCenter)))
  (if _done
    (Utilities|Struct|SetmembersinFAimInfo (Variables|Default|GetAimingInfo) true _getactorscreenpoint _getactorscreenmousepoint)))

(fn CenterMousePosition
  (bind _aiminginfo (Variables|Default|GetAimingInfo))
  (bind _viewportcentrepoint (Utilities|Struct|BreakFAimInfo _aiminginfo))
  (bind (_x _y) (Math|Vector2D|BreakVector2D _viewportcentrepoint))
  (bind _returnvalue (CallFunction|NotAIControlled))
  (if _returnvalue
    (Class|PlayerController|SetMouseLocation (Game|GetPlayerController 0) (Math|Float|Truncate _x) (Math|Float|Truncate _y))))

(fn NotAIControlled
  (bind _returnvalue (Components|GetOwner))
  (Utilities|IsValid _returnvalue
    (:Is%20Valid
      (bind _instigator (Variables|/Script/Engine.Actor|GetInstigator _returnvalue)
        (:then
          (return (not (Pawn|IsBotControlled _instigator))))
        (:else)))))

(fn UpdateDecalShap
  (if (.isNormalActivated (Utilities|Struct|BreakFSkillState (Variables|/Game/BrawlStarsReplica/Hero/Base/Blueprint/CP_SkillLock.CP_SkillLock_C|GetSkillState (Variables|/Game/BrawlStarsReplica/Hero/Base/Blueprint/BP_HeroBase.BP_HeroBase_C|GetCP_SkillLock (Variables|Default|GetHero)))))
    (LocalVariables|SetAngle (/ (Variables|Default|GetDecalAngelNormal) 3.6e+02))
    (LocalVariables|SetDistance (Variables|Default|GetDecalDistanceNormal))
    (else
      (LocalVariables|SetAngle (/ (Variables|Default|GetDecalAngelUltimate) 3.6e+02))
      (LocalVariables|SetDistance (Variables|Default|GetDecalDistanceUltimate))))
  (if (== 0.0 (Variables|Default|GetDecalAngelNormal))
    ;[1 1 1] Rectangle Aiming Decal
    (Rendering|Components|Decal|SetDecalMaterial (Variables|Default|GetAimingDecal) "/Game/BrawlStarsReplica/Hero/Base/Asset/M_Decal_FlatAim_Rectangle.M_Decal_FlatAim_Rectangle")
    (Rendering|Material|SetScalarParameterValue "/Game/BrawlStarsReplica/Hero/Base/Asset/MPC_Aim_Decal.MPC_Aim_Decal" "Angle" 0.0 :!class /Script/Engine.KismetMaterialLibrary)
    (Rendering|Material|SetScalarParameterValue "/Game/BrawlStarsReplica/Hero/Base/Asset/MPC_Aim_Decal.MPC_Aim_Decal" "Distance" (- (- 1.0 (/ (LocalVariables|GetDistance) 1.4e+03)) 0.3) :!class /Script/Engine.KismetMaterialLibrary)
    (else
      ;[1 1 1] Sector Aiming Decal
      (Rendering|Components|Decal|SetDecalMaterial (Variables|Default|GetAimingDecal) "/Game/BrawlStarsReplica/Hero/Base/Asset/M_Decal_FlatAim_Sector.M_Decal_FlatAim_Sector")
      (Rendering|Material|SetScalarParameterValue "/Game/BrawlStarsReplica/Hero/Base/Asset/MPC_Aim_Decal.MPC_Aim_Decal" "Angle" (LocalVariables|GetAngle) :!class /Script/Engine.KismetMaterialLibrary)
      (Rendering|Material|SetScalarParameterValue "/Game/BrawlStarsReplica/Hero/Base/Asset/MPC_Aim_Decal.MPC_Aim_Decal" "Distance" (+ (/ (LocalVariables|GetDistance) 1.5e+03) 0.3) :!class /Script/Engine.KismetMaterialLibrary))))