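; Base hero Blueprint for the Brawl Stars replica, for heroes whose normal and ultimate skills both use flat aiming.
; On BeginPlay it equips the flat aiming manager; activating either skill enables flat aiming and centers the mouse.
; Releasing ends aiming, sets release rotation, locks movement orientation and plays the skill's montage.
; A montage notify fires the flat skill; completion unlocks rotation and reports the skill finished to the skill lock component.
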(event Custom|ReleaseSkill
  (params (ReleaseRotationOffset :type Float%20%28single-precision%29) (NormalSkill :type Boolean) (Montage :type Anim%20Montage%20Object%20Reference) (MontageSection :type Name) (SkillType :type BP%20Skill%20Base%20Class%20Reference))
  (bind _aimingmanager (Variables|Default|GetAimingManager))
  (bind _aimingmanager_2 (Variables|Default|GetAimingManager))
  (bind _flataimingmanager (Utilities|Struct|BreakFAimingManager _aimingmanager_2))
  (bind _flataimingmanager_2 (Utilities|Struct|BreakFAimingManager _aimingmanager))
  ;[1 1 1] Skill Manager
  (Default|SkillMontageStop _flataimingmanager_2)
  (Default|SetHeroSkillReleaseRotation _flataimingmanager_2 ReleaseRotationOffset)
  (Default|LockMovementOrientRotation _flataimingmanager_2)
  (Default|ClientPlayMontage _flataimingmanager_2 Montage 1.0 MontageSection)
  (Animation|Montage|PlayMontage (Variables|Character|GetMesh) Montage 1.0 0.0 MontageSection
    (:OnCompleted
      (Default|UnlockMovementOrientRotation _flataimingmanager)
      (if NormalSkill
        (Default|CallNormalSkillFinished (Variables|Default|GetCP_SkillLock))
        (else
          (Default|CallUltimateSkillFinished (Variables|Default|GetCP_SkillLock)))))
    (:OnNotifyBegin
      (Default|ReleaseFlatSkill _flataimingmanager SkillType))))

(event EventBeginPlay
  ;[1 1 1] Init Aiming Manager
  (|CallParentFunction)
  (CallFunction|EquipFlatAimingManager))

(event EventReleaseUltimateSkill
  (bind _heroskills (Variables|Default|GetHeroSkills))
  (bind (_herotype _normalreleaseoffset _normalmontage _normalmontagesection _normalskilltype _ultimatereleaseoffset _ultimatemontage _ultimatemontagesection _ultimateskilltype) (Utilities|Struct|BreakFSkillMontage _heroskills))
  ;[1 1 1] Skill Manager
  (|CallParentFunction)
  (Utilities|Struct|SetmembersinFAimInfo (Variables|/Game/BrawlStarsReplica/Hero/Base/Blueprint/BP_Aiming_Flat.BP_Aiming_Flat_C|GetAimingInfo (.FlatAimingManager (Utilities|Struct|BreakFAimingManager (Variables|Default|GetAimingManager)))) false)
  (CallFunction|ReleaseSkill _ultimatereleaseoffset false _ultimatemontage _ultimatemontagesection _ultimateskilltype))

(event EventActivateNormalSkill
  (bind _aimingmanager (Variables|Default|GetAimingManager))
  (bind _flataimingmanager (Utilities|Struct|BreakFAimingManager _aimingmanager))
  ;[1 1 1] Skill Manager
  (|CallParentFunction)
  (Utilities|Struct|SetmembersinFAimInfo (Variables|/Game/BrawlStarsReplica/Hero/Base/Blueprint/BP_Aiming_Flat.BP_Aiming_Flat_C|GetAimingInfo _flataimingmanager) true)
  (Default|CenterMousePosition _flataimingmanager))

(event EventReleaseNormalSkill
  (bind _heroskills (Variables|Default|GetHeroSkills))
  (bind (_herotype _normalreleaseoffset _normalmontage _normalmontagesection _normalskilltype _ultimatereleaseoffset _ultimatemontage _ultimatemontagesection _ultimateskilltype) (Utilities|Struct|BreakFSkillMontage _heroskills))
  ;[1 1 1] Skill Manager
  (|CallParentFunction)
  (Utilities|Struct|SetmembersinFAimInfo (Variables|/Game/BrawlStarsReplica/Hero/Base/Blueprint/BP_Aiming_Flat.BP_Aiming_Flat_C|GetAimingInfo (.FlatAimingManager (Utilities|Struct|BreakFAimingManager (Variables|Default|GetAimingManager)))) false)
  (CallFunction|ReleaseSkill _normalreleaseoffset true _normalmontage _normalmontagesection _normalskilltype))

(event EventActivateUltimateSkill
  (bind _aimingmanager (Variables|Default|GetAimingManager))
  (bind _flataimingmanager (Utilities|Struct|BreakFAimingManager _aimingmanager))
  ;[1 1 1] Skill Manager
  (|CallParentFunction)
  (Utilities|Struct|SetmembersinFAimInfo (Variables|/Game/BrawlStarsReplica/Hero/Base/Blueprint/BP_Aiming_Flat.BP_Aiming_Flat_C|GetAimingInfo _flataimingmanager) true)
  (Default|CenterMousePosition _flataimingmanager))

(fn ConstructionScript
  (|CallParentFunction))