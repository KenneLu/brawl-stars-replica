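; Blueprint function library of small shared helpers for the Brawl Stars replica's heroes and game flow.
; It turns BP_Hero_ asset names into clean hero names, cutting at the first underscore and reporting whether a suffix existed.
; Other helpers pick a random sound from an array, roll a percentage chance from a fractional odds value, and detect the login level by casting the game state to GS_Login.
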(fn FLAdjustHeroName
  (params (OriginalName :type String))
  (bind _returnvalue (Utilities|String|Replace OriginalName "BP_Hero_"))
  (bind (_lefts _rights _returnvalue_2) (Utilities|String|Split _returnvalue "_"))
  (if _returnvalue_2
    (return _lefts _returnvalue_2)
    (else
      (return _returnvalue _returnvalue_2))))

(fn FLGetRandomSound
  (params (Sounds :type Array%20of%20Sound%20Base%20Object%20References))
  (return (Utilities|Array|Get(acopy) Sounds (Math|Random|RandomInteger (Utilities|Array|Length Sounds)))))

(fn FLEventOdds
  (params (Odds :type Float%20%28single-precision%29))
  (return (> (Math|Float|Truncate (* 100 Odds)) (Math|Random|RandomIntegerinRange 0 100))))

(fn FLIsLoginLevel
  (Utilities|Casting|CastToGS_Login (Game|GetGameState)
    (:then
      (return true))
    (:CastFailed
      (return false))))