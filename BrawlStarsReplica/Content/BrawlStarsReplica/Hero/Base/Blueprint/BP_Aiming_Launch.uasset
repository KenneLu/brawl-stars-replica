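; Aiming actor for arced launch skills that previews a trajectory, then moves the hero or another actor along it.
; While locally aiming, it smooths aim distance into a velocity, predicts the projectile path and sends both to the server.
; Non-AI players see the path as rebuilt spline meshes with a landing decal.
; On release, after a delay for replication, a velocity-scaled timeline sweeps the target through the path points until finished or stopped.
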(event Custom|ReleaseLaunchSkill
  (params (isHeroLaunch :type Boolean) (ActorLaunch :type Actor%20Object%20Reference))
  (bind _launchpath (Variables|Default|GetLaunchPath))
  (bind _launchdistance (Variables|Default|GetLaunchDistance))
  (bind _launchpath_2 (Variables|Default|GetLaunchPath))
  (bind _launchpathpositions (Utilities|Struct|BreakFLaunchPath _launchpath))
  (bind (_aimdistanceold _launchdistance_2 _aimdistancemax _launchvelocity _launchvelocitymax) (Utilities|Struct|BreakFLaunchDistance _launchdistance))
  ;[1 1 1] Release Launch Skill Manager
  (Variables|Default|SetIs%20Hero%20Launch isHeroLaunch)
  (Variables|Default|SetActor%20Launch ActorLaunch)
  (Variables|Default|SetStopLaunch false)
  ;;[1 1 1] Wait Set Server Launch Path
  (Utilities|FlowControl|Delay 0.2)
  (Components|Timeline|SetPlayRate (Variables|Default|GetLaunchTimeline) (/ _launchvelocitymax (Math|Vector|VectorLength _launchvelocity)))
  (if (> (Utilities|Array|Length _launchpathpositions) 0)
    (bind _timeline (Timeline|LaunchTimeline PlayFromStart)
      (:Update
        (bind _pass (CallFunction|GetLaunchActor))
        (if _pass
          (if (and (< _timeline 0.95) (not (Variables|Default|GetStopLaunch)))
            (if (Variables|Default|GetIs%20Hero%20Launch)
              (bind _launchcomponent (Variables|Default|GetLaunchComponent)
                (:then
                  (Transformation|SetWorldLocation _launchcomponent (Utilities|Array|Get(acopy) _launchpathpositions (Math|Float|Truncate (Math|Float|Lerp 0.0 (Math|Conversions|ToFloat(Integer) (Utilities|Array|Length _launchpathpositions)) _timeline))) true false))
                (:else))
              (else
                (bind _launchcomponent_2 (Variables|Default|GetLaunchComponent)
                  (:then
                    (Transformation|SetWorldLocation _launchcomponent_2 (Math|Interpolation|VInterpTo (Transformation|GetWorldLocation (Variables|Default|GetLaunchComponent)) (Utilities|Array|Get(acopy) _launchpathpositions (Math|Float|Truncate (Math|Float|Lerp 0.0 (Math|Conversions|ToFloat(Integer) (Utilities|Array|Length _launchpathpositions)) _timeline))) (Utilities|Time|GetWorldDeltaSeconds) 4.0) true false))
                  (:else))))
            (else
              (Audio|Components|Audio|Stop (Variables|Default|GetLaunchTimeline))
              (Utilities|FlowControl|Sequence :!label _label
                (:then_0
                  (Default|CallLaunchEnd)
                  (Variables|Default|SetIs%20Hero%20Launch false))
                (:then_1
                  (Utilities|Array|Clear (.LaunchPathPositions (Utilities|Struct|BreakFLaunchPath _launchpath_2)))
                  (Networking|SwitchHasAuthority
                    (:Remote
                      (CallFunction|SetServerLaunchPath _launchpath_2))))
                (:then_2
                  ;;[1 1 1] AI Clean Launch Info
                  (bind _returnvalue (CallFunction|NotAIControlled))
                  (if (not _returnvalue)
                    (Utilities|Struct|SetmembersinFLaunchDistance (Variables|Default|GetLaunchDistance) 0.0))))))))
      (:Finished
        (goto _label)))
    (else
      (goto _label))))

(event Custom|ServerStopLaunch
  ;[1 1 1] Release Launch Skill Manager
  (Variables|Default|SetStopLaunch true))

(event Custom|SetServerLaunchPath
  (params (LaunchPath :type F%20Launch%20Path%20Structure))
  ;[1 1 1] LaunchAimingManager
  (Variables|Default|SetLaunchPath LaunchPath))

(event Custom|SetServerLaunchDistance
  (params (LaunchDistance :type F%20Launch%20Distance%20Structure))
  ;[1 1 1] LaunchAimingManager
  (Variables|Default|SetLaunchDistance LaunchDistance))

(event Custom|LaunchAimManager
  (bind _aiminginfo (Variables|Default|GetAimingInfo))
  (bind _launchpath (Variables|Default|GetLaunchPath))
  (bind (_isflataiming _islaunchaming _isviewportcentrepointset _viewportcentrepoint _realviewportcentermousepoint _aimdistance) (Utilities|Struct|BreakFAimInfo _aiminginfo))
  (bind _launchpathcomponents (Utilities|Struct|BreakFLaunchPath _launchpath))
  ;[1 1 1] LaunchAimingManager
  (if (Pawn|IsLocallyControlled (Variables|Default|GetHero))
    (if _islaunchaming
      (Utilities|FlowControl|Sequence
        (:then_0
          (CallFunction|UpdateAimDistanceandRotation)
          (if (!= _aimdistance 0.0)
            (CallFunction|UpdateLaunchAimInfo)
            (bind _returnvalue (CallFunction|NotAIControlled))
            (if _returnvalue
              (Rendering|SetVisibility (Variables|Default|GetAimingDecal) true false))
            (CallFunction|ShowLaunchAim)))
        (:then_1
          (goto _label Reset)))
      (else
        (Utilities|FlowControl|DoOnce true :!label _label
          (:Completed
            (Rendering|SetVisibility (Variables|Default|GetAimingDecal) false false)
            (Utilities|Struct|SetmembersinFAimInfo (Variables|Default|GetAimingInfo) 0.0)
            (Utilities|Struct|SetmembersinFLaunchDistance (Variables|Default|GetLaunchDistance) 0.0)
            (Components|DestroyComponent _launchpathcomponents)
            (Utilities|Array|Clear _launchpathcomponents)
            (Networking|SwitchHasAuthority
              (:Remote
                (CallFunction|SetServerLaunchPath _launchpath)))))))))

(event EventBeginPlay)

(event Collision|EventActorBeginOverlap
  (params (OtherActor :type Actor%20Object%20Reference)))

(event EventTick
  (params (DeltaSeconds :type Float%20%28single-precision%29))
  (Variables|Default|GetHero
    (:then
      (CallFunction|LaunchAimManager))
    (:else)))

(fn ConstructionScript
  (bind _aimingdecal (Variables|Default|GetAimingDecal))
  (Rendering|Components|Decal|SetDecalMaterial _aimingdecal "/Game/BrawlStarsReplica/Hero/Base/Asset/M_Decal_LaunchAim_White.M_Decal_LaunchAim_White")
  (Transformation|SetWorldRotation _aimingdecal "90.000000,0.000000,0.000000" false false)
  (Transformation|SetWorldScale3D _aimingdecal "1.000000,1.000000,1.000000")
  (Rendering|SetVisibility _aimingdecal false false))

(fn ShowLaunchAim
  (bind _launchpath (Variables|Default|GetLaunchPath))
  (bind _launchspline (Variables|Default|GetLaunchSpline))
  (bind _launchpath_2 (Variables|Default|GetLaunchPath))
  (bind _launchpathpositions (Utilities|Struct|BreakFLaunchPath _launchpath_2))
  (bind _launchpathcomponents (Utilities|Struct|BreakFLaunchPath _launchpath))
  (bind _returnvalue (Transformation|GetWorldRotation _launchspline))
  (Transformation|SetWorldRotation _launchspline (Math|Rotator|MakeRotator (.roll _returnvalue) (.pitch _returnvalue) (.AimRotationZ (Utilities|Struct|BreakFAimInfo (Variables|Default|GetAimingInfo)))) false false)
  (Components|DestroyComponent _launchpathcomponents)
  (Utilities|Array|Clear _launchpathcomponents)
  (Spline|ClearSplinePoints (Variables|Default|GetLaunchSpline) true)
  (bind _outactors (Actor|GetAllActorsOfClass "/Game/BrawlStarsReplica/Scene/Base/BP_SenceBase.BP_SenceBase_C"))
  (bind (_outhit _outpathpositions _outlasttracedestination) (Class|GameplayStatics|BlueprintPredictProjectilePathbyObjectType (Transformation|GetSocketLocation (Variables|/Script/Engine.Character|GetMesh (Variables|Default|GetHero)) "LaunchStartPoint") (.LaunchVelocity (Utilities|Struct|BreakFLaunchDistance (Variables|Default|GetLaunchDistance))) true 1e+01 (Utilities|Array|MakeArray "ObjectTypeQuery1") false _outactors "None" 0.0 1e+02 12.0))
  (Utilities|Struct|SetmembersinFLaunchPath (Variables|Default|GetLaunchPath) _outpathpositions)
  (bind _returnvalue_2 (CallFunction|NotAIControlled))
  (if _returnvalue_2
    (Transformation|SetWorldLocation (Variables|Default|GetAimingDecal) _outlasttracedestination false false)
    (for (_array_element _array_index) _launchpathpositions
      (Spline|AddSplinePointatIndex (Variables|Default|GetLaunchSpline) _array_element _array_index "Local" true))
    (Spline|SetSplinePointType (Variables|Default|GetLaunchSpline) (Utilities|Array|LastIndex _launchpathpositions) "CurveClamped" true)
    (bind _returnvalue_3 (CallFunction|NotAIControlled))
    (if _returnvalue_3
      (CallFunction|AddLaunchPathComponent 0.05))))

(fn GetLaunchVelocity
  (params (LaunchDistance :type Float%20%28single-precision%29) (LaunchMax :type Float%20%28single-precision%29))
  (bind _launchspline (Variables|Default|GetLaunchSpline))
  (bind _returnvalue (Transformation|GetWorldRotation _launchspline))
  (bind _returnvalue_2 (Math|Vector|GetForwardVector _returnvalue))
  (bind _returnvalue_3 (Math|Vector|GetUpVector _returnvalue))
  (bind _returnvalue_4 (* _returnvalue_3 0.8))
  (bind _returnvalue_5 (+ _returnvalue_2 _returnvalue_4))
  (bind _returnvalue_6 (* _returnvalue_5 LaunchDistance))
  (bind _returnvalue_7 (+ _returnvalue_5 _returnvalue_6))
  (bind _returnvalue_8 (* _returnvalue_7 1e+01))
  (bind _returnvalue_9 (Math|Vector|ClampVectorSize _returnvalue_8 0.0 LaunchMax))
  (if (Pawn|IsBotControlled (Game|GetInstigator))
    (if (Class|KismetSystemLibrary|IsPackagedforDistribution)
      (return (* _returnvalue_9 6))
      (else
        (return (* _returnvalue_9 2))))
    (elif (Class|KismetSystemLibrary|IsPackagedforDistribution)
      (return (* _returnvalue_9 8))
      (else
        (return (* _returnvalue_9 3))))))

(fn UpdateLaunchAimInfo
  (bind _aiminginfo (Variables|Default|GetAimingInfo))
  (bind _launchdistance (Variables|Default|GetLaunchDistance))
  (bind (_aimdistanceold _launchdistance_2 _aimdistancemax _launchvelocity _launchvelocitymax) (Utilities|Struct|BreakFLaunchDistance _launchdistance))
  (bind _aimdistance (Utilities|Struct|BreakFAimInfo _aiminginfo))
  (LocalVariables|SetAimDistance _aimdistance)
  (bind _output_get (LocalVariables|SetAimDistanceDelta (- _aimdistance _aimdistanceold)))
  (if (> _output_get 0.0)
    _
    (else
      ;[1 1 1] Make Sure Distance Back to Zero
      (LocalVariables|SetAimDistanceDelta (* 5 (LocalVariables|GetAimDistanceDelta)))))
  (bind _returnvalue (CallFunction|GetLaunchVelocity (Math|Interpolation|FInterpTo _launchdistance_2 (Math|Float|Clamp(Float) (+ _launchdistance_2 (LocalVariables|GetAimDistanceDelta)) 0.0 _aimdistancemax) (Utilities|Time|GetWorldDeltaSeconds) 3.0) _aimdistancemax))
  (bind _structout (Utilities|Struct|SetmembersinFLaunchDistance (Variables|Default|GetLaunchDistance) (LocalVariables|GetAimDistance) (Math|Interpolation|FInterpTo _launchdistance_2 (Math|Float|Clamp(Float) (+ _launchdistance_2 (LocalVariables|GetAimDistanceDelta)) 0.0 _aimdistancemax) (Utilities|Time|GetWorldDeltaSeconds) 3.0) (Math|Vector|ClampVectorSize _returnvalue 0.0 _launchvelocitymax)))
  (Networking|SwitchHasAuthority
    (:Remote
      (CallFunction|SetServerLaunchDistance _structout))))

(fn AddLaunchPathComponent
  (params (InputPin :type Float%20%28single-precision%29))
  (bind _launchpath (Variables|Default|GetLaunchPath))
  (bind _launchpathpositions (Utilities|Struct|BreakFLaunchPath _launchpath))
  (LocalVariables|SetLaunchPathScale InputPin)
  (for _index (range 0 (- (Spline|GetNumberOfSplinePoints (Variables|Default|GetLaunchSpline)) 3))
    (LocalVariables|SetIndex _index)
    (bind _returnvalue (AddComponent|AddSplineMeshComponent true))
    (SplineMesh|SetStartScale _returnvalue (Math|Vector2D|MakeVector2D (LocalVariables|GetLaunchPathScale) (LocalVariables|GetLaunchPathScale)) true :!class /Script/Engine.SplineMeshComponent)
    (SplineMesh|SetEndScale _returnvalue (Math|Vector2D|MakeVector2D (LocalVariables|GetLaunchPathScale) (LocalVariables|GetLaunchPathScale)) true :!class /Script/Engine.SplineMeshComponent)
    (Utilities|Array|Add (.LaunchPathComponents (Utilities|Struct|BreakFLaunchPath (Variables|Default|GetLaunchPath))) _returnvalue)
    (SplineMesh|SetStartandEnd _returnvalue (Utilities|Array|Get(acopy) _launchpathpositions _index) (Spline|GetTangentatSplinePoint (Variables|Default|GetLaunchSpline) _index "Local") (Utilities|Array|Get(acopy) _launchpathpositions (+ (LocalVariables|GetIndex) 1)) (Spline|GetTangentatSplinePoint (Variables|Default|GetLaunchSpline) (+ (LocalVariables|GetIndex) 1) "Local") true :!class /Script/Engine.SplineMeshComponent)))

(fn GetLaunchActor
  (if (Variables|Default|GetIs%20Hero%20Launch)
    (Variables|Default|GetHero
      (:then
        (Variables|Default|SetLaunchComponent (Variables|/Script/Engine.Character|GetCapsuleComponent (Variables|Default|GetHero)))
        (return true))
      (:else
        (return false)))
    (else
      (bind _actor_launch (Variables|Default|GetActor%20Launch)
        (:then
          (Variables|Default|SetLaunchComponent (Variables|/Script/Engine.Actor|GetRootComponent _actor_launch))
          (return true))
        (:else
          (return false))))))