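; Hero component that gates normal and ultimate skills, tracking normal-skill charges and ultimate energy.
; A looping timer refills charges, paused by Tick when full or mid-skill, while a bound event adds ultimate energy.
; Check functions validate button, activation and release against a shared SkillState struct, which finish events unlock.
; Non-server instances change state locally, then push it to the server through SetServer events.
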(event Custom|SetServerSkillReleasable
  (params (SkillReleasable :type F%20Skill%20State%20Structure))
  ;[1 1 1] Net Sync
  (Variables|Default|SetSkillState SkillReleasable))

(event Custom|CheckNormalSkillReady
  (bind _skillstate (Variables|Default|GetSkillState))
  ;[1 1 1] Check Normal Skill Ready
  (if (>= (Variables|Default|GetNormalSkillCurrent) 1.0)
    (Utilities|Struct|SetmembersinFSkillState _skillstate true)
    (else
      (Utilities|Struct|SetmembersinFSkillState _skillstate false))))

(event Custom|ResetUltimateEnergyCurrent
  ;[1 1 1] Net Sync
  (Variables|Default|SetUltimateEnergyCurrent 0.0))

(event Custom|RechageUltimateSkill
  ;[1 1 1] Rechage Ultimate Skill
  (if (!= (Variables|Default|GetUltimateEnergyCurrent) (Variables|Default|GetUltimateEnergyDefault))
    (Variables|Default|SetUltimateEnergyCurrent (Math|Float|Clamp(Float) (+ (Variables|Default|GetUltimateEnergyCurrent) 1.0) 0.0 (Variables|Default|GetUltimateEnergyDefault)))))

(event Custom|NormalBulletRechage
  ;[1 1 1] Init
  (Variables|Default|SetNormalSkillCurrent (Math|Float|ClampAngle (+ (Variables|Default|GetNormalSkillCurrent) (/ 0.1 (Variables|Default|GetNormalSkillRechageTime))) 0.0 (Variables|Default|GetNormalSkillMax))))

(event Custom|RechageNormalSkill
  (bind _skillstate (Variables|Default|GetSkillState))
  (bind (_isskillpressenable _isskillreleaseenable _isnormalready _isnormalactivated _isnormalend _isultimateready _isultimateactivated _isultimateend) (Utilities|Struct|BreakFSkillState _skillstate))
  ;[1 1 1] Rechage Normal Skill
  (if (Math|Boolean|ANDBoolean (!= (Variables|Default|GetNormalSkillCurrent) (Variables|Default|GetNormalSkillMax)) _isnormalend _isultimateend)
    (if (Class|KismetSystemLibrary|IsTimerPausedHandle (Variables|Default|GetNormalSkillRechageTimer))
      (Utilities|Time|UnpauseTimerbyHandle (Variables|Default|GetNormalSkillRechageTimer)))
    (elif (not (Class|KismetSystemLibrary|IsTimerPausedHandle (Variables|Default|GetNormalSkillRechageTimer)))
      (Utilities|Time|PauseTimerbyHandle (Variables|Default|GetNormalSkillRechageTimer)))))

(event Custom|ResetUltimateLock
  ;[1 1 1] Init
  (bind _structout (Utilities|Struct|SetmembersinFSkillState (Variables|Default|GetSkillState) true true))
  (if (not (Networking|IsServer))
    (CallFunction|SetServerSkillReleasable _structout)))

(event Custom|SetServerSkillAmountCurrent
  (params (SkillAmountCurrent :type Float%20%28single-precision%29))
  ;[1 1 1] Net Sync
  (Variables|Default|SetNormalSkillCurrent SkillAmountCurrent))

(event Custom|CheckUltimateSkillReady
  (bind _skillstate (Variables|Default|GetSkillState))
  ;[1 1 1] Check Ultimate Skill Ready
  (if (>= (Variables|Default|GetUltimateEnergyCurrent) (Variables|Default|GetUltimateEnergyDefault))
    (Utilities|Struct|SetmembersinFSkillState _skillstate true)
    (else
      (Utilities|Struct|SetmembersinFSkillState _skillstate false))))

(event Custom|ResetNormalLock
  ;[1 1 1] Init
  (bind _structout (Utilities|Struct|SetmembersinFSkillState (Variables|Default|GetSkillState) true))
  (if (not (Networking|IsServer))
    (CallFunction|SetServerSkillReleasable _structout)))

(event Custom|RechageUltimateSkillByPercent
  (params (Percent :type Float%20%28single-precision%29))
  ;[1 1 1] Rechage Ultimate Skill
  (if (!= (Variables|Default|GetUltimateEnergyCurrent) (Variables|Default|GetUltimateEnergyDefault))
    (Variables|Default|SetUltimateEnergyCurrent (+ (Variables|Default|GetUltimateEnergyCurrent) (* (Variables|Default|GetUltimateEnergyDefault) Percent)))))

(event Custom|BindUltimateRechage
  ;[1 1 1] Init
  (CallFunction|RechageUltimateSkill))

(event EventBeginPlay
  ;[1 1 1] Init
  (Variables|Default|SetNormalSkillCurrent (Variables|Default|GetNormalSkillMax))
  (bind _returnvalue (Utilities|Time|SetTimerbyEvent (delegate Custom|NormalBulletRechage) 0.1 true))
  (Variables|Default|SetNormalSkillRechageTimer _returnvalue)
  (EventDispatchers|BindEventtoUltimateRechage (delegate Custom|BindUltimateRechage))
  (EventDispatchers|BindEventtoNormalSkillFinished (delegate Custom|ResetNormalLock))
  (EventDispatchers|BindEventtoUltimateSkillFinished (delegate Custom|ResetUltimateLock)))

(event EventTick
  (params (DeltaSeconds :type Float%20%28single-precision%29))
  ;[1 1 1] Tick
  (CallFunction|CheckNormalSkillReady)
  (CallFunction|RechageNormalSkill)
  (CallFunction|CheckUltimateSkillReady))

(fn CheckActivatableNormal
  (bind _skillstate (Variables|Default|GetSkillState))
  (bind (_isskillpressenable _isskillreleaseenable _isnormalready _isnormalactivated _isnormalend _isultimateready _isultimateactivated _isultimateend) (Utilities|Struct|BreakFSkillState _skillstate))
  (if (Math|Boolean|ANDBoolean _isskillpressenable _isnormalready _isnormalend _isultimateend)
    (bind _structout (Utilities|Struct|SetmembersinFSkillState (Variables|Default|GetSkillState) true))
    (if (Networking|IsServer)
      _
      (else
        (CallFunction|SetServerSkillReleasable _structout)))
    (return true)
    (else
      (return false))))

(fn CheckActivatableUltimate
  (bind _skillstate (Variables|Default|GetSkillState))
  (bind (_isskillpressenable _isskillreleaseenable _isnormalready _isnormalactivated _isnormalend _isultimateready _isultimateactivated _isultimateend) (Utilities|Struct|BreakFSkillState _skillstate))
  (if (Math|Boolean|ANDBoolean _isskillpressenable _isultimateready _isultimateend)
    (bind _structout (Utilities|Struct|SetmembersinFSkillState (Variables|Default|GetSkillState) false true))
    (if (Networking|IsServer)
      _
      (else
        (CallFunction|SetServerSkillReleasable _structout)))
    (return true)
    (else
      (return false))))

(fn CheckReleaseableNoremal
  (bind _skillstate (Variables|Default|GetSkillState))
  (bind _skillstate_2 (Variables|Default|GetSkillState))
  (bind (_isskillpressenable _isskillreleaseenable _isnormalready _isnormalactivated _isnormalend _isultimateready _isultimateactivated _isultimateend) (Utilities|Struct|BreakFSkillState _skillstate))
  (if (Math|Boolean|ANDBoolean _isskillreleaseenable _isnormalready _isnormalactivated _isnormalend _isultimateend)
    (Variables|Default|SetNormalSkillCurrent (- (Variables|Default|GetNormalSkillCurrent) 1.0))
    (Utilities|Struct|SetmembersinFSkillState _skillstate_2 false false)
    (if (Networking|IsServer)
      _
      (else
        (CallFunction|SetServerSkillReleasable _skillstate_2)
        (CallFunction|SetServerSkillAmountCurrent (Variables|Default|GetNormalSkillCurrent))))
    (return true)
    (else
      (return false))))

(fn CheckReleaseableUltimate
  (bind _skillstate (Variables|Default|GetSkillState))
  (bind (_isskillpressenable _isskillreleaseenable _isnormalready _isnormalactivated _isnormalend _isultimateready _isultimateactivated _isultimateend) (Utilities|Struct|BreakFSkillState _skillstate))
  (if (Math|Boolean|ANDBoolean _isskillreleaseenable _isultimateready _isultimateactivated _isultimateend)
    (bind _structout (Utilities|Struct|SetmembersinFSkillState (Variables|Default|GetSkillState) false true false false))
    (if (Networking|IsServer)
      _
      (else
        (CallFunction|SetServerSkillReleasable _structout)))
    (return true)
    (else
      (return false))))

(fn CheckPhysicsBottonNoremal
  (params (Press :type Boolean))
  (bind _skillstate (Variables|Default|GetSkillState))
  (bind (_isskillpressenable _isskillreleaseenable _isnormalready _isnormalactivated _isnormalend _isultimateready _isultimateactivated _isultimateend) (Utilities|Struct|BreakFSkillState _skillstate))
  (if Press
    (if (Variables|Default|GetNormalButtonReleased)
      (if (and _isnormalend _isultimateend)
        (Variables|Default|SetNormalButtonPressed true)
        (Variables|Default|SetNormalButtonReleased false)
        (return true)
        (else
          (return false))))
    (elif (Variables|Default|GetNormalButtonPressed)
      (Variables|Default|SetNormalButtonPressed false)
      (Variables|Default|SetNormalButtonReleased true)
      (return true)
      (else
        (return false)))))

(fn CheckPhysicsBottonUltimate
  (params (Press :type Boolean))
  (if Press
    (if (Variables|Default|GetUltimateButtonReleased)
      (if (.isSkillPressEnable (Utilities|Struct|BreakFSkillState (Variables|Default|GetSkillState)))
        (Variables|Default|SetUltimateButtonPressed true)
        (Variables|Default|SetUltimateButtonReleased false)
        (return true)
        (else
          (return false))))
    (elif (Variables|Default|GetUltimateButtonPressed)
      (Variables|Default|SetUltimateButtonPressed false)
      (Variables|Default|SetUltimateButtonReleased true)
      (return true)
      (else
        (return false)))))

(fn IsLocalPlayerControlled
  (bind _returnvalue (Components|GetOwner))
  (bind _instigator (Variables|/Script/Engine.Actor|GetInstigator _returnvalue))
  (return (and (Pawn|IsLocallyControlled _instigator) (not (Pawn|IsBotControlled _instigator)))))